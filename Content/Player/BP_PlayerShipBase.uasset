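; Base player ship with inertial, planar movement driven by Enhanced Input.
; Rotation inputs yaw the sprite, slower while aiming; thrust adds forward momentum, braking eases it toward zero, and Tick offsets the physics root by it.
; Boost plays a Fuel timeline that switches thrust speed and updates fuel.
; Shooting only draws a debug line trace, a test-named end-overlap reverses and dampens momentum, and HUD and asteroid-scoring nodes are unwired.
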(event OnComponentEndOverlap(PlayerCollision)
  (params (OverlappedComponent :type Primitive%20Component%20Object%20Reference) (OtherActor :type Actor%20Object%20Reference) (OtherComp :type Primitive%20Component%20Object%20Reference) (OtherBodyIndex :type Integer))
  (bind _returnvalue (Utilities|GetDisplayName OtherActor))
  (if (Utilities|Enum|Equal(Enum) _returnvalue "ChildCollisionTesting")
    (Development|PrintString _returnvalue)
    (Variables|Default|SetCurrentMomentum (Math|Vector|MakeVector (* (* (.x (Variables|Default|GetCurrentMomentum)) -1.0) 0.2) (* (* (.y (Variables|Default|GetCurrentMomentum)) -1.0) 0.2) 0.0))))

(event Input|EnhancedActionEvents|EnhancedInputActionIA_RotateR
  (params (ActionValue :type Float%20%28double-precision%29) (ElapsedSeconds :type Float%20%28double-precision%29) (TriggeredSeconds :type Float%20%28double-precision%29) (InputAction :type Input%20Action%20Object%20Reference :default "/Game/Player/Input/IA_RotateR.IA_RotateR"))
  (Transformation|AddRelativeRotation (Variables|Default|GetPlayerSprite) (Math|Rotator|MakeRotator 0.0 0.0 (* ActionValue (Math|Float|SelectFloat 4.0 8.0 (stale Input|EnhancedActionEvents|EnhancedInputActionIA_Aim _output_get)))) false false))

(event Input|EnhancedActionEvents|EnhancedInputActionIA_RotateL
  (params (ActionValue :type Float%20%28double-precision%29) (ElapsedSeconds :type Float%20%28double-precision%29) (TriggeredSeconds :type Float%20%28double-precision%29) (InputAction :type Input%20Action%20Object%20Reference :default "/Game/Player/Input/IA_RotateL.IA_RotateL"))
  (Transformation|AddRelativeRotation (Variables|Default|GetPlayerSprite) (Math|Rotator|MakeRotator 0.0 0.0 (* ActionValue (* (Math|Float|SelectFloat 4.0 8.0 (stale Input|EnhancedActionEvents|EnhancedInputActionIA_Aim _output_get)) -1.0))) false false))

(event Input|EnhancedActionEvents|EnhancedInputActionIA_Thrusters
  (params (ActionValue :type Float%20%28double-precision%29) (ElapsedSeconds :type Float%20%28double-precision%29) (TriggeredSeconds :type Float%20%28double-precision%29) (InputAction :type Input%20Action%20Object%20Reference :default "/Game/Player/Input/IA_Thrusters.IA_Thrusters"))
  (bind _playersprite (Variables|Default|GetPlayerSprite))
  (bind _updatespeedmultiplier (Variables|Default|GetUpdateSpeedMultiplier))
  (bind _returnvalue (Math|Vector|GetForwardVector _playersprite))
  (bind _returnvalue_2 (* _returnvalue _updatespeedmultiplier))
  (:Triggered
    (Variables|Default|SetIsThrusting true)
    (Variables|Default|SetCurrentMomentum (Math|Vector|MakeVector (+ (.x _returnvalue_2) (.x (Variables|Default|GetCurrentMomentum))) (+ (.y _returnvalue_2) (.y (Variables|Default|GetCurrentMomentum))) 0.0)))
  (:Canceled
    (Variables|Default|SetIsThrusting false :!label _label))
  (:Completed
    (goto _label)))

(event Input|EnhancedActionEvents|EnhancedInputActionIA_Boost
  (params (ActionValue :type Float%20%28double-precision%29) (ElapsedSeconds :type Float%20%28double-precision%29) (TriggeredSeconds :type Float%20%28double-precision%29) (InputAction :type Input%20Action%20Object%20Reference :default "/Game/Player/Input/IA_Boost.IA_Boost"))
  (:Started
    (bind (_direction _subtractfuel) (Timeline|+-Fuel Play)
      (:Update
        (switch Utilities|FlowControl|Switch|SwitchonETimelineDirection _direction
          (:Forward
            (Variables|Default|SetUpdateSpeedMultiplier (Variables|Default|GetBoostSpeed)))
          (:Backward
            (Variables|Default|SetUpdateSpeedMultiplier (Variables|Default|GetThrustSpeed) :!label _label))))
      (:Finished
        (goto _label)))
    (Variables|Default|SetFuel _subtractfuel))
  (:Canceled
    (Timeline|+-Fuel Reverse))
  (:Completed
    (Timeline|+-Fuel Reverse)))

(event Input|EnhancedActionEvents|EnhancedInputActionIA_Shoot
  (params (ActionValue :type Float%20%28double-precision%29) (ElapsedSeconds :type Float%20%28double-precision%29) (TriggeredSeconds :type Float%20%28double-precision%29) (InputAction :type Input%20Action%20Object%20Reference :default "/Game/Player/Input/IA_Shoot.IA_Shoot"))
  (bind _playersprite (Variables|Default|GetPlayerSprite))
  (bind _returnvalue (Transformation|GetWorldLocation _playersprite))
  (bind _returnvalue_2 (Collision|LineTraceByChannel _returnvalue (+ _returnvalue (* (Math|Vector|GetForwardVector _playersprite) (Math|Conversions|ToVector(Float) 2e+03))) "TraceTypeQuery1" false 0 "ForDuration" true "(R=1.000000,G=1.000000,B=1.000000,A=1.000000)" "(R=0.000000,G=1.000000,B=0.000000,A=1.000000)" 0.25))
  (if _returnvalue_2
    _))

(event Input|EnhancedActionEvents|EnhancedInputActionIA_Aim
  (params (ActionValue :type Boolean) (ElapsedSeconds :type Float%20%28double-precision%29) (TriggeredSeconds :type Float%20%28double-precision%29) (InputAction :type Input%20Action%20Object%20Reference :default "/Game/Player/Input/IA_Aim.IA_Aim"))
  (:Triggered
    (bind _output_get (Variables|Default|SetIsAiming true)))
  (:Canceled
    (Variables|Default|SetIsAiming false :!label _label))
  (:Completed
    (goto _label)))

(event Input|EnhancedActionEvents|EnhancedInputActionIA_Brake
  (params (ActionValue :type Float%20%28double-precision%29) (ElapsedSeconds :type Float%20%28double-precision%29) (TriggeredSeconds :type Float%20%28double-precision%29) (InputAction :type Input%20Action%20Object%20Reference :default "/Game/Player/Input/IA_Brake.IA_Brake"))
  (bind _returnvalue (Utilities|Time|GetWorldDeltaSeconds))
  (:Triggered
    (Variables|Default|SetIsBraking true)
    (Variables|Default|SetCurrentMomentum (Math|Vector|MakeVector (Math|Interpolation|FInterpTo (.x (Variables|Default|GetCurrentMomentum)) 0.0 _returnvalue 3.5) (Math|Interpolation|FInterpTo (.y (Variables|Default|GetCurrentMomentum)) 0.0 _returnvalue 3.5) 0.0)))
  (:Canceled
    (Variables|Default|SetIsBraking false :!label _label))
  (:Completed
    (goto _label)))

(event EventTick
  (params (DeltaSeconds :type Float%20%28single-precision%29))
  (bind _currentmomentum (Variables|Default|GetCurrentMomentum))
  (Utilities|FlowControl|Sequence
    (:then_0
      (Transformation|AddWorldOffset (Variables|Default|GetPhysicsRoot) (Math|Vector|MakeVector (* (.x _currentmomentum) 0.6) (* (.y _currentmomentum) 0.6) 0.0) false false))))

(event EventBeginPlay
  (bind _aspc_player (Utilities|Casting|CastToPC_Player (Game|GetPlayerController 0)))
  (Utilities|IsValid _aspc_player
    (:Is%20Valid
      (Utilities|IsValid (PlayerController|LocalPlayerSubsystems|GetEnhancedInputLocalPlayerSubsystem _aspc_player)
        (:Is%20Valid
          (Input|AddMappingContext (PlayerController|LocalPlayerSubsystems|GetEnhancedInputLocalPlayerSubsystem _aspc_player) "/Game/Player/Input/IMC_Default.IMC_Default" 0 "(bIgnoreAllPressedKeysUntilRelease=True,bForceImmediately=False,bNotifyUserSettings=False)"))))))

(fn ConstructionScript)