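; BP_Spectator is a player-controlled spectator that pans around the world on the horizontal plane.
; On BeginPlay it adds the IMC_Player input mapping and caches the HUD widget from BP_Standard_PlayerController.
; The thrust, brake and turn inputs offset its Scene component in world X/Y by SpectateSpeed, without delta-time scaling.
; Secondary input calls ExitSpectator on the controller, while pause toggles the game through BP_GameInstance and shows or hides the HUD.
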(event Input|EnhancedActionEvents|EnhancedInputActionIA_Thrust
  (params (ActionValue :type Float%20%28double-precision%29) (ElapsedSeconds :type Float%20%28double-precision%29) (TriggeredSeconds :type Float%20%28double-precision%29) (InputAction :type Input%20Action%20Object%20Reference :default "/Game/Player/Input/IA_Thrust.IA_Thrust"))
  (Transformation|AddWorldOffset (Variables|Default|GetScene) (Math|Vector|MakeVector 0.0 (* (Variables|Default|GetSpectateSpeed) -1.0) 0.0) false false))

(event Input|EnhancedActionEvents|EnhancedInputActionIA_Brake
  (params (ActionValue :type Float%20%28double-precision%29) (ElapsedSeconds :type Float%20%28double-precision%29) (TriggeredSeconds :type Float%20%28double-precision%29) (InputAction :type Input%20Action%20Object%20Reference :default "/Game/Player/Input/IA_Brake.IA_Brake"))
  (Transformation|AddWorldOffset (Variables|Default|GetScene) (Math|Vector|MakeVector 0.0 (Variables|Default|GetSpectateSpeed) 0.0) false false))

(event Input|EnhancedActionEvents|EnhancedInputActionIA_TurnL
  (params (ActionValue :type Float%20%28double-precision%29) (ElapsedSeconds :type Float%20%28double-precision%29) (TriggeredSeconds :type Float%20%28double-precision%29) (InputAction :type Input%20Action%20Object%20Reference :default "/Game/Player/Input/IA_TurnL.IA_TurnL"))
  (Transformation|AddWorldOffset (Variables|Default|GetScene) (Math|Vector|MakeVector (* (Variables|Default|GetSpectateSpeed) -1.0) 0.0 0.0) false false))

(event Input|EnhancedActionEvents|EnhancedInputActionIA_TurnR
  (params (ActionValue :type Float%20%28double-precision%29) (ElapsedSeconds :type Float%20%28double-precision%29) (TriggeredSeconds :type Float%20%28double-precision%29) (InputAction :type Input%20Action%20Object%20Reference :default "/Game/Player/Input/IA_TurnR.IA_TurnR"))
  (Transformation|AddWorldOffset (Variables|Default|GetScene) (Math|Vector|MakeVector (Variables|Default|GetSpectateSpeed) 0.0 0.0) false false))

(event Input|EnhancedActionEvents|EnhancedInputActionIA_Secondary
  (params (ActionValue :type Float%20%28double-precision%29) (ElapsedSeconds :type Float%20%28double-precision%29) (TriggeredSeconds :type Float%20%28double-precision%29) (InputAction :type Input%20Action%20Object%20Reference :default "/Game/Player/Input/IA_Secondary.IA_Secondary"))
  (bind _asbp_standard_player_controller (Utilities|Casting|CastToBP_Standard_PlayerController (Pawn|GetController)))
  (Default|ExitSpectator _asbp_standard_player_controller self))

(event Input|EnhancedActionEvents|EnhancedInputActionIA_Pause
  (params (ActionValue :type Boolean) (ElapsedSeconds :type Float%20%28double-precision%29) (TriggeredSeconds :type Float%20%28double-precision%29) (InputAction :type Input%20Action%20Object%20Reference :default "/Game/Player/Input/IA_Pause.IA_Pause"))
  (bind _wpb_hud (Variables|Default|GetWPB%20HUD))
  (:Started
    (bind _asbp_game_instance (Utilities|Casting|CastToBP_GameInstance (Game|GetGameInstance)))
    (bind _isgamepausedresult (Default|TogglePauseGame _asbp_game_instance))
    (if _isgamepausedresult
      (Widget|SetVisibility _wpb_hud "Hidden")
      (else
        (Widget|SetVisibility _wpb_hud "Visible")))))

(event EventBeginPlay
  (bind _asbp_standard_player_controller (Utilities|Casting|CastToBP_Standard_PlayerController (Game|GetPlayerController 0)))
  (Utilities|IsValid _asbp_standard_player_controller
    (:Is%20Valid
      (Utilities|IsValid (PlayerController|LocalPlayerSubsystems|GetEnhancedInputLocalPlayerSubsystem _asbp_standard_player_controller)
        (:Is%20Valid
          (Input|AddMappingContext (PlayerController|LocalPlayerSubsystems|GetEnhancedInputLocalPlayerSubsystem _asbp_standard_player_controller) "/Game/Player/Input/IMC_Player.IMC_Player" 0 "(bIgnoreAllPressedKeysUntilRelease=True,bForceImmediately=False,bNotifyUserSettings=False)")
          (bind _asbp_standard_player_controller_2 (Utilities|Casting|CastToBP_Standard_PlayerController (Game|GetPlayerController 0)))
          (Variables|Default|SetWPB%20HUD (Variables|/Game/Framework/BP_Standard_PlayerController.BP_Standard_PlayerController_C|GetWBP_HUD _asbp_standard_player_controller_2)))))))

(fn ConstructionScript)