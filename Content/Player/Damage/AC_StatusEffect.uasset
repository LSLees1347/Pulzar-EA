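; Actor component that applies status effects (Bleed, Slow or Stop) to the actor that owns it.
; TriggerEffect switches on the requested effect and spawns the matching effect actor at the owner's transform, owned by and snap-attached to that owner.
; Only Slow uses the Controller input, passing its controlled pawn as Instigator.
; The component holds no effect logic beyond spawning and attaching.
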(event EventBeginPlay)

(event EventTick
  (params (DeltaSeconds :type Float%20%28single-precision%29)))

(fn TriggerEffect
  (params (Effect :type E_StatusEffects%20Enum :default "E_StatusEffects_MAX") (Controller :type Controller%20Object%20Reference))
  (bind _returnvalue (Components|GetOwner))
  (bind _returnvalue_2 (Components|GetOwner))
  (bind _returnvalue_3 (Components|GetOwner))
  (switch Utilities|FlowControl|Switch|SwitchonE_StatusEffects Effect
    (:NewEnumerator0
      (bind _returnvalue_4 (Game|SpawnActorfromClass "/Game/Player/Damage/Bleed/Effect_Bleed.Effect_Bleed_C" (Transformation|GetActorTransform _returnvalue_2) "Undefined" "MultiplyWithRoot" _returnvalue_2 0))
      (Transformation|AttachActorToActor _returnvalue_4 (Components|GetOwner) "None" "SnapToTarget" "SnapToTarget" "SnapToTarget" true))
    (:NewEnumerator1
      (bind _returnvalue_5 (Game|SpawnActorfromClass "/Game/Player/Damage/Slow/Effect_Slow.Effect_Slow_C" (Transformation|GetActorTransform _returnvalue_3) "Undefined" "MultiplyWithRoot" _returnvalue_3 (Pawn|GetControlledPawn Controller)))
      (Transformation|AttachActorToActor _returnvalue_5 (Components|GetOwner) "None" "SnapToTarget" "SnapToTarget" "SnapToTarget" true))
    (:NewEnumerator2
      (bind _returnvalue_6 (Game|SpawnActorfromClass "/Game/Player/Damage/Stop/Effect_Stop.Effect_Stop_C" (Transformation|GetActorTransform _returnvalue) "Undefined" "MultiplyWithRoot" _returnvalue 0))
      (Transformation|AttachActorToActor _returnvalue_6 (Components|GetOwner) "None" "SnapToTarget" "SnapToTarget" "SnapToTarget" true))))