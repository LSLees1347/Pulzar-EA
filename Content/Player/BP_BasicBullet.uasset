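; BP_BasicBullet is a projectile that damages the first overlapped actor other than its instigator, then destroys itself.
; Tick moves it along local X by Speed each frame without delta-time scaling, and BeginPlay destroys it after a delay.
; On a hit it calls events named as server and multicast RPCs to apply fixed damage and spawn a small Niagara effect at its location.
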(event Custom|Svr_ApplyDamage
  (params (DamagedActor :type Actor%20Object%20Reference))
  (Game|Damage|ApplyDamage DamagedActor 25.0 0 (Game|GetInstigator)))

(event Custom|MC_HitEffect
  (Niagara|SpawnSystematLocation (Variables|Default|GetHitEffect) (Transformation|GetActorLocation) "0, 0, 0" "0.100000,0.100000,0.100000"))

(event EventBeginPlay
  (Utilities|FlowControl|Delay (Variables|Default|GetDuration))
  (Actor|DestroyActor))

(event EventTick
  (params (DeltaSeconds :type Float%20%28single-precision%29))
  (Transformation|AddActorLocalOffset (Math|Vector|MakeVector (Variables|Default|GetSpeed) 0.0 0.0) false false))

(event Collision|EventActorBeginOverlap
  (params (OtherActor :type Actor%20Object%20Reference))
  (if (not (== (Game|GetInstigator) OtherActor))
    (CallFunction|SvrApplyDamage OtherActor)
    (CallFunction|MCHitEffect)
    (Actor|DestroyActor)))

(fn ConstructionScript)