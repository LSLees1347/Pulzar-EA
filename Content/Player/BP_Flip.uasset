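; BP_Flip is a player pawn that turns toward the mouse cursor and thrusts forward, using Enhanced Input.
; The locally controlled pawn computes rotation from a cursor trace each tick, applies it immediately and sends it to the server when remote.
; Thrust adds movement along the sprite's forward vector while a timeline widens camera FOV, reversing on release.
; The construction script zeroes FloatingPawnMovement's speed, acceleration and deceleration.
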(event Custom|SVR_Tick
  (params (NewRot :type Rotator))
  (bind _output_get (Variables|Default|SetNewRot NewRot))
  (Transformation|SetActorRotation _output_get true))

(event Input|EnhancedActionEvents|EnhancedInputActionIA_Thrust
  (params (ActionValue :type Float%20%28double-precision%29) (ElapsedSeconds :type Float%20%28double-precision%29) (TriggeredSeconds :type Float%20%28double-precision%29) (InputAction :type Input%20Action%20Object%20Reference :default "/Game/Player/Input/IA_Thrust.IA_Thrust"))
  (bind _sprite (Variables|Default|GetSprite))
  (bind _returnvalue (Math|Vector|GetForwardVector _sprite))
  (:Triggered
    (Variables|Default|SetIsThrusting true)
    (Pawn|Input|AddMovementInput (Math|Vector|MakeVector (.x _returnvalue) (.y _returnvalue) 0.0) 1.0 true)
    (bind _zoomout (Timeline|Timeline Play)
      (:Update
        (Camera|SetFieldOfView (Variables|Default|GetCamera) (Math|Float|Lerp 9e+01 1e+02 _zoomout)))))
  (:Canceled
    (Variables|Default|SetIsThrusting false :!label _label)
    (Timeline|Timeline Reverse))
  (:Completed
    (goto _label)))

(event EventPossessed
  (params (NewController :type Controller%20Object%20Reference))
  (bind _asbp_standard_player_controller (Utilities|Casting|CastToBP_Standard_PlayerController NewController))
  (Variables|Default|SetAs%20BP%20Standard%20Player%20Controller _asbp_standard_player_controller))

(event EventBeginPlay
  (bind _returnvalue (Transformation|GetActorLocation))
  (Utilities|FlowControl|Sequence
    (:then_0
      (bind _asbp_standard_player_controller (Utilities|Casting|CastToBP_Standard_PlayerController (Game|GetPlayerController 0)))
      (Utilities|IsValid _asbp_standard_player_controller
        (:Is%20Valid
          (Utilities|IsValid (PlayerController|LocalPlayerSubsystems|GetEnhancedInputLocalPlayerSubsystem _asbp_standard_player_controller)
            (:Is%20Valid
              (Input|AddMappingContext (PlayerController|LocalPlayerSubsystems|GetEnhancedInputLocalPlayerSubsystem _asbp_standard_player_controller) "/Game/Player/Input/IMC_Player.IMC_Player" 0 "(bIgnoreAllPressedKeysUntilRelease=True,bForceImmediately=False,bNotifyUserSettings=False)")
              (Transformation|SetActorLocation (Math|Vector|MakeVector (.x _returnvalue) (.y _returnvalue) 0.0) false false))))))))

(event EventTick
  (params (DeltaSeconds :type Float%20%28single-precision%29))
  (bind _returnvalue (Transformation|GetActorLocation))
  (bind _as_bp_standard_player_controller (Variables|Default|GetAs%20BP%20Standard%20Player%20Controller))
  (bind _hitresult (Game|Player|GetHitResultUnderCursorbyChannel _as_bp_standard_player_controller "TraceTypeQuery1" true))
  (bind _returnvalue_2 (Math|Rotator|FindLookatRotation (Math|Vector|MakeVector (.x _returnvalue) (.y _returnvalue) 0.0) (Math|Vector|MakeVector (.x (.location _hitresult)) (.y (.location _hitresult)) 0.0)))
  (if (Pawn|IsLocallyControlled)
    (Transformation|SetActorRotation _returnvalue_2 true)
    (Networking|SwitchHasAuthority
      (:Authority
        (bind _output_get (Variables|Default|SetNewRot _returnvalue_2))
        (Transformation|SetActorRotation _output_get true))
      (:Remote
        (CallFunction|SVRTick _returnvalue_2)))))

(fn ConstructionScript
  (bind _floatingpawnmovement (Variables|Default|GetFloatingPawnMovement))
  (Variables|/Script/Engine.FloatingPawnMovement|SetMaxSpeed _floatingpawnmovement 0.0)
  (Variables|/Script/Engine.FloatingPawnMovement|SetAcceleration _floatingpawnmovement 0.0)
  (Variables|/Script/Engine.FloatingPawnMovement|SetDeceleration _floatingpawnmovement 0.0))

(fn SVR
  (params (NewParam1 :type Rotator)))