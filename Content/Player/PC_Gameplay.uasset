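; Gameplay player controller that spawns the player's selected ship and takes control of it.
; On BeginPlay it prints a debug greeting, caps the frame rate, hides the cursor and switches to game-only input.
; It reads the ship class from the GI_Player game instance, writing BPC_Starter back as the fallback when none is valid, then spawns and possesses that ship through player controller 0.
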(event EventPossess
  (params (PossessedPawn :type Pawn%20Object%20Reference)))

(event EventBeginPlay
  (bind _returnvalue (Game|GetPlayerController 0))
  (Development|PrintString "Hello")
  (bind _returnvalue_2 (Settings|GetGameUserSettings))
  (Class|GameUserSettings|SetFrameRateLimit _returnvalue_2 6e+01)
  (Variables|/Script/Engine.PlayerController|SetbShowMouseCursor _returnvalue false)
  (Input|SetInputModeGameOnly _returnvalue false)
  (bind _asgi_player (Utilities|Casting|CastToGI_Player (Game|GetGameInstance)))
  (if (Utilities|IsValidClass (Variables|/Game/Player/GI_Player.GI_Player_C|GetShipSelection _asgi_player))
    _
    (else
      (Variables|/Game/Player/GI_Player.GI_Player_C|SetShipSelection _asgi_player "/Game/Player/Ships/Starter/BPC_Starter.BPC_Starter_C")))
  (bind _returnvalue_3 (Game|SpawnActorfromClass (Variables|/Game/Player/GI_Player.GI_Player_C|GetShipSelection _asgi_player) (Variables|Default|GetSpawnTransform) "Undefined" "MultiplyWithRoot" 0 0))
  (Pawn|Possess (Game|GetPlayerController 0) _returnvalue_3))

(fn ConstructionScript)