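; Gameplay game mode with an event for scattering asteroids around the level.
; SpawnAsteroid creates one BP_AsteroidBase at a random X/Y within a square centered on the origin, in a narrow height band below zero.
; A loop meant to repeat the spawn AsteroidsToSpawn1 times is disconnected, so each event call spawns only one.
; The default pawn class override just returns the parent's result.
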(event Custom|Spawn%20Asteroid
  ;[1 1 1] spawn asteroids
  (Game|SpawnActorfromClass "/Game/Actors/Asteroids/BP_AsteroidBase.BP_AsteroidBase_C" (Math|Transform|MakeTransform (Math|Vector|MakeVector (* (Math|Random|RandomFloat) (Math|Float|SelectFloat -6.5e+03 6.5e+03 (Math|Random|RandomBool))) (* (Math|Random|RandomFloat) (Math|Float|SelectFloat -6.5e+03 6.5e+03 (Math|Random|RandomBool))) (Math|Random|RandomFloatinRange -485.0 -515.0)) "0, 0, 0" "1.000000,1.000000,1.000000") "Undefined" "MultiplyWithRoot" 0 0))

(fn ConstructionScript)

(fn GetDefaultPawnClassforController
  (params (InController :type Controller%20Object%20Reference))
  (bind _returnvalue (|CallParentFunction InController))
  (return _returnvalue))