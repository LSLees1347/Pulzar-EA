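; Game mode for the main menu that manages players joining the lobby and keeps their player lists in sync.
; When a new player starts on the lobby map, it registers their PC_MMenu controller, then has it create the lobby menu and run initial setup.
; UpdateLobby, when flagged for player names, rebuilds the profile list from all registered controllers and pushes it back to each one.
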(event Custom|UpdateLobby
  (params (PlayerNames :type Boolean))
  (if PlayerNames
    (Utilities|Array|Clear (Variables|Default|GetPlayerProfiles))
    (for _array_element (Variables|Default|GetAllConnectedPlayers)
      (Utilities|Array|Add (Variables|Default|GetPlayerProfiles) (Variables|/Game/Player/PC_MMenu.PC_MMenu_C|GetPlayer%20Profile _array_element)))
    (for _array_element_2 (Variables|Default|GetAllConnectedPlayers)
      (if PlayerNames
        (Default|UpdatePlayerNames _array_element_2 (Variables|Default|GetPlayerProfiles))))))

(event EventHandleStartingNewPlayer
  (params (NewPlayer :type Player%20Controller%20Object%20Reference))
  (bind _returnvalue (Game|GetCurrentLevelName true))
  (switch string _returnvalue
    (:LobbyMenuMap
      (bind _aspc_mmenu (Utilities|Casting|CastToPC_MMenu NewPlayer))
      (Utilities|Array|Add (Variables|Default|GetAllConnectedPlayers) _aspc_mmenu)
      (Default|CreateLobbyMenu _aspc_mmenu)
      (Default|InitialSetup _aspc_mmenu))))

(fn ConstructionScript)