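; Player ship base: Enhanced Input drives planar flight, aiming, camera zoom, a minimap and hitscan shots at asteroids.
; Thrust, boost and brake edit a momentum vector that Tick applies as world offset and a looping timer scales.
; Boost and shooting raise Temperature, which gates boost and cools on a delayed timer.
; Leaving game bounds starts timed health drain, while Death restores health and temperature at the spawn point.
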(event Custom|Death
  (Variables|Default|SetPlayerHealth (Variables|Default|GetPlayerMaxHealth))
  (Variables|Default|SetTemperature 0.15)
  (bind _sweephitresult (Transformation|SetWorldTransform (Variables|Default|GetRoot%20Collision) (Variables|Default|GetSpawnPoint) false true)))

(event Custom|CapSpeed
  (bind _capspeedmultiplier (Variables|Default|GetCapSpeedMultiplier))
  (Variables|Default|SetCurrentMomentum (Math|Vector|MakeVector (* (.x (Variables|Default|GetCurrentMomentum)) _capspeedmultiplier) (* (.y (Variables|Default|GetCurrentMomentum)) _capspeedmultiplier) 0.0)))

(event Custom|ExitGameBounds
  (bind _returnvalue (Utilities|Time|SetTimerbyFunctionName 0 "TakeZoneDamage" 0.016667 true true))
  (Variables|Timers|SetT_ZoneDamage _returnvalue))

(event Custom|EnterGameBounds
  (Utilities|Time|ClearandInvalidateTimerbyHandle (Variables|Timers|GetT_ZoneDamage)))

(event Input|EnhancedActionEvents|EnhancedInputActionIA_Shoot
  (params (ActionValue :type Float%20%28double-precision%29) (ElapsedSeconds :type Float%20%28double-precision%29) (TriggeredSeconds :type Float%20%28double-precision%29) (InputAction :type Input%20Action%20Object%20Reference :default "/Game/Player/Input/IA_Shoot.IA_Shoot"))
  (bind _sprite (Variables|Default|GetSprite))
  (bind _returnvalue (Transformation|GetWorldLocation _sprite))
  (Variables|Default|SetTemperature (Math|Float|Clamp(Float) (+ (Variables|Default|GetTemperature) 0.05)))
  (Utilities|FlowControl|Sequence
    (:then_0
      (bind _outhit (Collision|LineTraceByChannel _returnvalue (+ _returnvalue (* (Math|Vector|GetForwardVector _sprite) (Math|Conversions|ToVector(Float) (Variables|Default|GetHitScanRange)))) "TraceTypeQuery1" false 0 "ForOneFrame" true "(R=1.000000,G=1.000000,B=1.000000,A=1.000000)" "(R=0.000000,G=1.000000,B=0.000000,A=1.000000)" 0.25))
      (bind _asbp_asteroid_base (Utilities|Casting|CastToBP_AsteroidBase (.hitactor _outhit)))
      (Default|Hit _asbp_asteroid_base))
    (:then_1
      (bind _returnvalue_2 (Utilities|Time|SetTimerbyFunctionName 0 "SubtractTemp" 0.5 true true 1.0))
      (bind _output_get (Variables|Timers|SetT_SubtractTemp _returnvalue_2)))))

(event Input|EnhancedActionEvents|EnhancedInputActionIA_Thrust
  (params (ActionValue :type Float%20%28double-precision%29) (ElapsedSeconds :type Float%20%28double-precision%29) (TriggeredSeconds :type Float%20%28double-precision%29) (InputAction :type Input%20Action%20Object%20Reference :default "/Game/Player/Input/IA_Thrust.IA_Thrust"))
  (bind _sprite (Variables|Default|GetSprite))
  (bind _thrustspeed (Variables|Default|GetThrustSpeed))
  (bind _returnvalue (Math|Vector|GetForwardVector _sprite))
  (bind _returnvalue_2 (* _returnvalue _thrustspeed))
  (:Triggered
    (Variables|AnimCalls|SetIsThrusting true)
    (Variables|Default|SetCurrentMomentum (Math|Vector|MakeVector (+ (.x _returnvalue_2) (.x (Variables|Default|GetCurrentMomentum))) (+ (.y _returnvalue_2) (.y (Variables|Default|GetCurrentMomentum))) 0.0)))
  (:Canceled
    (Variables|AnimCalls|SetIsThrusting false :!label _label))
  (:Completed
    (goto _label)))

(event Input|EnhancedActionEvents|EnhancedInputActionIA_TurnL
  (params (ActionValue :type Float%20%28double-precision%29) (ElapsedSeconds :type Float%20%28double-precision%29) (TriggeredSeconds :type Float%20%28double-precision%29) (InputAction :type Input%20Action%20Object%20Reference :default "/Game/Player/Input/IA_TurnL.IA_TurnL"))
  (Transformation|AddRelativeRotation (Variables|Default|GetSprite) (Math|Rotator|MakeRotator 0.0 0.0 (* ActionValue (* (Math|Float|SelectFloat 4.0 8.0 (stale Input|EnhancedActionEvents|EnhancedInputActionIA_Aim _output_get)) -1.0))) false false))

(event Input|EnhancedActionEvents|EnhancedInputActionIA_Minimap
  (params (ActionValue :type Boolean) (ElapsedSeconds :type Float%20%28double-precision%29) (TriggeredSeconds :type Float%20%28double-precision%29) (InputAction :type Input%20Action%20Object%20Reference :default "/Game/Player/Input/IA_Minimap.IA_Minimap"))
  (:Started
    (Utilities|IsValid (stale _returnvalue)
      (:Is%20Valid
        (Widget|SetVisibility (stale _returnvalue) "Visible"))
      (:Is%20Not%20Valid
        (bind _returnvalue (UserInterface|CreateWidget "/Game/Widgets/WPB_MM.WPB_MM_C"))
        (UserInterface|Viewport|AddtoViewport _returnvalue 10)
        (Widget|SetVisibility _returnvalue "Visible"))))
  (:Canceled
    (Widget|SetVisibility _returnvalue "Hidden" :!label _label))
  (:Completed
    (goto _label)))

(event Input|EnhancedActionEvents|EnhancedInputActionIA_Boost
  (params (ActionValue :type Float%20%28double-precision%29) (ElapsedSeconds :type Float%20%28double-precision%29) (TriggeredSeconds :type Float%20%28double-precision%29) (InputAction :type Input%20Action%20Object%20Reference :default "/Game/Player/Input/IA_Boost.IA_Boost"))
  (bind _sprite (Variables|Default|GetSprite))
  (bind _boostspeed (Variables|Default|GetBoostSpeed))
  (bind _returnvalue (Math|Vector|GetForwardVector _sprite))
  (bind _returnvalue_2 (* _returnvalue _boostspeed))
  (:Triggered
    (if (and (Variables|AnimCalls|GetIsThrusting) (< (Variables|Default|GetTemperature) 1.0))
      (Variables|AnimCalls|SetIsBoosting true)
      (Utilities|Time|ClearandInvalidateTimerbyHandle (stale _output_get))
      (Variables|Default|SetCurrentMomentum (Math|Vector|MakeVector (+ (.x _returnvalue_2) (.x (Variables|Default|GetCurrentMomentum))) (+ (.y _returnvalue_2) (.y (Variables|Default|GetCurrentMomentum))) 0.0))
      (Variables|Default|SetTemperature (Math|Float|Clamp(Float) (+ (Variables|Default|GetTemperature) 0.002) 0.15))
      (else
        (Variables|AnimCalls|SetIsBoosting false))))
  (:Canceled
    (Variables|AnimCalls|SetIsBoosting false :!label _label)
    (bind _returnvalue_3 (Utilities|Time|SetTimerbyFunctionName 0 "SubtractTemp" 0.5 true true 1.0))
    (bind _output_get (Variables|Timers|SetT_SubtractTemp _returnvalue_3)))
  (:Completed
    (goto _label)))

(event Input|EnhancedActionEvents|EnhancedInputActionIA_Aim
  (params (ActionValue :type Float%20%28double-precision%29) (ElapsedSeconds :type Float%20%28double-precision%29) (TriggeredSeconds :type Float%20%28double-precision%29) (InputAction :type Input%20Action%20Object%20Reference :default "/Game/Player/Input/IA_Aim.IA_Aim"))
  (:Triggered
    (bind _output_get (Variables|AnimCalls|SetIsAiming true)))
  (:Canceled
    (Variables|AnimCalls|SetIsAiming false :!label _label))
  (:Completed
    (goto _label)))

(event Input|EnhancedActionEvents|EnhancedInputActionIA_TurnR
  (params (ActionValue :type Float%20%28double-precision%29) (ElapsedSeconds :type Float%20%28double-precision%29) (TriggeredSeconds :type Float%20%28double-precision%29) (InputAction :type Input%20Action%20Object%20Reference :default "/Game/Player/Input/IA_TurnR.IA_TurnR"))
  (Transformation|AddRelativeRotation (Variables|Default|GetSprite) (Math|Rotator|MakeRotator 0.0 0.0 (* ActionValue (Math|Float|SelectFloat 4.0 8.0 (stale Input|EnhancedActionEvents|EnhancedInputActionIA_Aim _output_get)))) false false))

(event Input|EnhancedActionEvents|EnhancedInputActionIA_Brake
  (params (ActionValue :type Float%20%28double-precision%29) (ElapsedSeconds :type Float%20%28double-precision%29) (TriggeredSeconds :type Float%20%28double-precision%29) (InputAction :type Input%20Action%20Object%20Reference :default "/Game/Player/Input/IA_Brake.IA_Brake"))
  (bind _returnvalue (Utilities|Time|GetWorldDeltaSeconds))
  (:Triggered
    (Variables|AnimCalls|SetIsBraking true)
    (Variables|Default|SetCurrentMomentum (Math|Vector|MakeVector (Math|Interpolation|FInterpTo (.x (Variables|Default|GetCurrentMomentum)) 0.0 _returnvalue 2.0) (Math|Interpolation|FInterpTo (.y (Variables|Default|GetCurrentMomentum)) 0.0 _returnvalue 2.0) 0.0)))
  (:Canceled
    (Variables|AnimCalls|SetIsBraking false :!label _label))
  (:Completed
    (goto _label)))

(event Input|EnhancedActionEvents|EnhancedInputActionIA_CamScroll
  (params (ActionValue :type Float%20%28double-precision%29) (ElapsedSeconds :type Float%20%28double-precision%29) (TriggeredSeconds :type Float%20%28double-precision%29) (InputAction :type Input%20Action%20Object%20Reference :default "/Game/Player/Input/IA_CamScroll.IA_CamScroll"))
  (bind _camera (Variables|Default|GetCamera))
  (Camera|SetFieldOfView _camera (Math|Float|Clamp(Float) (- (Variables|/Script/Engine.CameraComponent|GetFieldOfView _camera) (* ActionValue 3.0)) 6e+01 1e+02)))

(event EventTick
  (params (DeltaSeconds :type Float%20%28single-precision%29))
  (bind _currentmomentum (Variables|Default|GetCurrentMomentum))
  (bind _shipcontrol (Variables|Default|GetShipControl))
  (Utilities|FlowControl|Sequence
    (:then_0
      (Transformation|AddWorldOffset (Variables|Default|GetRoot%20Collision) (Math|Vector|MakeVector (* (.x _currentmomentum) _shipcontrol) (* (.y _currentmomentum) _shipcontrol) 0.0) false false))))

(event EventBeginPlay
  (bind _aspc_player (Utilities|Casting|CastToPC_Player (Game|GetPlayerController 0)))
  (Utilities|IsValid _aspc_player
    (:Is%20Valid
      (Utilities|IsValid (PlayerController|LocalPlayerSubsystems|GetEnhancedInputLocalPlayerSubsystem _aspc_player)
        (:Is%20Valid
          (Input|AddMappingContext (PlayerController|LocalPlayerSubsystems|GetEnhancedInputLocalPlayerSubsystem _aspc_player) "/Game/Player/Input/IMC_Player.IMC_Player" 0 "(bIgnoreAllPressedKeysUntilRelease=True,bForceImmediately=False,bNotifyUserSettings=False)")
          (Transformation|SetWorldTransform (Variables|Default|GetRoot%20Collision) (Math|Transform|MakeTransform "0, 0, 0" "0, 0, 0" "1.000000,1.000000,1.000000") false true)
          (Variables|Default|SetPlayerHealth (Variables|Default|GetPlayerMaxHealth))
          (bind _asgi_player (Utilities|Casting|CastToGI_Player (Game|GetGameInstance)))
          (Rendering|Components|TextRender|SetText (Variables|Default|GetPlayerName) (Variables|/Game/Player/GI_Player.GI_Player_C|GetPlayerName _asgi_player))
          (Transformation|SetWorldTransform (Variables|Default|GetRoot%20Collision) (Variables|Default|GetSpawnPoint) false true)
          (Utilities|Time|SetTimerbyEvent (delegate Custom|CapSpeed) 0.03 true true))))))

(fn ConstructionScript)

(fn TakeZoneDamage
  (Variables|Default|SetPlayerHealth (Math|Float|Clamp(Float) (- (Variables|Default|GetPlayerHealth) 0.006))))

(fn SubtractTemp
  (if (>= (Variables|Default|GetTemperature) 0.15)
    (Variables|Default|SetTemperature (Math|Float|Clamp(Float) (- (Variables|Default|GetTemperature) 0.05) 0.15))
    (else
      (Utilities|Time|ClearandInvalidateTimerbyHandle (Variables|Timers|GetT_SubtractTemp)))))