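; GM_Gamplay is the gameplay game mode that sets up the player's ship and HUD when play begins.
; BeginPlay hides the cursor, switches to game-only input and reads the ship class chosen in GI_Player, writing BP_StarterShip back as the fallback when none is valid.
; It spawns that ship at SpawnTransform, has the first player controller possess it, then adds WBP_Player_HUD to the viewport.
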(event EventBeginPlay
  (bind _returnvalue (Game|GetPlayerController 0))
  (Variables|/Script/Engine.PlayerController|SetbShowMouseCursor _returnvalue false)
  (Input|SetInputModeGameOnly _returnvalue false)
  (bind _asgi_player (Utilities|Casting|CastToGI_Player (Game|GetGameInstance)))
  (if (Utilities|IsValidClass (Variables|/Game/Player/GI_Player.GI_Player_C|GetShipSelection _asgi_player))
    _
    (else
      (Variables|/Game/Player/GI_Player.GI_Player_C|SetShipSelection _asgi_player "/Game/Player/Ships/Starter/BP_StarterShip.BP_StarterShip_C")))
  (bind _returnvalue_2 (Game|SpawnActorfromClass (Variables|/Game/Player/GI_Player.GI_Player_C|GetShipSelection _asgi_player) (Variables|Default|GetSpawnTransform) "Undefined" "MultiplyWithRoot" 0 0))
  (Pawn|Possess (Game|GetPlayerController 0) _returnvalue_2)
  (bind _returnvalue_3 (UserInterface|CreateWidget "/Game/Widgets/WBP_Player_HUD.WBP_Player_HUD_C"))
  (UserInterface|Viewport|AddtoViewport _returnvalue_3 5))

(fn ConstructionScript)