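; BP_HealthComponent is a player component that tracks health and reports damage and death.
; Health starts at MaxHealth on BeginPlay.
; TakeHealth subtracts an amount, clamps the result between zero and MaxHealth, then fires the Died dispatcher at zero or the Hit dispatcher otherwise.
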(event EventBeginPlay
  (Variables|Default|SetHealth (Variables|Default|GetMaxHealth)))

(fn TakeHealth
  (params (Amount :type Float%20%28double-precision%29))
  (bind _output_get (Variables|Default|SetHealth (Math|Float|Clamp(Float) (- (Variables|Default|GetHealth) Amount) 0.0 (Variables|Default|GetMaxHealth))))
  (if (== _output_get 0.0)
    (Default|CallDiedEventDispatcher)
    (else
      (Default|CallHitEventDispatcher))))