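; Player XP component for a ship that tracks XP and level, capped at level 10.
; Init builds the level threshold map and loads XP and level from player controller 0's profile.
; AddXP checks thresholds for level-ups, writes back to that profile and refreshes the local HUD.
; As wired, AddXP stores the XP sum in PlayerLevel, leaving PlayerXP unchanged and skewing the level check.
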(event Custom|XP_Component_Init
  (CallFunction|SetupXPMap)
  (bind _asbp_ship_base (Utilities|Casting|CastToBP_ShipBase (Components|GetOwner)))
  (Variables|Default|SetAs%20BP%20Ship%20Base _asbp_ship_base)
  (bind _asbp_standard_player_controller (Utilities|Casting|CastToBP_Standard_PlayerController (Game|GetPlayerController 0)))
  (bind _output_get (Variables|Default|SetAs%20BP%20Standard%20Player%20Controller _asbp_standard_player_controller))
  (Variables|Default|SetPlayer%20XP (.player_xp (Variables|/Game/Framework/BP_Standard_PlayerController.BP_Standard_PlayerController_C|GetS_PlayerProfile _output_get)))
  (Variables|Default|SetPlayer%20Level (.player_level (Variables|/Game/Framework/BP_Standard_PlayerController.BP_Standard_PlayerController_C|GetS_PlayerProfile _output_get)))
  (if (Pawn|IsLocalPlayerController (Variables|Default|GetAs%20BP%20Standard%20Player%20Controller))
    (Default|UpdateXPAmount (Variables|/Game/Framework/BP_Standard_PlayerController.BP_Standard_PlayerController_C|GetWPB_HUD (Variables|Default|GetAs%20BP%20Standard%20Player%20Controller)))
    (Default|UpdateXPLevel (Variables|/Game/Framework/BP_Standard_PlayerController.BP_Standard_PlayerController_C|GetWPB_HUD (Variables|Default|GetAs%20BP%20Standard%20Player%20Controller)))))

(event Custom|AddXP
  (params (XP%20Amount :type Integer))
  (bind _as_bp_ship_base (Variables|Default|GetAs%20BP%20Ship%20Base))
  (bind _wpb_hud (Variables|/Game/Player/BP_ShipBase.BP_ShipBase_C|GetWPB%20HUD _as_bp_ship_base))
  (bind _output_get (Variables|Default|SetPlayer%20Level (+ XP%20Amount (Variables|Default|GetPlayer%20XP))))
  (bind (_canlevelup _newlevel) (CallFunction|CheckforLevelUp _output_get))
  (if _canlevelup
    (Variables|Default|SetPlayer%20Level _newlevel))
  (CallFunction|UpdatePlayerControllerProfile)
  (if (Pawn|IsLocallyControlled _as_bp_ship_base)
    (Default|UpdateXPAmount _wpb_hud)
    (Default|UpdateXPLevel _wpb_hud)))

(fn SetupXPMap
  (Variables|Default|SetXP_Map_Levels (.xp_map_levels (LocalVariables|GetS_XPandLevel)))
  (return))

(fn CheckforLevelUp
  (params (XPAmount :type Integer))
  (LocalVariables|SetLcl_CurrentPlayerXP XPAmount)
  (LocalVariables|SetLcl_CurrentPlayerLevel (Variables|Default|GetPlayer%20Level))
  (if (and (> (LocalVariables|GetLcl_CurrentPlayerXP) (Utilities|Array|Get(acopy) (Variables|Default|GetXP_Map_Levels) (LocalVariables|GetLcl_CurrentPlayerLevel))) (< (LocalVariables|GetLcl_CurrentPlayerLevel) 10))
    (LocalVariables|SetLcl_CanLevelUp true)
    (bind _index (Utilities|FlowControl|ForLoopwithBreak (LocalVariables|GetLcl_CurrentPlayerLevel) 10 :!label _label)
      (:LoopBody
        (if (not (> (LocalVariables|GetLcl_CurrentPlayerXP) (Utilities|Array|Get(acopy) (Variables|Default|GetXP_Map_Levels) _index)))
          (LocalVariables|SetLcl_CurrentPlayerLevel _index)
          (goto _label Break)))
      (:Completed
        (return (LocalVariables|GetLcl_CanLevelUp) (LocalVariables|GetLcl_CurrentPlayerLevel))))
    (else
      (LocalVariables|SetLcl_CanLevelUp false)
      (return (LocalVariables|GetLcl_CanLevelUp) (LocalVariables|GetLcl_CurrentPlayerLevel)))))

(fn UpdatePlayerControllerProfile
  (bind _as_bp_standard_player_controller (Variables|Default|GetAs%20BP%20Standard%20Player%20Controller))
  (Variables|/Game/Framework/BP_Standard_PlayerController.BP_Standard_PlayerController_C|SetS_PlayerProfile _as_bp_standard_player_controller (Utilities|Struct|MakeS_PlayerProfile (.playername (Variables|/Game/Framework/BP_Standard_PlayerController.BP_Standard_PlayerController_C|GetS_PlayerProfile _as_bp_standard_player_controller)) (.characterrowname (Variables|/Game/Framework/BP_Standard_PlayerController.BP_Standard_PlayerController_C|GetS_PlayerProfile _as_bp_standard_player_controller)) (.characterclass (Variables|/Game/Framework/BP_Standard_PlayerController.BP_Standard_PlayerController_C|GetS_PlayerProfile _as_bp_standard_player_controller)) (Variables|Default|GetPlayer%20XP) (Variables|Default|GetPlayer%20Level)))
  (return))