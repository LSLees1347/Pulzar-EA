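; BP_SharkChomp is a short-lived hit actor for the Shark ship's chomp ability.
; It destroys itself after a brief lifetime, or shortly after overlapping an actor other than its instigator.
; On such an overlap, Svr_ApplyDamage deals base damage credited to the instigator and MC_DestroyedEffect spawns a scaled-down hit effect, their names suggesting server and multicast RPCs.
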(event Custom|Svr_ApplyDamage
  (params (DamagedActor :type Actor%20Object%20Reference))
  (Game|Damage|ApplyDamage DamagedActor (Variables|Default|GetBase%20Damage) 0 (Game|GetInstigator)))

(event Custom|MC_DestroyedEffect
  (Niagara|SpawnSystematLocation (Variables|Default|GetHitEffect) (Transformation|GetActorLocation) "0, 0, 0" "0.700000,0.700000,0.700000"))

(event EventBeginPlay
  (Utilities|FlowControl|Delay 0.45)
  (Actor|DestroyActor))

(event Collision|EventActorBeginOverlap
  (params (OtherActor :type Actor%20Object%20Reference))
  (if (not (== (Game|GetInstigator) OtherActor))
    (CallFunction|SvrApplyDamage OtherActor)
    (CallFunction|MCDestroyedEffect)
    (Utilities|FlowControl|Delay 0.3)
    (Actor|DestroyActor)))

(fn ConstructionScript)