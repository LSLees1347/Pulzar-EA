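; Shark ship ability actor: a tornado projectile that snaps to its instigator on spawn and damages the first other actor it overlaps.
; LaunchTornado adds the instigator's horizontal momentum to its speed, then a roughly 60 Hz looping timer pushes it along local X.
; Damage goes through a Svr_ event and destroys it immediately.
; The MC_ hit effect plays only when its duration expires.
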(event Custom|Svr_ApplyDamage
  (params (DamagedActor :type Actor%20Object%20Reference))
  (Game|Damage|ApplyDamage DamagedActor (Variables|Default|GetBase%20Damage) 0 (Game|GetInstigator)))

(event Custom|MC_DestroyedEffect
  (Niagara|SpawnSystematLocation (Variables|Default|GetHitEffect) (Transformation|GetActorLocation)))

(event Custom|LaunchTornado
  (bind _lcl_newspeed (CallFunction|CalcMomentum))
  (Variables|Default|SetSpeed (+ _lcl_newspeed (Variables|Default|GetSpeed)))
  (Utilities|Time|SetTimerbyEvent (delegate Custom|Add%20Actor%20Offset) 0.016667 true)
  (Utilities|FlowControl|Delay (Variables|Default|GetDuration))
  (CallFunction|MCDestroyedEffect)
  (Actor|DestroyActor))

(event Custom|Add%20Actor%20Offset
  (Transformation|AddActorLocalOffset (Math|Vector|MakeVector (Variables|Default|GetSpeed) 0.0 0.0) false false))

(event EventBeginPlay
  (Transformation|AttachActorToActor (Game|GetInstigator) "None" "SnapToTarget" "SnapToTarget" "SnapToTarget" true))

(event Collision|EventActorBeginOverlap
  (params (OtherActor :type Actor%20Object%20Reference))
  (if (not (== (Game|GetInstigator) OtherActor))
    (CallFunction|SvrApplyDamage OtherActor)
    (Actor|DestroyActor)))

(fn ConstructionScript)

(fn CalcMomentum
  (bind _returnvalue (Game|GetInstigator))
  (bind _returnvalue_2 (Transformation|GetVelocity _returnvalue))
  (LocalVariables|SetLcl_X (.x _returnvalue_2))
  (LocalVariables|SetLcl_Y (.y _returnvalue_2))
  (if (< (LocalVariables|GetLcl_X) 0.0)
    (LocalVariables|SetLcl_X (* (LocalVariables|GetLcl_X) -1.0)))
  (if (< (LocalVariables|GetLcl_Y) 0.0)
    (LocalVariables|SetLcl_Y (* (LocalVariables|GetLcl_Y) -1.0)))
  (LocalVariables|SetLcl_Nspeed (/ (+ (LocalVariables|GetLcl_X) (LocalVariables|GetLcl_Y)) 5e+01))
  (return (LocalVariables|GetLcl_Nspeed)))