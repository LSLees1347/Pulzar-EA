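; Shark player ship with a chomp primary, a chargeable SharkNado secondary and a stubbed invisibility tertiary.
; Holding secondary grows a preview tornado; release past a minimum charge spawns BP_SharkNado at that scale.
; Primary and secondary route through Svr events to MC events that spawn the actors, with DoOnce cooldowns and HUD timelines.
; Tertiary calls the empty MC_Invisibity directly, bypassing its Svr event, then waits out duration and cooldown.
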(event Custom|Svr_Invisibity
  (CallFunction|MCInvisibity))

(event Custom|MC_Invisibity)

(event Custom|MC_PrimaryFire
  (params (Spawn%20Transform%20Location :type Vector) (Spawn%20Transform%20Rotation :type Rotator))
  (bind _self self)
  (Game|SpawnActorfromClass "/Game/Player/Ships/Shark/Abilities/BP_SharkChomp.BP_SharkChomp_C" (Math|Transform|MakeTransform Spawn%20Transform%20Location Spawn%20Transform%20Rotation "1.000000,1.000000,1.000000") "Undefined" "MultiplyWithRoot" _self _self))

(event Custom|Svr_PrimaryFire
  (bind _sprite (Variables|Default|GetSprite))
  (bind _returnvalue (Math|Vector|GetForwardVector _sprite))
  (CallFunction|MCPrimaryFire (+ (Transformation|GetWorldLocation _sprite) (* (Math|Vector|MakeVector (.x _returnvalue) (.y _returnvalue) 0.0) 1.5e+02)) (Math|Conversions|RotationFromXVector (Math|Vector|GetForwardVector (Variables|Default|GetSprite)))))

(event Custom|Svr_SecondaryFire
  (params (Spawn%20Transform%20Scale :type Vector))
  (bind _sprite (Variables|Default|GetSprite))
  (bind _returnvalue (Math|Vector|GetForwardVector _sprite))
  (CallFunction|MCSecondaryFire (+ (Transformation|GetWorldLocation _sprite) (* (Math|Vector|MakeVector (.x _returnvalue) (.y _returnvalue) 0.0) "")) (Math|Conversions|RotationFromXVector (Math|Vector|GetForwardVector (Variables|Default|GetSprite))) Spawn%20Transform%20Scale))

(event Custom|MC_SecondaryFire
  (params (Spawn%20Transform%20Location :type Vector) (Spawn%20Transform%20Rotation :type Rotator) (Spawn%20Transform%20Scale :type Vector))
  (bind _self self)
  (bind _returnvalue (Game|SpawnActorfromClass "/Game/Player/Ships/Shark/Abilities/BP_SharkNado.BP_SharkNado_C" (Math|Transform|MakeTransform Spawn%20Transform%20Location Spawn%20Transform%20Rotation Spawn%20Transform%20Scale) "Undefined" "MultiplyWithRoot" _self _self))
  (Variables|Default|SetA_Tornado _returnvalue))

(event Input|EnhancedActionEvents|EnhancedInputActionIA_Tertiary
  (params (ActionValue :type Boolean) (ElapsedSeconds :type Float%20%28double-precision%29) (TriggeredSeconds :type Float%20%28double-precision%29) (InputAction :type Input%20Action%20Object%20Reference :default "/Game/Player/Input/IA_Tertiary.IA_Tertiary"))
  (:Started
    (Utilities|FlowControl|DoOnce false :!label _label
      (:Completed
        (CallFunction|MCInvisibity)
        (Utilities|FlowControl|Delay (Variables|Default|GetTertiaryDuration))
        (Utilities|FlowControl|Delay (Variables|Default|GetTertiaryCooldown))
        (goto _label Reset)))))

(event Input|EnhancedActionEvents|EnhancedInputActionIA_Primary
  (params (ActionValue :type Float%20%28double-precision%29) (ElapsedSeconds :type Float%20%28double-precision%29) (TriggeredSeconds :type Float%20%28double-precision%29) (InputAction :type Input%20Action%20Object%20Reference :default "/Game/Player/Input/IA_Primary.IA_Primary"))
  (Utilities|FlowControl|DoOnce false :!label _label
    (:Completed
      (CallFunction|SvrPrimaryFire)
      (bind _cooldown (Timeline|PrimaryCooldown PlayFromStart)
        (:Update
          (Default|Ability1Cooldown (Variables|Default|GetWPB%20HUD) _cooldown))
        (:Finished
          (goto _label Reset))))))

(event Input|EnhancedActionEvents|EnhancedInputActionIA_Secondary
  (params (ActionValue :type Float%20%28double-precision%29) (ElapsedSeconds :type Float%20%28double-precision%29) (TriggeredSeconds :type Float%20%28double-precision%29) (InputAction :type Input%20Action%20Object%20Reference :default "/Game/Player/Input/IA_Secondary.IA_Secondary"))
  (bind _torn (Variables|Default|GetTorn))
  (:Started
    (Utilities|FlowControl|DoOnce false :!label _label
      (:Completed
        (Rendering|SetVisibility (Variables|Default|GetTorn) true false)
        (bind _scaleup (Timeline|ResizeTorn PlayFromStart)
          (:Update
            (Transformation|SetWorldScale3D (Variables|Default|GetTorn) (Math|Vector|MakeVector (Math|Float|Lerp 0.0 1.0 _scaleup) (Math|Float|Lerp 0.0 1.0 _scaleup) (Math|Float|Lerp 0.0 1.0 _scaleup)))
            (Variables|Default|SetLerpAlpha (Math|Float|Lerp 0.0 1.0 _scaleup))
            (bind _cooldown (Timeline|Timeline PlayFromStart)
              (:Update
                (Default|Ability2Cooldown (Variables|Default|GetWPB%20HUD) _cooldown))))))))
  (:Completed
    (Utilities|FlowControl|Sequence
      (:then_0
        (Timeline|ResizeTorn Stop))
      (:then_1
        (Rendering|SetVisibility _torn false false)
        (Transformation|SetWorldScale3D _torn (Math|Vector|MakeVector 0.0 0.0 0.0))
        (if (> (Variables|Default|GetLerpAlpha) 0.3)
          (CallFunction|SvrSecondaryFire (Math|Vector|MakeVector (Variables|Default|GetLerpAlpha) (Variables|Default|GetLerpAlpha) (Variables|Default|GetLerpAlpha)))
          (Variables|Default|SetLerpAlpha 0.0)
          (Utilities|FlowControl|Delay (Variables|Default|GetSecondaryFireRate))
          (goto _label Reset)
          (else
            (goto _label Reset)))))))

(event EventBeginPlay
  (|CallParentFunction) ; This node is disabled and will not be called.\nDrag off pins to build functionality.
)

(fn ConstructionScript
  (|CallParentFunction))