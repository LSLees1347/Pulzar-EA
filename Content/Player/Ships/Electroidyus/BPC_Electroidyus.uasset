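; Electroidyus player ship Blueprint that adds an area-of-effect secondary attack against asteroids.
; Secondary input enables the AOE collision for a brief timed window, with a flag blocking retriggers until it ends.
; The end of the window reuses the BeginPlay reset that disables collision and clears the flag.
; Any BP_AsteroidBase that begins overlapping the AOE receives a Hit call, with debug prints on hit and shutdown.
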(event OnComponentBeginOverlap(AOE_Colision)
  (params (OverlappedComponent :type Primitive%20Component%20Object%20Reference) (OtherActor :type Actor%20Object%20Reference) (OtherComp :type Primitive%20Component%20Object%20Reference) (OtherBodyIndex :type Integer) (bFromSweep :type Boolean) (SweepResult :type Hit%20Result%20Structure%20%28by%20ref%29))
  (bind _asbp_asteroid_base (Utilities|Casting|CastToBP_AsteroidBase OtherActor))
  (Default|Hit _asbp_asteroid_base)
  (Development|PrintString "hit"))

(event Input|EnhancedActionEvents|EnhancedInputActionIA_Secondary
  (params (ActionValue :type Float%20%28double-precision%29) (ElapsedSeconds :type Float%20%28double-precision%29) (TriggeredSeconds :type Float%20%28double-precision%29) (InputAction :type Input%20Action%20Object%20Reference :default "/Game/Player/Input/IA_Secondary.IA_Secondary"))
  (bind _aoe_colision (Variables|Default|GetAOE_Colision))
  (:Triggered
    (if (not (Variables|Default|GetIsAOEattacking))
      (Variables|Default|SetIsAOEattacking true)
      (Collision|SetCollisionEnabled _aoe_colision "QueryAndPhysics")
      (Utilities|FlowControl|Delay 1.0)
      (Development|PrintString "disabled")
      (Collision|SetCollisionEnabled _aoe_colision "NoCollision")
      (Variables|Default|SetIsAOEattacking false))))

(event EventBeginPlay
  (|CallParentFunction)
  (Collision|SetCollisionEnabled (Variables|Default|GetAOE_Colision) "NoCollision")
  (Variables|Default|SetIsAOEattacking false))

(event Collision|EventActorBeginOverlap
  (params (OtherActor :type Actor%20Object%20Reference)))

(event EventTick
  (params (DeltaSeconds :type Float%20%28single-precision%29))
  (|CallParentFunction DeltaSeconds) ; This node is disabled and will not be called.\nDrag off pins to build functionality.
)

(fn ConstructionScript
  (|CallParentFunction))