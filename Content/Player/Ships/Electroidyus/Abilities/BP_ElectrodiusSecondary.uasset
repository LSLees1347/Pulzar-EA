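; BP_ElectrodiusSecondary is a short-lived damage actor for the secondary ability of the Electrodius player ship.
; On overlapping any actor other than its instigator, it calls a server damage event and destroys itself.
; That event applies its base damage with a slow damage type, naming the instigator as damage causer.
; Without a hit, it destroys itself after a fraction of a second.
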(event Custom|Svr_ApplyDamage
  (params (DamagedActor :type Actor%20Object%20Reference))
  (Game|Damage|ApplyDamage DamagedActor (Variables|Default|GetBase%20Damage) 0 (Game|GetInstigator) "/Game/Player/Damage/Slow/DamageType_Slow.DamageType_Slow_C"))

(event EventBeginPlay
  (Utilities|FlowControl|Delay 0.2)
  (Actor|DestroyActor))

(event Collision|EventActorBeginOverlap
  (params (OtherActor :type Actor%20Object%20Reference))
  (if (not (== OtherActor (Game|GetInstigator)))
    (CallFunction|SvrApplyDamage OtherActor)
    (Actor|DestroyActor)))

(fn ConstructionScript)