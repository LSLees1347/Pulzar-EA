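; Ghost player ship with three abilities: a primary shot, a bomb and a timed invisibility.
; Inputs call Server events that relay to Multicast events, which spawn projectiles or hide the sprite between burst effects, leaving an attached trail.
; DoOnce gates stay locked until cooldown Timelines, which also drive the HUD, finish.
; Invisibility blocks both attacks for its duration, then starts its cooldown.
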(event Custom|Svr_Invisibity
  (CallFunction|MCInvisibity))

(event Custom|MC_Invisibity
  (Niagara|SpawnSystemAttached "/Game/Player/Ships/Ghost/Abilities/NS_InvisBoom.NS_InvisBoom" (Variables|Default|GetSprite) "None" "0, 0, 0" "0, 0, 0" "SnapToTarget" true)
  (Rendering|SetVisibility (Variables|Default|GetSprite) false false)
  (bind _returnvalue (Niagara|SpawnSystemAttached "/Game/Player/Ships/Ghost/Abilities/NS_InvisTrail.NS_InvisTrail" (Variables|Default|GetSprite) "None" "0, 0, 0" "0, 0, 0" "SnapToTarget" true))
  (Utilities|FlowControl|Delay (Variables|Default|GetInvisDuration))
  (Components|DestroyComponent _returnvalue)
  (Niagara|SpawnSystemAttached "/Game/Player/Ships/Ghost/Abilities/NS_InvisBoom.NS_InvisBoom" (Variables|Default|GetSprite) "None" "0, 0, 0" "0, 0, 0" "SnapToTarget" true)
  (Rendering|SetVisibility (Variables|Default|GetSprite) true false))

(event Custom|MC_SecondaryFire
  (params (Spawn%20Transform%20Location :type Vector) (Spawn%20Transform%20Rotation :type Rotator))
  (bind _self self)
  (Game|SpawnActorfromClass "/Game/Player/Ships/Ghost/Abilities/BP_GhostBomb.BP_GhostBomb_C" (Math|Transform|MakeTransform Spawn%20Transform%20Location Spawn%20Transform%20Rotation "1.000000,1.000000,1.000000") "Undefined" "MultiplyWithRoot" _self _self))

(event Custom|Svr_SecondaryFire
  (bind _sprite (Variables|Default|GetSprite))
  (bind _returnvalue (Math|Vector|GetForwardVector _sprite))
  (CallFunction|MCSecondaryFire (+ (Transformation|GetWorldLocation _sprite) (* (Math|Vector|MakeVector (.x _returnvalue) (.y _returnvalue) 0.0) (Variables|Default|GetFiringStartDistanceFromSelf))) (Math|Conversions|RotationFromXVector (Math|Vector|GetForwardVector (Variables|Default|GetSprite)))))

(event Custom|MC_PrimaryFire
  (params (Spawn%20Transform%20Location :type Vector) (Spawn%20Transform%20Rotation :type Rotator))
  (bind _self self)
  (Game|SpawnActorfromClass "/Game/Player/Ships/Ghost/Abilities/BP_GhostPrimary.BP_GhostPrimary_C" (Math|Transform|MakeTransform Spawn%20Transform%20Location Spawn%20Transform%20Rotation "0.100000,0.100000,0.100000") "Undefined" "MultiplyWithRoot" _self _self))

(event Custom|Svr_PrimaryFire
  (bind _sprite (Variables|Default|GetSprite))
  (bind _returnvalue (Math|Vector|GetForwardVector _sprite))
  (CallFunction|MCPrimaryFire (+ (Transformation|GetWorldLocation _sprite) (* (Math|Vector|MakeVector (.x _returnvalue) (.y _returnvalue) 0.0) (Variables|Default|GetFiringStartDistanceFromSelf))) (Math|Conversions|RotationFromXVector (Math|Vector|GetForwardVector (Variables|Default|GetSprite)))))

(event Input|EnhancedActionEvents|EnhancedInputActionIA_Tertiary
  (params (ActionValue :type Boolean) (ElapsedSeconds :type Float%20%28double-precision%29) (TriggeredSeconds :type Float%20%28double-precision%29) (InputAction :type Input%20Action%20Object%20Reference :default "/Game/Player/Input/IA_Tertiary.IA_Tertiary"))
  (:Started
    (Utilities|FlowControl|DoOnce false :!label _label
      (:Completed
        (Variables|Default|SetCanFire? false)
        (CallFunction|SvrInvisibity)
        (Default|Ability3Cooldown (Variables|Default|GetWPB%20HUD) 0.0)
        (Utilities|FlowControl|Delay (Variables|Default|GetInvisDuration))
        (Variables|Default|SetCanFire? true)
        (bind _ability3 (Timeline|Ability3Cooldown PlayFromStart)
          (:Update
            (Default|Ability3Cooldown (Variables|Default|GetWPB%20HUD) _ability3))
          (:Finished
            (goto _label Reset)))))))

(event Input|EnhancedActionEvents|EnhancedInputActionIA_Primary
  (params (ActionValue :type Float%20%28double-precision%29) (ElapsedSeconds :type Float%20%28double-precision%29) (TriggeredSeconds :type Float%20%28double-precision%29) (InputAction :type Input%20Action%20Object%20Reference :default "/Game/Player/Input/IA_Primary.IA_Primary"))
  (if (Variables|Default|GetCanFire?)
    (Utilities|FlowControl|DoOnce false :!label _label
      (:Completed
        (CallFunction|SvrPrimaryFire)
        (bind _ability1 (Timeline|Ability1Cooldown PlayFromStart)
          (:Update
            (Default|Ability1Cooldown (Variables|Default|GetWPB%20HUD) _ability1))
          (:Finished
            (goto _label Reset)))))))

(event Input|EnhancedActionEvents|EnhancedInputActionIA_Secondary
  (params (ActionValue :type Float%20%28double-precision%29) (ElapsedSeconds :type Float%20%28double-precision%29) (TriggeredSeconds :type Float%20%28double-precision%29) (InputAction :type Input%20Action%20Object%20Reference :default "/Game/Player/Input/IA_Secondary.IA_Secondary"))
  (if (Variables|Default|GetCanFire?)
    (Utilities|FlowControl|DoOnce false :!label _label
      (:Completed
        (CallFunction|SvrSecondaryFire)
        (bind _ability2 (Timeline|Ability2Cooldown PlayFromStart)
          (:Update
            (Default|Ability2Cooldown (Variables|Default|GetWPB%20HUD) _ability2))
          (:Finished
            (goto _label Reset)))))))

(event EventBeginPlay
  (|CallParentFunction) ; This node is disabled and will not be called.\nDrag off pins to build functionality.
)

(fn ConstructionScript
  (|CallParentFunction))