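; BP_BasicJet is a player jet Blueprint that handles shooting and thruster smoke through Enhanced Input.
; IA_Shoot spawns a BP_BJet_Bullets actor on each press, using the Sprite's world X and Y and its relative rotation.
; IA_Thrusters switches the left and right smoke effects on when started and off when completed.
; The file contains no movement logic, and its BeginPlay, overlap and Tick events are disabled stubs.
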(event Input|EnhancedActionEvents|EnhancedInputActionIA_Shoot
  (params (ActionValue :type Float%20%28double-precision%29) (ElapsedSeconds :type Float%20%28double-precision%29) (TriggeredSeconds :type Float%20%28double-precision%29) (InputAction :type Input%20Action%20Object%20Reference :default "/Game/Player/Input/IA_Shoot.IA_Shoot"))
  (bind _sprite (Variables|Default|GetSprite))
  (bind _returnvalue (Transformation|GetWorldLocation _sprite))
  (:Started
    (Game|SpawnActorfromClass "/Game/Player/Ships/BasicJet/BP_BJet_Bullets.BP_BJet_Bullets_C" (Math|Transform|MakeTransform (Math|Vector|MakeVector (.x _returnvalue) (.y _returnvalue) 0.0) (Variables|/Script/Engine.SceneComponent|GetRelativeRotation _sprite) "1.000000,1.000000,1.000000") "Undefined" "MultiplyWithRoot" 0 0)))

(event Input|EnhancedActionEvents|EnhancedInputActionIA_Thrusters
  (params (ActionValue :type Float%20%28double-precision%29) (ElapsedSeconds :type Float%20%28double-precision%29) (TriggeredSeconds :type Float%20%28double-precision%29) (InputAction :type Input%20Action%20Object%20Reference :default "/Game/Player/Input/IA_Thrusters.IA_Thrusters"))
  (bind _r_smoke (Variables|Default|GetR_Smoke))
  (:Started
    (Components|Activation|SetActive _r_smoke true false))
  (:Completed
    (Components|Activation|SetActive _r_smoke false false)))

(event EventBeginPlay
  (|CallParentFunction) ; This node is disabled and will not be called.\nDrag off pins to build functionality.
)

(event Collision|EventActorBeginOverlap
  (params (OtherActor :type Actor%20Object%20Reference)))

(event EventTick
  (params (DeltaSeconds :type Float%20%28single-precision%29))
  (|CallParentFunction DeltaSeconds) ; This node is disabled and will not be called.\nDrag off pins to build functionality.
)

(fn ConstructionScript
  (|CallParentFunction))