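; BP_BJet_Bullets is a projectile actor for the basic jet player ship.
; Each tick it offsets its Sprite in X and Y along the sprite's forward vector by BulletSpeed, without scaling by delta time.
; On BeginPlay it waits for LifeSpan and then destroys itself.
; A cast that would store the player's BP_BasicJet reference is present but never runs.
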(event EventTick
  (params (DeltaSeconds :type Float%20%28single-precision%29))
  (bind _sprite (Variables|Default|GetSprite))
  (bind _bulletspeed (Variables|Default|GetBulletSpeed))
  (bind _returnvalue (Math|Vector|GetForwardVector _sprite))
  (Transformation|AddWorldOffset _sprite (Math|Vector|MakeVector (+ (* (.x _returnvalue) _bulletspeed) 0.0) (+ (* (.y _returnvalue) _bulletspeed) 0.0) 0.0) false false))

(event EventBeginPlay
  (Utilities|FlowControl|Delay (Variables|Default|GetLifeSpan))
  (Actor|DestroyActor))

(fn ConstructionScript)