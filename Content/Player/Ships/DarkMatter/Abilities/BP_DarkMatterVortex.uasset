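; Dark matter ship ability projectile: a vortex that moves at a set velocity and damages actors it overlaps, except its instigator, with a slow damage type.
; A timeline drives its X/Y scale, then triggers a Niagara explosion and destroys the actor.
; Damage and explosion go through server and multicast events, judging by their names.
; CalcMomentum derives a speed from the instigator's velocity but is not called here.
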(event Custom|Svr_ApplyDamage
  (params (DamagedActor :type Actor%20Object%20Reference))
  (Game|Damage|ApplyDamage DamagedActor (Variables|Default|GetBase%20Damage) 0 (Game|GetInstigator) "/Game/Player/Damage/Slow/DamageType_Slow.DamageType_Slow_C"))

(event Custom|MC_DestroyedEffect
  (Niagara|SpawnSystematLocation "/Game/Player/Ships/DarkMatter/NS_DM_BigExplosion.NS_DM_BigExplosion" (Transformation|GetActorLocation) "0, 0, 0" (Math|Vector|MakeVector 0.5 0.5 0.5)))

(event Collision|EventActorBeginOverlap
  (params (OtherActor :type Actor%20Object%20Reference))
  (if (not (== (Game|GetInstigator) OtherActor))
    (CallFunction|SvrApplyDamage OtherActor)))

(event EventBeginPlay
  (Variables|/Script/Engine.MovementComponent|SetVelocity (Variables|Default|GetProjectileMovement) (Variables|Default|GetVelocity))
  (bind _size (Timeline|Reduce PlayFromStart)
    (:Update
      (Transformation|SetActorScale3D (Math|Vector|MakeVector _size _size 0.0)))
    (:Finished
      (CallFunction|MCDestroyedEffect)
      (Actor|DestroyActor))))

(fn ConstructionScript)

(fn CalcMomentum
  (bind _returnvalue (Game|GetInstigator))
  (bind _returnvalue_2 (Transformation|GetVelocity _returnvalue))
  (LocalVariables|SetLcl_X (.x _returnvalue_2))
  (LocalVariables|SetLcl_Y (.y _returnvalue_2))
  (if (< (LocalVariables|GetLcl_X) 0.0)
    (LocalVariables|SetLcl_X (* (LocalVariables|GetLcl_X) -1.0)))
  (if (< (LocalVariables|GetLcl_Y) 0.0)
    (LocalVariables|SetLcl_Y (* (LocalVariables|GetLcl_Y) -1.0)))
  (LocalVariables|SetLcl_NewSpeed (/ (+ (LocalVariables|GetLcl_X) (LocalVariables|GetLcl_Y)) 5e+01))
  (return (LocalVariables|GetLcl_NewSpeed)))