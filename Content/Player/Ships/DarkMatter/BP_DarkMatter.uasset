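; BP_DarkMatter is a player ship whose secondary ability fires an attached BP_DM_Beam along the sprite's forward direction.
; A timeline reverses while firing to drive the HUD ability bar, and input release or timeline completion ends the beam.
; After a delay it plays forward, then DoOnce gates re-arm the ability.
; The locally controlled ship spawns and destroys the beam directly with authority, otherwise through server events.
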(event Custom|SecondaryFire_Start
  (bind _self self)
  (bind _sprite (Variables|Default|GetSprite))
  (bind _returnvalue (Math|Vector|GetForwardVector _sprite))
  (if (Pawn|IsLocallyControlled)
    (Networking|SwitchHasAuthority
      (:Authority
        (bind _returnvalue_2 (Game|SpawnActorfromClass "/Game/Player/Ships/DarkMatter/Abilities/BP_DM_Beam.BP_DM_Beam_C" (Math|Transform|MakeTransform (+ (Transformation|GetWorldLocation _sprite) (* (Math|Vector|MakeVector (.x _returnvalue) (.y _returnvalue) 0.0) (Variables|Default|GetFiringStartDistanceFromSelf))) (Math|Conversions|RotationFromXVector (Math|Vector|GetForwardVector (Variables|Default|GetSprite))) "1.000000,1.000000,1.000000") "Undefined" "MultiplyWithRoot" _self _self))
        (bind _output_get (Variables|Default|SetBeamREF _returnvalue_2))
        (Transformation|AttachActorToActor _output_get self "None" "SnapToTarget" "SnapToTarget" "SnapToTarget" true))
      (:Remote
        (CallFunction|SvrSecondaryFireStart)))))

(event Custom|SecondaryFire_End
  (if (Pawn|IsLocallyControlled)
    (Networking|SwitchHasAuthority
      (:Authority
        (Actor|DestroyActor (Variables|Default|GetBeamREF)))
      (:Remote
        (CallFunction|SVRSecondaryFireEnd)))))

(event Custom|Svr_SecondaryFire_Start
  (bind _self self)
  (bind _sprite (Variables|Default|GetSprite))
  (bind _returnvalue (Math|Vector|GetForwardVector _sprite))
  (bind _returnvalue_2 (Game|SpawnActorfromClass "/Game/Player/Ships/DarkMatter/Abilities/BP_DM_Beam.BP_DM_Beam_C" (Math|Transform|MakeTransform (+ (Transformation|GetWorldLocation _sprite) (* (Math|Vector|MakeVector (.x _returnvalue) (.y _returnvalue) 0.0) (Variables|Default|GetFiringStartDistanceFromSelf))) (Math|Conversions|RotationFromXVector (Math|Vector|GetForwardVector (Variables|Default|GetSprite))) "1.000000,1.000000,1.000000") "Undefined" "MultiplyWithRoot" _self _self))
  (bind _output_get (Variables|Default|SetBeamREF _returnvalue_2))
  (Transformation|AttachActorToActor _output_get self "None" "SnapToTarget" "SnapToTarget" "SnapToTarget" true))

(event Custom|SVR_SecondaryFire_End
  (Actor|DestroyActor (Variables|Default|GetBeamREF)))

(event Input|EnhancedActionEvents|EnhancedInputActionIA_Secondary
  (params (ActionValue :type Float%20%28double-precision%29) (ElapsedSeconds :type Float%20%28double-precision%29) (TriggeredSeconds :type Float%20%28double-precision%29) (InputAction :type Input%20Action%20Object%20Reference :default "/Game/Player/Input/IA_Secondary.IA_Secondary"))
  (:Triggered
    (Utilities|FlowControl|DoOnce false :!label _label
      (:Completed
        (CallFunction|SecondaryFireStart)
        (bind (_direction _ability2) (Timeline|Timeline ReverseFromEnd)
          (:Update
            (Default|Ability2Cooldown (Variables|Default|GetWPB%20HUD) _ability2))
          (:Finished
            (switch Utilities|FlowControl|Switch|SwitchonETimelineDirection _direction
              (:Forward
                (Utilities|FlowControl|Sequence
                  (:then_0
                    (goto _label Reset))
                  (:then_1
                    (goto _label_2 Reset))))
              (:Backward
                (Utilities|FlowControl|DoOnce false :!label _label_2
                  (:Completed
                    (CallFunction|SecondaryFireEnd)
                    (Utilities|FlowControl|Sequence
                      (:then_0
                        (Timeline|Timeline Stop))
                      (:then_1
                        (Utilities|FlowControl|Delay 8.5)
                        (Timeline|Timeline Play))))))))))))
  (:Canceled
    (goto _label_2))
  (:Completed
    (goto _label_2)))

(event EventBeginPlay
  (|CallParentFunction) ; This node is disabled and will not be called.\nDrag off pins to build functionality.
)

(fn ConstructionScript
  (|CallParentFunction))