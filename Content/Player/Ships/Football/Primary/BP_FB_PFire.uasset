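; Primary-fire projectile for the Football player ship.
; On spawn it sets its planar velocity from Speed plus 70% of an inherited velocity, then expires after Duration.
; Overlapping any actor except its instigator or expiring triggers a multicast hit effect and destroys it.
; A server damage event and a CalcMomentum helper based on instigator velocity are defined but not called here.
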(event Custom|Svr_ApplyDamage
  (params (DamagedActor :type Actor%20Object%20Reference))
  (Game|Damage|ApplyDamage DamagedActor (Variables|Default|GetBase%20Damage) 0 (Game|GetInstigator) (Variables|Default|GetDamage%20Type%20Class)))

(event Custom|MC_DestroyedEffect
  (Niagara|SpawnSystematLocation (Variables|Default|GetHitEffect) (Transformation|GetActorLocation) "0, 0, 0" (Variables|Default|GetHitSize)))

(event EventBeginPlay
  (bind _speed (Variables|Default|GetSpeed))
  (Variables|/Script/Engine.MovementComponent|SetVelocity (Variables|Default|GetProjectileMovement) (+ (* (Variables|Default|GetFVector) (Math|Vector|MakeVector _speed _speed 0.0)) (* (Variables|Default|GetVelocity) (Math|Vector|MakeVector 0.7 0.7 0.0))))
  (Utilities|FlowControl|Delay (Variables|Default|GetDuration))
  (CallFunction|MCDestroyedEffect)
  (Actor|DestroyActor))

(event Collision|EventActorBeginOverlap
  (params (OtherActor :type Actor%20Object%20Reference))
  (if (not (== OtherActor (Game|GetInstigator)))
    (CallFunction|MCDestroyedEffect)
    (Actor|DestroyActor)))

(fn ConstructionScript)

(fn CalcMomentum
  (bind _returnvalue (Game|GetInstigator))
  (bind _returnvalue_2 (Transformation|GetVelocity _returnvalue))
  (LocalVariables|SetLcl_X (.x _returnvalue_2))
  (LocalVariables|SetLcl_Y (.y _returnvalue_2))
  (if (< (LocalVariables|GetLcl_X) 0.0)
    (LocalVariables|SetLcl_X (* (LocalVariables|GetLcl_X) -1.0)))
  (if (< (LocalVariables|GetLcl_Y) 0.0)
    (LocalVariables|SetLcl_Y (* (LocalVariables|GetLcl_Y) -1.0)))
  (LocalVariables|SetLcl_NewSpeed (/ (+ (LocalVariables|GetLcl_X) (LocalVariables|GetLcl_Y)) 5e+01))
  (return (LocalVariables|GetLcl_NewSpeed)))