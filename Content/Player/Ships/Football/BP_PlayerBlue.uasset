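; Blue player ship for the Football mode, adding a primary fire ability.
; The primary input passes through a DoOnce gate that a Timeline resets on finish, while that Timeline drives the HUD's Ability1 cooldown display.
; A locally controlled ship fires directly with authority or through a server event otherwise.
; The shot spawns BP_FB_PFire ahead of the sprite, passing in the ship's velocity and facing direction.
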(event Custom|PrimaryFire
  (bind _self self)
  (bind _sprite (Variables|Default|GetSprite))
  (bind _returnvalue (Math|Vector|GetForwardVector _sprite))
  (if (Pawn|IsLocallyControlled)
    (Networking|SwitchHasAuthority
      (:Authority
        (Game|SpawnActorfromClass "/Game/Player/Ships/Football/Primary/BP_FB_PFire.BP_FB_PFire_C" (Math|Transform|MakeTransform (+ (Transformation|GetWorldLocation _sprite) (* (Math|Vector|MakeVector (.x _returnvalue) (.y _returnvalue) 0.0) (Variables|Default|GetFiringStartDistanceFromSelf))) (Math|Conversions|RotationFromXVector (Math|Vector|GetForwardVector _sprite)) "0.100000,0.100000,0.100000") "AlwaysSpawn" "MultiplyWithRoot" _self (Transformation|GetVelocity) (Math|Vector|GetForwardVector (Variables|Default|GetSprite)) _self))
      (:Remote
        (CallFunction|SVRPrimaryFire)))))

(event Custom|SVR_PrimaryFire
  (bind _self self)
  (bind _sprite (Variables|Default|GetSprite))
  (bind _returnvalue (Math|Vector|GetForwardVector _sprite))
  (Game|SpawnActorfromClass "/Game/Player/Ships/Football/Primary/BP_FB_PFire.BP_FB_PFire_C" (Math|Transform|MakeTransform (+ (Transformation|GetWorldLocation _sprite) (* (Math|Vector|MakeVector (.x _returnvalue) (.y _returnvalue) 0.0) (Variables|Default|GetFiringStartDistanceFromSelf))) (Math|Conversions|RotationFromXVector (Math|Vector|GetForwardVector _sprite)) "0.100000,0.100000,0.100000") "AlwaysSpawn" "MultiplyWithRoot" _self (Transformation|GetVelocity) (Math|Vector|GetForwardVector (Variables|Default|GetSprite)) _self))

(event Input|EnhancedActionEvents|EnhancedInputActionIA_Primary
  (params (ActionValue :type Float%20%28double-precision%29) (ElapsedSeconds :type Float%20%28double-precision%29) (TriggeredSeconds :type Float%20%28double-precision%29) (InputAction :type Input%20Action%20Object%20Reference :default "/Game/Player/Input/IA_Primary.IA_Primary"))
  (Utilities|FlowControl|DoOnce false :!label _label
    (:Completed
      (CallFunction|PrimaryFire)
      (bind _resize (Timeline|Timeline PlayFromStart)
        (:Update
          (Default|Ability1Cooldown (Variables|Default|GetWPB%20HUD) _resize))
        (:Finished
          (goto _label Reset))))))

(event EventBeginPlay
  (|CallParentFunction) ; This node is disabled and will not be called.\nDrag off pins to build functionality.
)

(event EventTick
  (params (DeltaSeconds :type Float%20%28single-precision%29))
  (|CallParentFunction DeltaSeconds) ; This node is disabled and will not be called.\nDrag off pins to build functionality.
)

(fn ConstructionScript
  (|CallParentFunction))