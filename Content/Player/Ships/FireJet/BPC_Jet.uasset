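; Player FireJet ship Blueprint that handles the jet's primary gun fire and its secondary ability input.
; Primary fire is gated by a DoOnce that a Timeline resets, while the Timeline drives the HUD cooldown display.
; A server event alternates left and right guns, then a multicast event spawns BP_JetBullet ahead of that gun, with a horizontal-only offset.
; Secondary input only activates CentralEffect.
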(event Custom|MC_PrimaryFire
  (params (Spawn%20Transform%20Location :type Vector) (Spawn%20Transform%20Rotation :type Rotator))
  (bind _self self)
  (Game|SpawnActorfromClass "/Game/Player/Ships/FireJet/Abilities/BP_JetBullet.BP_JetBullet_C" (Math|Transform|MakeTransform Spawn%20Transform%20Location Spawn%20Transform%20Rotation "0.100000,0.100000,0.100000") "AlwaysSpawn" "MultiplyWithRoot" _self _self))

(event Custom|Svr_PrimaryFire
  (bind _gunl (Variables|Default|GetGunL))
  (bind _gunr (Variables|Default|GetGunR))
  (bind _returnvalue (Math|Vector|GetForwardVector _gunl))
  (bind _returnvalue_2 (Math|Vector|GetForwardVector _gunr))
  (Utilities|FlowControl|FlipFlop
    (:A
      (CallFunction|MCPrimaryFire (+ (Transformation|GetWorldLocation _gunl) (* (Math|Vector|MakeVector (.x _returnvalue) (.y _returnvalue) 0.0) (Variables|Default|GetFiringStartDistanceFromSelf))) (Math|Conversions|RotationFromXVector (Math|Vector|GetForwardVector _gunl))))
    (:B
      (CallFunction|MCPrimaryFire (+ (Transformation|GetWorldLocation _gunr) (* (Math|Vector|MakeVector (.x _returnvalue_2) (.y _returnvalue_2) 0.0) (Variables|Default|GetFiringStartDistanceFromSelf))) (Math|Conversions|RotationFromXVector (Math|Vector|GetForwardVector _gunr))))))

(event Input|EnhancedActionEvents|EnhancedInputActionIA_Secondary
  (params (ActionValue :type Float%20%28double-precision%29) (ElapsedSeconds :type Float%20%28double-precision%29) (TriggeredSeconds :type Float%20%28double-precision%29) (InputAction :type Input%20Action%20Object%20Reference :default "/Game/Player/Input/IA_Secondary.IA_Secondary"))
  (:Started
    (Components|Activation|SetActive (Variables|Default|GetCentralEffect) true false)))

(event Input|EnhancedActionEvents|EnhancedInputActionIA_Primary
  (params (ActionValue :type Float%20%28double-precision%29) (ElapsedSeconds :type Float%20%28double-precision%29) (TriggeredSeconds :type Float%20%28double-precision%29) (InputAction :type Input%20Action%20Object%20Reference :default "/Game/Player/Input/IA_Primary.IA_Primary"))
  (Utilities|FlowControl|DoOnce false :!label _label
    (:Completed
      (CallFunction|SvrPrimaryFire)
      (bind _resize (Timeline|Timeline PlayFromStart)
        (:Update
          (Default|Ability1Cooldown (Variables|Default|GetWPB%20HUD) _resize))
        (:Finished
          (goto _label Reset))))))

(event EventBeginPlay
  (|CallParentFunction) ; This node is disabled and will not be called.\nDrag off pins to build functionality.
)

(fn ConstructionScript
  (|CallParentFunction))