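; BP_FirePrim is a FireJet primary-fire ability actor whose damage and look depend on a Charged value.
; On BeginPlay it runs the parent logic, then scales BaseDamage by Charged plus one half.
; A full charge also shows the particle system and sets the actor scale to one.
; Charged has an empty OnRep handler, and the overlap event is disabled.
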(event EventBeginPlay
  (|CallParentFunction)
  (Variables|Default|SetBase%20Damage (* (Variables|Default|GetBase%20Damage) (+ (Variables|Default|GetCharged?) 0.5)))
  (if (== (Variables|Default|GetCharged?) 1.0)
    (Rendering|SetVisibility (Variables|Default|GetParticleSystem) true false)
    (Transformation|SetActorScale3D (Math|Vector|MakeVector 1.0 1.0 1.0))))

(event Collision|EventActorBeginOverlap
  (params (OtherActor :type Actor%20Object%20Reference))
  (|CallParentFunction OtherActor) ; This node is disabled and will not be called.\nDrag off pins to build functionality.
)

(fn ConstructionScript
  (|CallParentFunction))

(fn OnRepCharged?)