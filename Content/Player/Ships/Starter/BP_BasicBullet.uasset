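; BP_BasicBullet is the projectile for the starter player ship, dealing damage to actors it overlaps other than its instigator.
; On BeginPlay it adds speed from the instigator's absolute X and Y velocity, then moves along local X every tick without delta-time scaling.
; Hits apply damage through a Svr-prefixed event and destroy the bullet.
; The hit effect spawns through an MC-prefixed event only when the lifetime expires.
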(event Custom|Svr_ApplyDamage
  (params (DamagedActor :type Actor%20Object%20Reference))
  (Game|Damage|ApplyDamage DamagedActor (Variables|Default|GetBase%20Damage) 0 (Game|GetInstigator)))

(event Custom|MC_DestroyedEffect
  (Niagara|SpawnSystematLocation (Variables|Default|GetHitEffect) (Transformation|GetActorLocation) "0, 0, 0" "0.100000,0.100000,0.100000"))

(event EventBeginPlay
  (bind _newspeed (CallFunction|CalcMomentum))
  (Variables|Default|SetSpeed (+ _newspeed (Variables|Default|GetSpeed)))
  (Utilities|FlowControl|Delay (Variables|Default|GetDuration))
  (CallFunction|MCDestroyedEffect)
  (Actor|DestroyActor))

(event EventTick
  (params (DeltaSeconds :type Float%20%28single-precision%29))
  (Transformation|AddActorLocalOffset (Math|Vector|MakeVector (Variables|Default|GetSpeed) 0.0 0.0) false false))

(event Collision|EventActorBeginOverlap
  (params (OtherActor :type Actor%20Object%20Reference))
  (if (not (== (Game|GetInstigator) OtherActor))
    (CallFunction|SvrApplyDamage OtherActor)
    (Actor|DestroyActor)))

(fn ConstructionScript)

(fn CalcMomentum
  (bind _returnvalue (Game|GetInstigator))
  (bind _returnvalue_2 (Transformation|GetVelocity _returnvalue))
  (LocalVariables|SetLcl_X (.x _returnvalue_2))
  (LocalVariables|SetLcl_Y (.y _returnvalue_2))
  (if (< (LocalVariables|GetLcl_X) 0.0)
    (LocalVariables|SetLcl_X (* (LocalVariables|GetLcl_X) -1.0)))
  (if (< (LocalVariables|GetLcl_Y) 0.0)
    (LocalVariables|SetLcl_Y (* (LocalVariables|GetLcl_Y) -1.0)))
  (LocalVariables|SetLcl_NewSpeed (/ (+ (LocalVariables|GetLcl_X) (LocalVariables|GetLcl_Y)) 5e+01))
  (return (LocalVariables|GetLcl_NewSpeed)))