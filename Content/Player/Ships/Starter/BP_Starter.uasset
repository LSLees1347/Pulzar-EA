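; BP_Starter is the starter player ship, handling shooting and thruster smoke through Enhanced Input actions.
; IA_Shoot fires a debug-drawn Visibility line trace forward from the Sprite and calls Hit on any BP_AsteroidBase it strikes.
; The trace also prints the hit actor's name unless that display name equals BP_AsteroidBase.
; IA_Thrusters switches the Smoke component on when started and off when completed, with no movement logic here.
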(event Input|EnhancedActionEvents|EnhancedInputActionIA_Thrusters
  (params (ActionValue :type Float%20%28double-precision%29) (ElapsedSeconds :type Float%20%28double-precision%29) (TriggeredSeconds :type Float%20%28double-precision%29) (InputAction :type Input%20Action%20Object%20Reference :default "/Game/Player/Input/IA_Thrusters.IA_Thrusters"))
  (bind _smoke (Variables|Default|GetSmoke))
  (:Started
    (Components|Activation|SetActive _smoke true false))
  (:Completed
    (Components|Activation|SetActive _smoke false false)))

(event Input|EnhancedActionEvents|EnhancedInputActionIA_Shoot
  (params (ActionValue :type Float%20%28double-precision%29) (ElapsedSeconds :type Float%20%28double-precision%29) (TriggeredSeconds :type Float%20%28double-precision%29) (InputAction :type Input%20Action%20Object%20Reference :default "/Game/Player/Input/IA_Shoot.IA_Shoot"))
  (bind _sprite (Variables|Default|GetSprite))
  (bind _returnvalue (Transformation|GetWorldLocation _sprite))
  (bind _outhit (Collision|LineTraceByChannel _returnvalue (+ _returnvalue (* (Math|Vector|GetForwardVector _sprite) (Math|Conversions|ToVector(Float) 2e+03))) "TraceTypeQuery1" false 0 "ForOneFrame" true "(R=1.000000,G=1.000000,B=1.000000,A=1.000000)" "(R=0.000000,G=1.000000,B=0.000000,A=1.000000)" 0.25))
  (if (Utilities|Enum|Equal(Enum) (Utilities|GetDisplayName (.hitactor _outhit)) "BP_AsteroidBase")
    _
    (else
      (Development|PrintString (Utilities|GetDisplayName (.hitactor _outhit)))))
  (bind _asbp_asteroid_base (Utilities|Casting|CastToBP_AsteroidBase (.hitactor _outhit)))
  (Default|Hit _asbp_asteroid_base))

(event EventBeginPlay
  (|CallParentFunction) ; This node is disabled and will not be called.\nDrag off pins to build functionality.
)

(event Collision|EventActorBeginOverlap
  (params (OtherActor :type Actor%20Object%20Reference)))

(event EventTick
  (params (DeltaSeconds :type Float%20%28single-precision%29))
  (|CallParentFunction DeltaSeconds) ; This node is disabled and will not be called.\nDrag off pins to build functionality.
)

(fn ConstructionScript
  (|CallParentFunction))