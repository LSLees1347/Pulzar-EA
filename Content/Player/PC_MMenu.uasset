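; Player controller for the main menu and multiplayer lobby that shows the lobby widget and syncs each player's profile.
; On local BeginPlay it enables the cursor and UI-only input.
; InitialSetup loads the profile from a save slot, creating one if missing, and sends it to GM_MM to refresh the lobby.
; It also updates player names in the lobby widget and returns to MainMenu when a client session ends.
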(event Custom|EndClientSession
  (|DestroySession self
    (:then
      (Game|OpenLevel(byName) "MainMenu"))))

(event Custom|CreateLobbyMenu
  (CallFunction|UIShowLobbyMenu))

(event Custom|InitialSetup
  (CallFunction|LoadSavedProfile)
  (CallFunction|ServerUpdateLobby (Variables|Default|GetPlayer%20Profile)))

(event Custom|UpdatePlayerNames
  (params (PlayerProfiles :type Array%20of%20S%20Player%20Profile%20Structures))
  (bind _wb_lobby_menu (Variables|Default|GetWB%20Lobby%20Menu))
  (Utilities|IsValid _wb_lobby_menu
    (:Is%20Valid
      (Default|ClearPlayerNames _wb_lobby_menu)
      (Default|UpdatePlayerNames _wb_lobby_menu PlayerProfiles))))

(event Custom|ServerUpdateLobby
  (params (PlayerProfile :type S%20Player%20Profile%20Structure))
  (Variables|Default|SetPlayer%20Profile PlayerProfile)
  (bind _asgm_mm (Utilities|Casting|CastToGM_MM (Game|GetGameMode)))
  (Default|UpdateLobby _asgm_mm true))

(event EventBeginPlay
  (if (Pawn|IsLocalController)
    (Variables|Default|SetbShowMouseCursor true)
    (Input|SetInputModeUIOnly self 0 "DoNotLock" false)))

(fn ConstructionScript)

(fn UIShowLobbyMenu
  (Utilities|IsValid (Variables|Default|GetWB%20Lobby%20Menu)
    (:Is%20Valid
      _)
    (:Is%20Not%20Valid
      (bind _returnvalue (UserInterface|CreateWidget "/Game/Widgets/WPB_Lobby.WPB_Lobby_C" self))
      (Variables|Default|SetWB%20Lobby%20Menu _returnvalue)))
  (UserInterface|Viewport|AddtoViewport (Variables|Default|GetWB%20Lobby%20Menu) 0)
  (return))

(fn LoadSavedProfile
  (bind _returnvalue (SaveGame|DoesSaveGameExist (LocalVariables|GetLocal_SlotName)))
  (if _returnvalue
    _
    (else
      (bind _returnvalue_2 (SaveGame|CreateSaveGameObject "/Game/Player/SaveData/SG_PlayerProfile.SG_PlayerProfile_C"))
      (SaveGame|SaveGametoSlot _returnvalue_2 (LocalVariables|GetLocal_SlotName))))
  (bind _returnvalue_3 (SaveGame|LoadGamefromSlot (LocalVariables|GetLocal_SlotName)))
  (bind _assg_player_profile (Utilities|Casting|CastToSG_PlayerProfile _returnvalue_3))
  (Variables|Default|SetPlayer%20Profile (Variables|/Game/Player/SaveData/SG_PlayerProfile.SG_PlayerProfile_C|GetPlayerProfile _assg_player_profile))
  (return))