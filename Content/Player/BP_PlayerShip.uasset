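; Player-controlled ship with momentum-based planar flight, fuel-limited boost, braking, camera zoom and a toggleable name label.
; Enhanced Input rotates the sprite, slower while aiming, and adds thrust or boost along its forward vector to CurrentMomentum.
; Tick offsets the root by that momentum without delta-time scaling, while looping timers scale momentum and refill fuel after boosting.
; Overlaps with out-of-bounds walls, matched by display name, bounce the momentum.
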(event OnComponentBeginOverlap(RootCollision)
  (params (OverlappedComponent :type Primitive%20Component%20Object%20Reference) (OtherActor :type Actor%20Object%20Reference) (OtherComp :type Primitive%20Component%20Object%20Reference) (OtherBodyIndex :type Integer) (bFromSweep :type Boolean) (SweepResult :type Hit%20Result%20Structure%20%28by%20ref%29))
  (bind _returnvalue (Utilities|GetDisplayName OtherComp))
  (bind _wallbouncynessmultiplier (Variables|Default|GetWallBouncynessMultiplier))
  (Development|PrintString _returnvalue)
  (Utilities|FlowControl|Sequence
    (:then_0
      (if (or (Utilities|Enum|Equal(Enum) _returnvalue "BP_oobTrigger.LeftWall") (Utilities|Enum|Equal(Enum) _returnvalue "BP_oobTrigger.RightWall"))
        (Variables|Default|SetCurrentMomentum (Math|Vector|MakeVector (* (* (.x (Variables|Default|GetCurrentMomentum)) 1.0) _wallbouncynessmultiplier) (* (* (.y (Variables|Default|GetCurrentMomentum)) -1.0) _wallbouncynessmultiplier) 0.0))))
    (:then_1
      (if (or (Utilities|Enum|Equal(Enum) _returnvalue "BP_oobTrigger.TopWall") (Utilities|Enum|Equal(Enum) _returnvalue "BP_oobTrigger.BottomWall"))
        (Variables|Default|SetCurrentMomentum (Math|Vector|MakeVector (* (* (.x (Variables|Default|GetCurrentMomentum)) -1.0) _wallbouncynessmultiplier) (* (* (.y (Variables|Default|GetCurrentMomentum)) 1.0) _wallbouncynessmultiplier) 0.0))))))

(event Custom|RefillFuel
  (Variables|Default|SetFuel (Math|Interpolation|FInterptoConstant (Variables|Default|GetFuel) 1.0 (Utilities|Time|GetWorldDeltaSeconds) 0.1)))

(event Custom|CapSpeed
  (bind _capspeedmultiplier (Variables|Default|GetCapSpeedMultiplier))
  (Variables|Default|SetCurrentMomentum (Math|Vector|MakeVector (* (.x (Variables|Default|GetCurrentMomentum)) _capspeedmultiplier) (* (.y (Variables|Default|GetCurrentMomentum)) _capspeedmultiplier) 0.0)))

(event Input|EnhancedActionEvents|EnhancedInputActionIA_RotateR
  (params (ActionValue :type Float%20%28double-precision%29) (ElapsedSeconds :type Float%20%28double-precision%29) (TriggeredSeconds :type Float%20%28double-precision%29) (InputAction :type Input%20Action%20Object%20Reference :default "/Game/Player/Input/IA_RotateR.IA_RotateR"))
  (Transformation|AddRelativeRotation (Variables|Default|GetSprite) (Math|Rotator|MakeRotator 0.0 0.0 (* ActionValue (Math|Float|SelectFloat 4.0 8.0 (stale Input|EnhancedActionEvents|EnhancedInputActionIA_Aim _output_get)))) false false))

(event Input|EnhancedActionEvents|EnhancedInputActionIA_RotateL
  (params (ActionValue :type Float%20%28double-precision%29) (ElapsedSeconds :type Float%20%28double-precision%29) (TriggeredSeconds :type Float%20%28double-precision%29) (InputAction :type Input%20Action%20Object%20Reference :default "/Game/Player/Input/IA_RotateL.IA_RotateL"))
  (Transformation|AddRelativeRotation (Variables|Default|GetSprite) (Math|Rotator|MakeRotator 0.0 0.0 (* ActionValue (* (Math|Float|SelectFloat 4.0 8.0 (stale Input|EnhancedActionEvents|EnhancedInputActionIA_Aim _output_get)) -1.0))) false false))

(event Input|EnhancedActionEvents|EnhancedInputActionIA_Thrusters
  (params (ActionValue :type Float%20%28double-precision%29) (ElapsedSeconds :type Float%20%28double-precision%29) (TriggeredSeconds :type Float%20%28double-precision%29) (InputAction :type Input%20Action%20Object%20Reference :default "/Game/Player/Input/IA_Thrusters.IA_Thrusters"))
  (bind _sprite (Variables|Default|GetSprite))
  (bind _thrustspeed (Variables|Default|GetThrustSpeed))
  (bind _returnvalue (Math|Vector|GetForwardVector _sprite))
  (bind _returnvalue_2 (* _returnvalue _thrustspeed))
  (:Triggered
    (Variables|AnimCalls|SetIsThrusting true)
    (Variables|Default|SetCurrentMomentum (Math|Vector|MakeVector (+ (.x _returnvalue_2) (.x (Variables|Default|GetCurrentMomentum))) (+ (.y _returnvalue_2) (.y (Variables|Default|GetCurrentMomentum))) 0.0)))
  (:Canceled
    (Variables|AnimCalls|SetIsThrusting false :!label _label))
  (:Completed
    (goto _label)))

(event Input|EnhancedActionEvents|EnhancedInputActionIA_Boost
  (params (ActionValue :type Float%20%28double-precision%29) (ElapsedSeconds :type Float%20%28double-precision%29) (TriggeredSeconds :type Float%20%28double-precision%29) (InputAction :type Input%20Action%20Object%20Reference :default "/Game/Player/Input/IA_Boost.IA_Boost"))
  (bind _sprite (Variables|Default|GetSprite))
  (bind _boostspeed (Variables|Default|GetBoostSpeed))
  (bind _returnvalue (Math|Vector|GetForwardVector _sprite))
  (bind _returnvalue_2 (* _returnvalue _boostspeed))
  (:Triggered
    (Utilities|Time|ClearandInvalidateTimerbyHandle (Variables|Default|GetRefillFuelTimer))
    (if (and (Variables|AnimCalls|GetIsThrusting) (!= (Variables|Default|GetFuel) 0.0))
      (Variables|Default|SetCurrentMomentum (Math|Vector|MakeVector (+ (.x _returnvalue_2) (.x (Variables|Default|GetCurrentMomentum))) (+ (.y _returnvalue_2) (.y (Variables|Default|GetCurrentMomentum))) 0.0))
      (Variables|Default|SetFuel (Math|Interpolation|FInterptoConstant (Variables|Default|GetFuel) 0.0 (Utilities|Time|GetWorldDeltaSeconds) 0.5))
      (else
        (Variables|AnimCalls|SetIsBoosting false))))
  (:Started
    (Variables|AnimCalls|SetIsBoosting true))
  (:Completed
    (Variables|AnimCalls|SetIsBoosting false)
    (bind _returnvalue_3 (Utilities|Time|SetTimerbyEvent (delegate Custom|RefillFuel) 0.016667 true true))
    (Variables|Default|SetRefillFuelTimer _returnvalue_3)))

(event Input|EnhancedActionEvents|EnhancedInputActionIA_Aim
  (params (ActionValue :type Boolean) (ElapsedSeconds :type Float%20%28double-precision%29) (TriggeredSeconds :type Float%20%28double-precision%29) (InputAction :type Input%20Action%20Object%20Reference :default "/Game/Player/Input/IA_Aim.IA_Aim"))
  (:Triggered
    (bind _output_get (Variables|AnimCalls|SetIsAiming true)))
  (:Canceled
    (Variables|AnimCalls|SetIsAiming false :!label _label))
  (:Completed
    (goto _label)))

(event Input|EnhancedActionEvents|EnhancedInputActionIA_ShowNames
  (params (ActionValue :type Boolean) (ElapsedSeconds :type Float%20%28double-precision%29) (TriggeredSeconds :type Float%20%28double-precision%29) (InputAction :type Input%20Action%20Object%20Reference :default "/Game/Player/Input/IA_ShowNames.IA_ShowNames"))
  (bind _playername (Variables|Default|GetPlayerName))
  (:Started
    (Rendering|SetVisibility _playername true false))
  (:Canceled
    (Rendering|SetVisibility _playername false false :!label _label))
  (:Completed
    (goto _label)))

(event Input|EnhancedActionEvents|EnhancedInputActionIA_Brake
  (params (ActionValue :type Float%20%28double-precision%29) (ElapsedSeconds :type Float%20%28double-precision%29) (TriggeredSeconds :type Float%20%28double-precision%29) (InputAction :type Input%20Action%20Object%20Reference :default "/Game/Player/Input/IA_Brake.IA_Brake"))
  (bind _returnvalue (Utilities|Time|GetWorldDeltaSeconds))
  (:Triggered
    (Variables|AnimCalls|SetIsBraking true)
    (Variables|Default|SetCurrentMomentum (Math|Vector|MakeVector (Math|Interpolation|FInterpTo (.x (Variables|Default|GetCurrentMomentum)) 0.0 _returnvalue 2.0) (Math|Interpolation|FInterpTo (.y (Variables|Default|GetCurrentMomentum)) 0.0 _returnvalue 2.0) 0.0)))
  (:Canceled
    (Variables|AnimCalls|SetIsBraking false :!label _label))
  (:Completed
    (goto _label)))

(event Input|EnhancedActionEvents|EnhancedInputActionIA_CamScroll
  (params (ActionValue :type Float%20%28double-precision%29) (ElapsedSeconds :type Float%20%28double-precision%29) (TriggeredSeconds :type Float%20%28double-precision%29) (InputAction :type Input%20Action%20Object%20Reference :default "/Game/Player/Input/IA_CamScroll.IA_CamScroll"))
  (bind _camera (Variables|Default|GetCamera))
  (Camera|SetFieldOfView _camera (Math|Float|Clamp(Float) (- (Variables|/Script/Engine.CameraComponent|GetFieldOfView _camera) (* ActionValue 3.0)) 6e+01 1e+02)))

(event EventTick
  (params (DeltaSeconds :type Float%20%28single-precision%29))
  (bind _currentmomentum (Variables|Default|GetCurrentMomentum))
  (bind _shipcontrol (Variables|Default|GetShipControl))
  (Utilities|FlowControl|Sequence
    (:then_0
      (Transformation|AddWorldOffset (Variables|Default|GetRoot%20Collision) (Math|Vector|MakeVector (* (.x _currentmomentum) _shipcontrol) (* (.y _currentmomentum) _shipcontrol) 0.0) false false))))

(event EventBeginPlay
  (bind _aspc_player (Utilities|Casting|CastToPC_Player (Game|GetPlayerController 0)))
  (Utilities|IsValid _aspc_player
    (:Is%20Valid
      (Utilities|IsValid (PlayerController|LocalPlayerSubsystems|GetEnhancedInputLocalPlayerSubsystem _aspc_player)
        (:Is%20Valid
          (Input|AddMappingContext (PlayerController|LocalPlayerSubsystems|GetEnhancedInputLocalPlayerSubsystem _aspc_player) "/Game/Player/Input/IMC_Default.IMC_Default" 0 "(bIgnoreAllPressedKeysUntilRelease=True,bForceImmediately=False,bNotifyUserSettings=False)")
          (Transformation|SetWorldTransform (Variables|Default|GetRoot%20Collision) (Math|Transform|MakeTransform "0, 0, 0" "0, 0, 0" "1.000000,1.000000,1.000000") false false)
          (bind _asgi_player (Utilities|Casting|CastToGI_Player (Game|GetGameInstance)))
          (Rendering|Components|TextRender|SetText (Variables|Default|GetPlayerName) (Variables|/Game/Player/GI_Player.GI_Player_C|GetPlayerName _asgi_player))
          (Transformation|SetWorldTransform (Variables|Default|GetRoot%20Collision) (Variables|Default|GetSpawnPoint) false false)
          (Utilities|Time|SetTimerbyEvent (delegate Custom|CapSpeed) 0.05 true true))))))

(fn ConstructionScript)