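; Base player ship Character for multiplayer, flying on the XY plane with cursor aiming, thrust, braking and two cooldown-limited velocity flips.
; Rotation, braking and flips go through server events, with multicasts for the latter two and for effects.
; Damage is reduced by data-table Defence, releases any held orb, shows indicators and reports death to the player controller.
; Health, flip cooldowns and timer-polled speed feed the HUD.
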(event Custom|DisableAllInput
  (params (PlayerController :type Player%20Controller%20Object%20Reference))
  (Input|DisableInput PlayerController))

(event Custom|MC_Flip
  (Variables|/Script/Engine.MovementComponent|SetVelocity (Variables|Character|GetCharacterMovement) (Math|Vector|MakeVector (* (.x (Variables|/Script/Engine.MovementComponent|GetVelocity (Variables|Character|GetCharacterMovement))) -1.0) (* (.y (Variables|/Script/Engine.MovementComponent|GetVelocity (Variables|Character|GetCharacterMovement))) -1.0) 0.0)))

(event Custom|Svr_Braking
  (params (Braking? :type Boolean))
  (CallFunction|MCBraking Braking?))

(event Custom|MC_Braking
  (params (Braking? :type Boolean))
  (bind _charactermovement (Variables|Character|GetCharacterMovement))
  (if Braking?
    (Variables|Default|SetIsBraking true)
    (Variables|/Script/Engine.CharacterMovementComponent|SetBrakingDecelerationFlying _charactermovement (Variables|Default|GetBrakeDF))
    (else
      (Variables|Default|SetIsBraking false)
      (Variables|/Script/Engine.CharacterMovementComponent|SetBrakingDecelerationFlying _charactermovement (Variables|Default|GetDeacceleration)))))

(event Custom|GainPossession
  (params (Orb :type Actor%20Object%20Reference))
  (Variables|Default|SetHasPossession true)
  (bind _asbp_orb (Utilities|Casting|CastToBP_Orb Orb))
  (Variables|Default|SetAs%20BP%20Uorb _asbp_orb))

(event Custom|MC_DamageIndicator
  (bind _self self)
  (bind _returnvalue (Game|SpawnActorfromClass "/Game/Player/BP_DamageTextIndicator.BP_DamageTextIndicator_C" (Transformation|GetActorTransform) "Undefined" "MultiplyWithRoot" _self _self))
  (Transformation|AttachActorToActor _returnvalue self "None" "SnapToTarget" "SnapToTarget" "SnapToTarget" true))

(event Custom|UpdateSpeed
  (params (Acceleration :type Float%20%28single-precision%29) (TopSpeed :type Float%20%28single-precision%29))
  (Variables|Default|SetAcceleration (* (Variables|Default|GetAcceleration) Acceleration))
  (Variables|Default|SetTopSpeed (* (Variables|Default|GetTopSpeed) TopSpeed))
  (Variables|/Script/Engine.CharacterMovementComponent|SetMaxAcceleration (Variables|Character|GetCharacterMovement) (Variables|Default|GetAcceleration))
  (Variables|/Script/Engine.CharacterMovementComponent|SetMaxFlySpeed (Variables|Character|GetCharacterMovement) (Variables|Default|GetTopSpeed)))

(event Custom|DamageRelease
  (if (and (Utilities|IsValid (Variables|Default|GetAs%20BP%20Uorb)) (Variables|Default|GetHasPossession))
    (Default|ReleaseOrb (Variables|Default|GetAs%20BP%20Uorb))))

(event Custom|CustomEvent
  (params (Velocity%20X :type Float%20%28double-precision%29) (Velocity%20Y :type Float%20%28double-precision%29))
  (bind _output_get (Variables|Default|Setvx Velocity%20X))
  (bind _output_get_2 (Variables|Default|Setvy Velocity%20Y))
  (Variables|/Script/Engine.MovementComponent|SetVelocity (Variables|Character|GetCharacterMovement) (Math|Vector|MakeVector _output_get _output_get_2 0.0)))

(event Custom|SVR
  (params (NewParam :type Rotator))
  (bind _output_get (Variables|Default|SetNewRot NewParam))
  (Transformation|SetActorRotation _output_get true))

(event Custom|Svr_Flip
  (CallFunction|MCFlip))

(event Custom|MC_Death
  (params (Location :type Vector))
  (Niagara|SpawnSystematLocation (Variables|Default|GetDeathEffect) Location "0, 0, 0" "0.700000,0.700000,0.700000"))

(event Custom|MC_SpawnEffect
  (Niagara|SpawnSystematLocation (Variables|Default|GetSpawnEffect) (Transformation|GetWorldLocation (Variables|Default|GetSprite)) "0, 0, 0" "0.900000,0.900000,0.900000"))

(event Custom|ClientUpdateHUD_Health
  (params (Vignette? :type Boolean))
  (Default|UpdateHealth (Variables|Default|GetWPB%20HUD) (Math|Conversions|ToFloat(Integer) (Variables|Default|GetHealth)) Vignette?))

(event Custom|MC_Impact
  (params (Location :type Vector))
  (Niagara|SpawnSystematLocation (Variables|Default|GetShotEffect) Location "0, 0, 0" "0.200000,0.200000,0.200000"))

(event Custom|ClientUpdateSpeedo
  (params (NewSpeed :type Float%20%28double-precision%29))
  (Default|UpdateSpeedo (Variables|Default|GetWPB%20HUD) NewSpeed))

(event Custom|Svr_DamageIndicator
  (CallFunction|MCDamageIndicator))

(event Input|EnhancedActionEvents|EnhancedInputActionIA_Thrust
  (params (ActionValue :type Float%20%28double-precision%29) (ElapsedSeconds :type Float%20%28double-precision%29) (TriggeredSeconds :type Float%20%28double-precision%29) (InputAction :type Input%20Action%20Object%20Reference :default "/Game/Player/Input/IA_Thrust.IA_Thrust"))
  (bind _sprite (Variables|Default|GetSprite))
  (bind _returnvalue (Math|Vector|GetForwardVector _sprite))
  (:Triggered
    (Variables|Default|SetIsThrusting true)
    (Pawn|Input|AddMovementInput (Math|Vector|MakeVector (.x _returnvalue) (.y _returnvalue) 0.0) 1.0 true)
    (bind _zoomout (Timeline|FovScale Play)
      (:Update
        (Camera|SetFieldOfView (Variables|Default|GetCamera) (Math|Float|Lerp 9e+01 1e+02 _zoomout)))))
  (:Canceled
    (Variables|Default|SetIsThrusting false :!label _label)
    (Timeline|FovScale Reverse))
  (:Completed
    (goto _label)))

(event Input|EnhancedActionEvents|EnhancedInputActionIA_Flip
  (params (ActionValue :type Float%20%28double-precision%29) (ElapsedSeconds :type Float%20%28double-precision%29) (TriggeredSeconds :type Float%20%28double-precision%29) (InputAction :type Input%20Action%20Object%20Reference :default "/Game/Player/Input/IA_Flip.IA_Flip"))
  (:Started
    (if (Variables|Default|GetFlip2?)
      (Variables|Default|SetFlip2? false)
      (CallFunction|SvrFlip)
      (bind _cooldown (Timeline|Flip2 PlayFromStart)
        (:Update
          (Default|Flip2Cooldown (Variables|Default|GetWPB%20HUD) _cooldown))
        (:Finished
          (Variables|Default|SetFlip2? true)))
      (elif (Variables|Default|GetFlip1?)
        (Variables|Default|SetFlip1? false)
        (CallFunction|SvrFlip)
        (bind _cooldown_2 (Timeline|Flip1 PlayFromStart)
          (:Update
            (Default|Flip1Cooldown (Variables|Default|GetWPB%20HUD) _cooldown_2))
          (:Finished
            (Variables|Default|SetFlip1? true)))))))

(event Input|EnhancedActionEvents|EnhancedInputActionIA_Minimap
  (params (ActionValue :type Boolean) (ElapsedSeconds :type Float%20%28double-precision%29) (TriggeredSeconds :type Float%20%28double-precision%29) (InputAction :type Input%20Action%20Object%20Reference :default "/Game/Player/Input/IA_Minimap.IA_Minimap"))
  (bind _returnvalue (Pawn|GetController))
  (:Started
    (bind _asbp_standard_player_controller (Utilities|Casting|CastToBP_Standard_PlayerController _returnvalue))
    (Default|UIToggleScoreboard _asbp_standard_player_controller true))
  (:Completed
    (bind _asbp_standard_player_controller_2 (Utilities|Casting|CastToBP_Standard_PlayerController _returnvalue))
    (Default|UIToggleScoreboard _asbp_standard_player_controller_2 false)))

(event Input|EnhancedActionEvents|EnhancedInputActionIA_Flip
  (params (ActionValue :type Float%20%28double-precision%29) (ElapsedSeconds :type Float%20%28double-precision%29) (TriggeredSeconds :type Float%20%28double-precision%29) (InputAction :type Input%20Action%20Object%20Reference :default "/Game/Player/Input/IA_Flip.IA_Flip")))

(event Input|EnhancedActionEvents|EnhancedInputActionIA_Release
  (params (ActionValue :type Boolean) (ElapsedSeconds :type Float%20%28double-precision%29) (TriggeredSeconds :type Float%20%28double-precision%29) (InputAction :type Input%20Action%20Object%20Reference :default "/Game/Player/Input/IA_Release.IA_Release"))
  (:Started
    (if (and (Utilities|IsValid (Variables|Default|GetAs%20BP%20Uorb)) (Variables|Default|GetHasPossession))
      (Default|ReleaseOrb (Variables|Default|GetAs%20BP%20Uorb)))))

(event Input|EnhancedActionEvents|EnhancedInputActionIA_Pause
  (params (ActionValue :type Boolean) (ElapsedSeconds :type Float%20%28double-precision%29) (TriggeredSeconds :type Float%20%28double-precision%29) (InputAction :type Input%20Action%20Object%20Reference :default "/Game/Player/Input/IA_Pause.IA_Pause"))
  (bind _wpb_hud (Variables|Default|GetWPB%20HUD))
  (:Started
    (bind _asbp_game_instance (Utilities|Casting|CastToBP_GameInstance (Game|GetGameInstance)))
    (bind _isgamepausedresult (Default|TogglePauseGame _asbp_game_instance))
    (if _isgamepausedresult
      (Widget|SetVisibility _wpb_hud "Hidden")
      (else
        (Widget|SetVisibility _wpb_hud "Visible")))))

(event Input|EnhancedActionEvents|EnhancedInputActionIA_Brake
  (params (ActionValue :type Float%20%28double-precision%29) (ElapsedSeconds :type Float%20%28double-precision%29) (TriggeredSeconds :type Float%20%28double-precision%29) (InputAction :type Input%20Action%20Object%20Reference :default "/Game/Player/Input/IA_Brake.IA_Brake"))
  (:Started
    (CallFunction|SvrBraking true))
  (:Canceled
    (CallFunction|SvrBraking false :!label _label))
  (:Completed
    (goto _label)))

(event EventPossessed
  (params (NewController :type Controller%20Object%20Reference))
  (bind _asplayer_controller (Utilities|Casting|CastToPlayerController NewController))
  (bind _asbp_standard_player_controller (Utilities|Casting|CastToBP_Standard_PlayerController _asplayer_controller))
  (Variables|Default|SetAs%20BP%20Standard%20Player%20Controller _asbp_standard_player_controller)
  (CallFunction|DisableAllInput _asplayer_controller))

(event Game|Damage|EventAnyDamage
  (params (Damage :type Float%20%28single-precision%29) (DamageType :type Damage%20Type%20Object%20Reference) (InstigatedBy :type Controller%20Object%20Reference) (DamageCauser :type Actor%20Object%20Reference))
  (bind _returnvalue (Transformation|GetActorLocation))
  (bind _sprite (Variables|Default|GetSprite))
  (bind _returnvalue_2 (Transformation|GetWorldLocation _sprite))
  (Class|BPIDamageType|TriggerEffect(Message) DamageType (Variables|Default|GetAC_StatusEffect) InstigatedBy)
  (CallFunction|DamageRelease)
  (Variables|Default|SetIncomingDamage (Math|Float|Truncate Damage))
  (CallFunction|SvrDamageIndicator)
  (Variables|Default|SetHealth (Math|Integer|Clamp(Integer) (- (Variables|Default|GetHealth) (* Damage (/ (- 100 (Variables|Default|GetDefence)) 100))) 0 100))
  (CallFunction|ClientUpdateHUDHealth true)
  (Camera|PlayWorldCameraShake "/Game/Player/BP_CameraShake.BP_CameraShake_C" (Math|Vector|MakeVector (.x _returnvalue) (.y _returnvalue) 1e+03) 0.0 5e+02)
  (if (<= (Variables|Default|GetHealth) 0)
    (CallFunction|MCDeath _returnvalue_2)
    (bind _asbp_standard_player_controller (Utilities|Casting|CastToBP_Standard_PlayerController (Pawn|GetController)))
    (Default|PlayerDeath _asbp_standard_player_controller self)
    (else
      (CallFunction|MCImpact _returnvalue_2))))

(event EventOnBecomeViewTarget
  (params (PC :type Player%20Controller%20Object%20Reference))
  ;[0 0 0] Comment
)

(event EventBeginPlay
  (bind _returnvalue (Transformation|GetActorLocation))
  (Utilities|FlowControl|Sequence
    (:then_0
      (bind _asbp_standard_player_controller (Utilities|Casting|CastToBP_Standard_PlayerController (Game|GetPlayerController 0)))
      (Utilities|IsValid _asbp_standard_player_controller
        (:Is%20Valid
          (Utilities|IsValid (PlayerController|LocalPlayerSubsystems|GetEnhancedInputLocalPlayerSubsystem _asbp_standard_player_controller)
            (:Is%20Valid
              (Input|AddMappingContext (PlayerController|LocalPlayerSubsystems|GetEnhancedInputLocalPlayerSubsystem _asbp_standard_player_controller) "/Game/Player/Input/IMC_Player.IMC_Player" 0 "(bIgnoreAllPressedKeysUntilRelease=True,bForceImmediately=False,bNotifyUserSettings=False)")
              (Transformation|SetActorLocation (Math|Vector|MakeVector (.x _returnvalue) (.y _returnvalue) 0.0) false false))))))
    (:then_1
      (CallFunction|MCSpawnEffect))
    (:then_2
      (Utilities|Time|SetTimerbyFunctionName 0 "TimedSpeedoUpdate" 0.1 true))))

(event Game|Damage|EventPointDamage
  (params (Damage :type Float%20%28single-precision%29) (DamageType :type Damage%20Type%20Object%20Reference) (HitLocation :type Vector :default "0, 0, 0") (HitNormal :type Vector :default "0, 0, 0") (HitComponent :type Primitive%20Component%20Object%20Reference) (BoneName :type Name :default "None") (ShotFromDirection :type Vector :default "0, 0, 0") (InstigatedBy :type Controller%20Object%20Reference) (DamageCauser :type Actor%20Object%20Reference) (HitInfo :type Hit%20Result%20Structure%20%28by%20ref%29)))

(event EventTick
  (params (DeltaSeconds :type Float%20%28single-precision%29))
  (bind _returnvalue (Transformation|GetActorLocation))
  (bind _as_bp_standard_player_controller (Variables|Default|GetAs%20BP%20Standard%20Player%20Controller))
  (bind _hitresult (Game|Player|GetHitResultUnderCursorbyChannel _as_bp_standard_player_controller "TraceTypeQuery1" true))
  (bind _returnvalue_2 (Math|Rotator|FindLookatRotation (Math|Vector|MakeVector (.x _returnvalue) (.y _returnvalue) 0.0) (Math|Vector|MakeVector (.x (.location _hitresult)) (.y (.location _hitresult)) 0.0)))
  (if (Pawn|IsLocallyControlled)
    (Transformation|SetActorRotation _returnvalue_2 true)
    (Networking|SwitchHasAuthority
      (:Authority
        (bind _output_get (Variables|Default|SetNewRot _returnvalue_2))
        (Transformation|SetActorRotation _output_get true))
      (:Remote
        (CallFunction|SVR _returnvalue_2)))))

(fn ConstructionScript
  (bind _charactermovement (Variables|Character|GetCharacterMovement))
  (Variables|Default|SetStamina 0)
  (Variables|Default|SetHealth 100)
  (Variables|/Script/Engine.CharacterMovementComponent|SetMaxAcceleration _charactermovement (Variables|Default|GetAcceleration))
  (Variables|/Script/Engine.CharacterMovementComponent|SetMaxFlySpeed _charactermovement (Variables|Default|GetTopSpeed))
  (Variables|/Script/Engine.CharacterMovementComponent|SetBrakingDecelerationFlying _charactermovement (Variables|Default|GetDeacceleration))
  (Pawn|Components|CharacterMovement|SetMovementMode (Variables|Character|GetCharacterMovement) "MOVE_Flying" 0)
  (Networking|SwitchHasAuthority
    (:Authority
      (bind _returnvalue (Utilities|GetDataTableRow "/Game/Player/CharacterInfoTable.CharacterInfoTable" (Variables|Default|GetCharaRowName))
        (:then
          (Variables|Default|SetDefence (.Defence (Utilities|Struct|BreakS_CharacterInfo _returnvalue))))
        (:RowNotFound
          (Variables|Default|SetDefence 0))))))

(fn LineTrace
  (bind _sprite (Variables|Default|GetSprite))
  (bind _returnvalue (Transformation|GetWorldLocation _sprite))
  (bind _returnvalue_2 (Math|Vector|GetForwardVector _sprite))
  (bind (_outhit _returnvalue_3) (Collision|LineTraceByChannel _returnvalue (+ _returnvalue (* (Math|Vector|MakeVector (.x _returnvalue_2) (.y _returnvalue_2) 0.0) (Variables|Default|GetHitScanRange))) "TraceTypeQuery1" false 0 "ForOneFrame" true "(R=1.000000,G=1.000000,B=1.000000,A=1.000000)" "(R=0.000000,G=1.000000,B=0.000000,A=1.000000)" 0.25))
  (return _returnvalue_3 _outhit))

(fn TimedSpeedoUpdate
  (CallFunction|ClientUpdateSpeedo (/ (Math|Vector|VectorLengthXY (Variables|/Script/Engine.MovementComponent|GetVelocity (Variables|Character|GetCharacterMovement))) (Variables|Default|GetTopSpeed)))
  (return))