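; Player character for a 2D game that rotates its sprite and boosts along the sprite's facing direction.
; BeginPlay adds the Enhanced Input mapping, shows a DebugInfo widget and sets movement to Flying.
; Left and right inputs yaw the sprite; boost speed grows with hold time up to a cap.
; Boost offsets Sprite and SpringArm directly in world XY, bypassing the movement component.
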(event Input|EnhancedActionEvents|EnhancedInputActionIA_LeftRotate
  (params (ActionValue :type Float%20%28double-precision%29) (ElapsedSeconds :type Float%20%28double-precision%29) (TriggeredSeconds :type Float%20%28double-precision%29) (InputAction :type Input%20Action%20Object%20Reference :default "/Game/Blueprints/Input/IA_LeftRotate.IA_LeftRotate"))
  (Transformation|AddWorldRotation (Variables|Default|GetSprite) (Math|Rotator|MakeRotator 0.0 0.0 (* (* ActionValue -1.0) (Variables|Default|GetRotationMultiplier))) false false))

(event Input|EnhancedActionEvents|EnhancedInputActionIA_RightRotate
  (params (ActionValue :type Float%20%28double-precision%29) (ElapsedSeconds :type Float%20%28double-precision%29) (TriggeredSeconds :type Float%20%28double-precision%29) (InputAction :type Input%20Action%20Object%20Reference :default "/Game/Blueprints/Input/IA_RightRotate.IA_RightRotate"))
  (Transformation|AddWorldRotation (Variables|Default|GetSprite) (Math|Rotator|MakeRotator 0.0 0.0 (* ActionValue (Variables|Default|GetRotationMultiplier))) false false))

(event Input|EnhancedActionEvents|EnhancedInputActionIA_Boost
  (params (ActionValue :type Float%20%28double-precision%29) (ElapsedSeconds :type Float%20%28double-precision%29) (TriggeredSeconds :type Float%20%28double-precision%29) (InputAction :type Input%20Action%20Object%20Reference :default "/Game/Blueprints/Input/IA_Boost.IA_Boost"))
  (bind _returnvalue (Math|Float|Lerp 0.0 ActionValue TriggeredSeconds))
  (bind _boostaccelmultiplier (Variables|Default|GetBoostAccelMultiplier))
  (bind _sprite (Variables|Default|GetSprite))
  (bind _boostmaxspeed (Variables|Default|GetBoostMaxSpeed))
  (bind _returnvalue_2 (Math|Vector|GetForwardVector _sprite))
  (bind _returnvalue_3 (* _returnvalue _boostaccelmultiplier))
  (bind _returnvalue_4 (Math|Float|Clamp(Float) _returnvalue_3 0.0 _boostmaxspeed))
  (bind _returnvalue_5 (* (.y _returnvalue_2) _returnvalue_4))
  (bind _returnvalue_6 (* (.x _returnvalue_2) _returnvalue_4))
  (:Triggered
    (Transformation|AddWorldOffset _sprite (Math|Vector|MakeVector _returnvalue_6 _returnvalue_5 0.0) false false)
    (Transformation|AddWorldOffset (Variables|Default|GetSpringArm) (Math|Vector|MakeVector _returnvalue_6 _returnvalue_5 0.0) false false)))

(event EventTick
  (params (DeltaSeconds :type Float%20%28single-precision%29))
  (Development|PrintString ""))

(event EventBeginPlay
  (bind _aspc_player (Utilities|Casting|CastToPC_Player (Game|GetPlayerController 0)))
  (Utilities|IsValid _aspc_player
    (:Is%20Valid
      (Utilities|IsValid (PlayerController|LocalPlayerSubsystems|GetEnhancedInputLocalPlayerSubsystem _aspc_player)
        (:Is%20Valid
          (Input|AddMappingContext (PlayerController|LocalPlayerSubsystems|GetEnhancedInputLocalPlayerSubsystem _aspc_player) "/Game/Blueprints/Input/IMC_Default.IMC_Default" 0 "(bIgnoreAllPressedKeysUntilRelease=True,bForceImmediately=False,bNotifyUserSettings=False)")
          (bind _returnvalue (UserInterface|CreateWidget "/Game/Widgets/DebugInfo.DebugInfo_C"))
          (UserInterface|Viewport|AddtoViewport _returnvalue 0)
          (Pawn|Components|CharacterMovement|SetMovementMode (Variables|Character|GetCharacterMovement) "MOVE_Flying" 0))))))

(fn ConstructionScript
  (Transformation|SetWorldTransform (Variables|Collision|GetCapsuleComponent) (Math|Transform|MakeTransform (Math|Vector|MakeVector 0.0 0.0 2e+01) (Math|Rotator|MakeRotator 0.0 0.0 0.0) (Math|Vector|MakeVector 1.0 1.0 1.0)) false false))