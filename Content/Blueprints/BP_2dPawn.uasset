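; Player pawn for a flipbook-sprite craft with inertial thruster movement, braking, fuel-limited boost, debug trace shooting and mark-and-return teleport.
; Enhanced Input thrust builds a momentum vector that Tick applies while coasting, moving the sprite and spring arm rather than the actor.
; Boost drains fuel, and a looping timer refills it on release.
; BeginPlay creates the HUD, and Tick feeds position and yaw to the minimap parameter collection.
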(event Custom|CallLineTrace
  (bind _sprite (Variables|Default|GetSprite))
  (Collision|LineTraceComponent _sprite (Transformation|GetWorldLocation _sprite) (Variables|Default|GetTeleportLocation) false true false))

(event Custom|Refuel
  (if (<= (Variables|Default|GetFuel) 1.0)
    (Variables|Default|SetFuel (Math|Float|Lerp (Variables|Default|GetFuel) 1.1 0.001))
    (else
      (Utilities|Time|ClearandInvalidateTimerbyHandle (stale Input|EnhancedActionEvents|EnhancedInputActionIA_Boost _returnvalue)))))

(event Input|EnhancedActionEvents|EnhancedInputActionIA_Boost
  (params (ActionValue :type Float%20%28double-precision%29) (ElapsedSeconds :type Float%20%28double-precision%29) (TriggeredSeconds :type Float%20%28double-precision%29) (InputAction :type Input%20Action%20Object%20Reference :default "/Game/Blueprints/Input/IA_Boost.IA_Boost"))
  (:Triggered
    (Utilities|Time|ClearandInvalidateTimerbyHandle (stale _returnvalue))
    (if (>= (Variables|Default|GetFuel) 0.0)
      (Variables|Default|SetCurrentThrustSpeed (Variables|Default|GetBoostSpeed))
      (Variables|Default|SetFuel (Math|Float|Lerp (Variables|Default|GetFuel) -0.1 0.015))
      (else
        (Variables|Default|SetCurrentThrustSpeed 0.04))))
  (:Completed
    (Variables|Default|SetCurrentThrustSpeed 0.04)
    (bind _returnvalue (Utilities|Time|SetTimerbyEvent (delegate Custom|Refuel) 0.01 true true))))

(event Input|EnhancedActionEvents|EnhancedInputActionIA_RotateL
  (params (ActionValue :type Float%20%28double-precision%29) (ElapsedSeconds :type Float%20%28double-precision%29) (TriggeredSeconds :type Float%20%28double-precision%29) (InputAction :type Input%20Action%20Object%20Reference :default "/Game/Blueprints/Input/IA_RotateL.IA_RotateL")))

(event Input|EnhancedActionEvents|EnhancedInputActionIA_RotateR
  (params (ActionValue :type Float%20%28double-precision%29) (ElapsedSeconds :type Float%20%28double-precision%29) (TriggeredSeconds :type Float%20%28double-precision%29) (InputAction :type Input%20Action%20Object%20Reference :default "/Game/Blueprints/Input/IA_RotateR.IA_RotateR"))
  (Transformation|AddWorldRotation (Variables|Default|GetSprite) (Math|Rotator|MakeRotator 0.0 0.0 (* ActionValue 3.2)) false false))

(event Input|EnhancedActionEvents|EnhancedInputActionIA_Thrusters
  (params (ActionValue :type Float%20%28double-precision%29) (ElapsedSeconds :type Float%20%28double-precision%29) (TriggeredSeconds :type Float%20%28double-precision%29) (InputAction :type Input%20Action%20Object%20Reference :default "/Game/Blueprints/Input/IA_Thrusters.IA_Thrusters"))
  (bind _currentthrustspeed (Variables|Default|GetCurrentThrustSpeed))
  (bind _sprite (Variables|Default|GetSprite))
  (bind _returnvalue (Math|Vector|GetForwardVector _sprite))
  (bind _returnvalue_2 (* ActionValue _currentthrustspeed))
  (:Triggered
    (Variables|Default|SetThrustSeconds TriggeredSeconds)
    (Transformation|AddWorldOffset (Variables|Default|GetSpringArm) (Math|Vector|MakeVector (+ (* (.x _returnvalue) _returnvalue_2) (.x (Variables|Default|GetCurrentMomentum))) (+ (* (.y _returnvalue) _returnvalue_2) (.y (Variables|Default|GetCurrentMomentum))) 0.0) false false)
    (Variables|Default|SetCurrentMomentum (Math|Vector|MakeVector (+ (* (.x _returnvalue) _returnvalue_2) (.x (Variables|Default|GetCurrentMomentum))) (+ (* (.y _returnvalue) _returnvalue_2) (.y (Variables|Default|GetCurrentMomentum))) 0.0))
    (if (== (Variables|Default|GetCurrentThrustSpeed) (Variables|Default|GetBoostSpeed))
      (Sprite|SetFlipbook _sprite "/Game/IMG/Player/FB_P1Boost.FB_P1Boost")
      (else
        (Sprite|SetFlipbook _sprite "/Game/IMG/Player/FB_P1_Thrust.FB_P1_Thrust"))))
  (:Completed
    (Variables|Default|SetThrustSeconds 0.0)
    (Sprite|SetFlipbook _sprite "/Game/IMG/Player/FB_P1Idle.FB_P1Idle")))

(event Input|EnhancedActionEvents|EnhancedInputActionIA_Shoot
  (params (ActionValue :type Boolean) (ElapsedSeconds :type Float%20%28double-precision%29) (TriggeredSeconds :type Float%20%28double-precision%29) (InputAction :type Input%20Action%20Object%20Reference :default "/Game/Blueprints/Input/IA_Shoot.IA_Shoot"))
  (Collision|LineTraceByChannel (Transformation|GetWorldLocation (Variables|Default|GetSprite)) (Transformation|GetWorldLocation (Variables|Default|GetAimPoint)) "TraceTypeQuery1" false 0 "ForDuration" true "(R=1.000000,G=1.000000,B=1.000000,A=1.000000)" "(R=0.000000,G=1.000000,B=0.000000,A=1.000000)" 1.0))

(event Input|EnhancedActionEvents|EnhancedInputActionIA_Teleport
  (params (ActionValue :type Boolean) (ElapsedSeconds :type Float%20%28double-precision%29) (TriggeredSeconds :type Float%20%28double-precision%29) (InputAction :type Input%20Action%20Object%20Reference :default "/Game/Blueprints/Input/IA_Teleport.IA_Teleport"))
  (Utilities|FlowControl|FlipFlop
    (:A
      (Variables|Default|SetTeleportLocation (Transformation|GetWorldLocation (Variables|Default|GetSprite)))
      (bind _returnvalue (Utilities|Time|SetTimerbyEvent (delegate Custom|CallLineTrace) 0.001 true true))
      (Variables|Default|SetTeleportTraceTimer _returnvalue))
    (:B
      (Utilities|Time|ClearandInvalidateTimerbyHandle (Variables|Default|GetTeleportTraceTimer))
      (Transformation|SetWorldLocation (Variables|Default|GetSprite) (Variables|Default|GetTeleportLocation) false false))))

(event Input|EnhancedActionEvents|EnhancedInputActionIA_CamScroll
  (params (ActionValue :type Float%20%28double-precision%29) (ElapsedSeconds :type Float%20%28double-precision%29) (TriggeredSeconds :type Float%20%28double-precision%29) (InputAction :type Input%20Action%20Object%20Reference :default "/Game/Blueprints/Input/IA_CamScroll.IA_CamScroll"))
  (Transformation|AddRelativeRotation (Variables|Default|GetSpringArm) (Math|Rotator|MakeRotator 0.0 ActionValue 0.0) false false))

(event Input|EnhancedActionEvents|EnhancedInputActionIA_Brake
  (params (ActionValue :type Boolean) (ElapsedSeconds :type Float%20%28double-precision%29) (TriggeredSeconds :type Float%20%28double-precision%29) (InputAction :type Input%20Action%20Object%20Reference :default "/Game/Blueprints/Input/IA_Brake.IA_Brake"))
  (bind _returnvalue (Utilities|Time|GetWorldDeltaSeconds))
  (:Triggered
    (Variables|Default|SetCurrentMomentum (Math|Vector|MakeVector (Math|Interpolation|FInterpTo (.x (Variables|Default|GetCurrentMomentum)) 0.0 _returnvalue 1.0) (Math|Interpolation|FInterpTo (.y (Variables|Default|GetCurrentMomentum)) 0.0 _returnvalue 1.0) 0.0))
    (Sprite|SetFlipbook (Variables|Default|GetSprite) "/Game/IMG/Player/FB_P1_Break.FB_P1_Break"))
  (:Completed
    (Sprite|SetFlipbook (Variables|Default|GetSprite) "/Game/IMG/Player/FB_P1Idle.FB_P1Idle")))

(event EventTick
  (params (DeltaSeconds :type Float%20%28single-precision%29))
  (bind _sprite (Variables|Default|GetSprite))
  (bind _returnvalue (Transformation|GetWorldRotation _sprite))
  (bind _yaw (Math|Rotator|BreakRotator _returnvalue))
  (Utilities|FlowControl|Sequence
    (:then_0
      (if (== (Variables|Default|GetThrustSeconds) 0.0)
        (Transformation|AddWorldOffset (Variables|Default|GetSprite) (Variables|Default|GetCurrentMomentum) false false)))
    (:then_1
      (Rendering|Material|SetVectorParameterValue "/Game/Widgets/MP_Minimap.MP_Minimap" "Player Location" (Math|Conversions|ToLinearColor(Vector) (Transformation|GetWorldLocation _sprite)) :!class /Script/Engine.KismetMaterialLibrary)
      (Rendering|Material|SetScalarParameterValue "/Game/Widgets/MP_Minimap.MP_Minimap" "Player Yaw" (/ (Math|Float|SelectFloat (+ _yaw 3.6e+02) _yaw (< _yaw 0.0)) 3.6e+02) :!class /Script/Engine.KismetMaterialLibrary))))

(event EventBeginPlay
  (bind _aspc_player (Utilities|Casting|CastToPC_Player (Game|GetPlayerController 0)))
  (Utilities|IsValid _aspc_player
    (:Is%20Valid
      (Utilities|IsValid (PlayerController|LocalPlayerSubsystems|GetEnhancedInputLocalPlayerSubsystem _aspc_player)
        (:Is%20Valid
          (Input|AddMappingContext (PlayerController|LocalPlayerSubsystems|GetEnhancedInputLocalPlayerSubsystem _aspc_player) "/Game/Blueprints/Input/IMC_Default.IMC_Default" 0 "(bIgnoreAllPressedKeysUntilRelease=True,bForceImmediately=False,bNotifyUserSettings=False)")
          (bind _returnvalue (UserInterface|CreateWidget "/Game/Widgets/OLDPlayerHUD.OLDPlayerHUD_C"))
          (UserInterface|Viewport|AddtoViewport _returnvalue 0))))))

(fn ConstructionScript
  (Transformation|SetWorldTransform (Variables|Default|GetSpawn%20Collision) (Math|Transform|MakeTransform (Math|Vector|MakeVector 0.0 0.0 2e+01) (Math|Rotator|MakeRotator 0.0 0.0 0.0) (Math|Vector|MakeVector 1.0 1.0 1.0)) true true))