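; BP_3dPawn is a player pawn that rotates and thrusts using Enhanced Input.
; BeginPlay adds IMC_Default through PC_Player, and the rotate actions yaw PlayerSprite left or right.
; Thrusters move PhysicsRoot along the sprite's XY forward vector by fixed world offsets, without delta time or applied forces.
; The construction script places PhysicsRoot at a fixed transform; Tick prints an empty string, and old HUD creation is disconnected.
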(event Input|EnhancedActionEvents|EnhancedInputActionIA_RotateR
  (params (ActionValue :type Float%20%28double-precision%29) (ElapsedSeconds :type Float%20%28double-precision%29) (TriggeredSeconds :type Float%20%28double-precision%29) (InputAction :type Input%20Action%20Object%20Reference :default "/Game/Blueprints/Input/IA_RotateR.IA_RotateR"))
  (Transformation|AddRelativeRotation (Variables|Default|GetPlayerSprite) (Math|Rotator|MakeRotator 0.0 0.0 (* ActionValue 7.0)) false false))

(event Input|EnhancedActionEvents|EnhancedInputActionIA_RotateL
  (params (ActionValue :type Float%20%28double-precision%29) (ElapsedSeconds :type Float%20%28double-precision%29) (TriggeredSeconds :type Float%20%28double-precision%29) (InputAction :type Input%20Action%20Object%20Reference :default "/Game/Blueprints/Input/IA_RotateL.IA_RotateL"))
  (Transformation|AddRelativeRotation (Variables|Default|GetPlayerSprite) (Math|Rotator|MakeRotator 0.0 0.0 (* ActionValue -7.0)) false false))

(event Input|EnhancedActionEvents|EnhancedInputActionIA_Thrusters
  (params (ActionValue :type Float%20%28double-precision%29) (ElapsedSeconds :type Float%20%28double-precision%29) (TriggeredSeconds :type Float%20%28double-precision%29) (InputAction :type Input%20Action%20Object%20Reference :default "/Game/Blueprints/Input/IA_Thrusters.IA_Thrusters"))
  (bind _playersprite (Variables|Default|GetPlayerSprite))
  (bind _returnvalue (Math|Vector|GetForwardVector _playersprite))
  (:Triggered
    (Transformation|AddWorldOffset (Variables|Default|GetPhysicsRoot) (Math|Vector|MakeVector (* (.x _returnvalue) 1e+01) (* (.y _returnvalue) 1e+01) 0.0) false false)))

(event EventTick
  (params (DeltaSeconds :type Float%20%28single-precision%29))
  (Development|PrintString "" true true "(R=0.000000,G=0.660000,B=1.000000,A=1.000000)" 0.05))

(event EventBeginPlay
  (bind _aspc_player (Utilities|Casting|CastToPC_Player (Game|GetPlayerController 0)))
  (Utilities|IsValid _aspc_player
    (:Is%20Valid
      (Utilities|IsValid (PlayerController|LocalPlayerSubsystems|GetEnhancedInputLocalPlayerSubsystem _aspc_player)
        (:Is%20Valid
          (Input|AddMappingContext (PlayerController|LocalPlayerSubsystems|GetEnhancedInputLocalPlayerSubsystem _aspc_player) "/Game/Blueprints/Input/IMC_Default.IMC_Default" 0 "(bIgnoreAllPressedKeysUntilRelease=True,bForceImmediately=False,bNotifyUserSettings=False)"))))))

(fn ConstructionScript
  (Transformation|SetWorldTransform (Variables|Default|GetPhysicsRoot) (Math|Transform|MakeTransform (Math|Vector|MakeVector 0.0 0.0 2e+01) (Math|Rotator|MakeRotator 0.0 0.0 0.0) (Math|Vector|MakeVector 1.0 1.0 1.0)) true true))