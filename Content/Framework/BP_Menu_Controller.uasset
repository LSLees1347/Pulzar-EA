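; Player controller for the menu and multiplayer lobby, managing lobby, character and loading-screen widgets with UI-only input.
; It loads the saved player profile and sends it, ready state and character picks to BP_Menu_Gamemode through server events.
; Update events push names, readiness, level, duration and gamemode into the lobby widget.
; Menu switches blend the camera between pawn and lobby character, routing remote clients through server events.
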(event Custom|EndClientSession
  (|DestroySession self
    (:then
      (Game|OpenLevel(byName) "MainMenu"))))

(event Custom|CreateLoadScreen
  (CallFunction|UIShowLoadScreen))

(event Custom|Svr_UpdatePlayerReady
  (params (IsReady :type Boolean))
  (bind _asbp_menu_gamemode (Utilities|Casting|CastToBP_Menu_Gamemode (Game|GetGameMode)))
  (Default|SetPlayerReady _asbp_menu_gamemode self IsReady))

(event Custom|UpdatePlayerReady
  (params (IsPlayerReady :type Array%20of%20Booleans))
  (bind _wbp_lobbymenu (Variables|Default|GetWBP_LobbyMenu))
  (Utilities|IsValid _wbp_lobbymenu
    (:Is%20Valid
      (Default|UpdatePlayersReady _wbp_lobbymenu IsPlayerReady))))

(event Custom|Update%20Match%20Duration
  (params (InText :type Text))
  (bind _wbp_lobbymenu (Variables|Default|GetWBP_LobbyMenu))
  (Utilities|IsValid _wbp_lobbymenu
    (:Is%20Valid
      (Default|UpdateDuration _wbp_lobbymenu InText))))

(event Custom|Update%20Gamemode
  (params (Gamemode :type E_Gamemodes%20Enum :default "NewEnumerator1"))
  (bind _wbp_lobbymenu (Variables|Default|GetWBP_LobbyMenu))
  (Utilities|IsValid _wbp_lobbymenu
    (:Is%20Valid
      (Default|UpdateGamemode _wbp_lobbymenu Gamemode))))

(event Custom|CreateLobbyMenu
  (CallFunction|UIShowNewLobby))

(event Custom|UpdateLevelSelection
  (params (LevelRowName :type Name))
  (bind _wbp_lobbymenu (Variables|Default|GetWBP_LobbyMenu))
  (Utilities|IsValid _wbp_lobbymenu
    (:Is%20Valid
      (Default|UpdateLevelSelection _wbp_lobbymenu LevelRowName))))

(event Custom|Initial_Setup
  (CallFunction|LoadSavedProfile)
  (CallFunction|ServerUpdateLobby (Variables|Default|GetPlayerProfileInfo)))

(event Custom|UpdatePlayerNames
  (params (PlayerProfiles :type Array%20of%20S%20Player%20Profile%20Structures))
  (bind _wbp_lobbymenu (Variables|Default|GetWBP_LobbyMenu))
  (Utilities|IsValid _wbp_lobbymenu
    (:Is%20Valid
      (Default|ClearPlayerNames _wbp_lobbymenu)
      (Default|UpdatePlayerNames _wbp_lobbymenu PlayerProfiles))))

(event Custom|Server_UpdateLobby
  (params (PlayerProfile :type S%20Player%20Profile%20Structure))
  (Variables|Default|SetPlayerProfileInfo PlayerProfile)
  (bind _asbp_menu_gamemode (Utilities|Casting|CastToBP_Menu_Gamemode (Game|GetGameMode)))
  (Default|UpdateLobby _asbp_menu_gamemode true true true true true true))

(event Custom|Svr_SetViewTarget_Normal
  (Game|Player|SetViewTargetwithBlend (Pawn|GetControlledPawn) 1.0 "VTBlend_Cubic" 1e+01 false))

(event Custom|Svr_SetViewTarget_Char
  (Game|Player|SetViewTargetwithBlend (Variables|/Script/Engine.ChildActorComponent|GetChildActor (Variables|/Game/Player/Lobby/BP_Lobby_Character.BP_Lobby_Character_C|GetViewTarget (Variables|Default|GetBP_LobbyCharacter))) 1.0 "VTBlend_Cubic" 1e+01 false))

(event Custom|Svr_UpdateSelectedChar
  (params (PlayerProfileInfo :type S%20Player%20Profile%20Structure))
  (bind _output_get (Variables|Default|SetPlayerProfileInfo PlayerProfileInfo))
  (bind _asbp_menu_gamemode (Utilities|Casting|CastToBP_Menu_Gamemode (Game|GetGameMode)))
  (Default|UpdateCharforController _asbp_menu_gamemode self _output_get))

(event EventBeginPlay
  (if (Pawn|IsLocalController)
    (Variables|Default|SetbShowMouseCursor true)
    (Input|SetInputModeUIOnly self 0 "DoNotLock" false)))

(fn ConstructionScript)

(fn UIShowLobbyMenu
  (Utilities|IsValid (Variables|Default|GetWBP_LobbyMenu)
    (:Is%20Valid
      _)
    (:Is%20Not%20Valid
      (bind _returnvalue (UserInterface|CreateWidget "/Game/Widgets/Main/WBP_LobbyMenu.WBP_LobbyMenu_C" self))
      (Variables|Default|SetWBP_LobbyMenu _returnvalue)))
  (UserInterface|Viewport|AddtoViewport (Variables|Default|GetWBP_LobbyMenu) 0)
  (Networking|SwitchHasAuthority
    (:Authority
      (Game|Player|SetViewTargetwithBlend (Pawn|GetControlledPawn) 0.5 "VTBlend_Linear" 0.0 false))
    (:Remote
      (CallFunction|SvrSetViewTargetNormal)))
  (return))

(fn LoadSavedProfile
  (bind _returnvalue (SaveGame|DoesSaveGameExist (LocalVariables|GetLcl_SlotName)))
  (if _returnvalue
    _
    (else
      (bind _returnvalue_2 (SaveGame|CreateSaveGameObject "/Game/SaveData/SG_PlayerProfile.SG_PlayerProfile_C"))
      (SaveGame|SaveGametoSlot _returnvalue_2 (LocalVariables|GetLcl_SlotName))))
  (bind _returnvalue_3 (SaveGame|LoadGamefromSlot (LocalVariables|GetLcl_SlotName)))
  (bind _assg_player_profile (Utilities|Casting|CastToSG_PlayerProfile _returnvalue_3))
  (Variables|Default|SetPlayerProfileInfo (Variables|/Game/SaveData/SG_PlayerProfile.SG_PlayerProfile_C|GetPlayerProfile _assg_player_profile))
  (return))

(fn UIShowLoadScreen
  (Viewport|RemoveAllWidgets)
  (Utilities|IsValid (Variables|Default|GetWPB_LoadScreen)
    (:Is%20Valid
      _)
    (:Is%20Not%20Valid
      (bind _returnvalue (UserInterface|CreateWidget "/Game/Widgets/Deprecated/WBP_LoadingScreen.WBP_LoadingScreen_C" self))
      (Variables|Default|SetWPB_LoadScreen _returnvalue)))
  (UserInterface|Viewport|AddtoViewport (Variables|Default|GetWPB_LoadScreen) 0))

(fn UIShowCharacterMenu
  (Utilities|IsValid (Variables|Default|GetWPB_CharacterMenu)
    (:Is%20Valid
      _)
    (:Is%20Not%20Valid
      (bind _returnvalue (UserInterface|CreateWidget "/Game/Widgets/Main/WBP_CharacterMenu.WBP_CharacterMenu_C" self))
      (Variables|Default|SetWPB_CharacterMenu _returnvalue)))
  (UserInterface|Viewport|AddtoViewport (Variables|Default|GetWPB_CharacterMenu) 0)
  (Networking|SwitchHasAuthority
    (:Authority
      (Game|Player|SetViewTargetwithBlend (Variables|/Script/Engine.ChildActorComponent|GetChildActor (Variables|/Game/Player/Lobby/BP_Lobby_Character.BP_Lobby_Character_C|GetViewTarget (Variables|Default|GetBP_LobbyCharacter))) 1.0 "VTBlend_Cubic" 1e+01 false))
    (:Remote
      (CallFunction|SvrSetViewTargetChar)))
  (return))

(fn SaveSelectedCharacter
  (params (CharRowName :type Name) (Player%20Profile%20Info%20Character%20Class :type Actor%20Class%20Reference))
  (Variables|Default|SetPlayerProfileInfo (Utilities|Struct|MakeS_PlayerProfile (.playername (Variables|Default|GetPlayerProfileInfo)) CharRowName Player%20Profile%20Info%20Character%20Class (.playerxp (Variables|Default|GetPlayerProfileInfo)) (.playerlevel (Variables|Default|GetPlayerProfileInfo)) (.xptilllevelup (Variables|Default|GetPlayerProfileInfo))))
  (Utilities|IsValid (Variables|Default|GetSG_PlayerProfile)
    (:Is%20Valid
      _)
    (:Is%20Not%20Valid
      (bind _returnvalue (SaveGame|CreateSaveGameObject "/Game/SaveData/SG_PlayerProfile.SG_PlayerProfile_C"))
      (Variables|Default|SetSG_PlayerProfile _returnvalue)))
  (Variables|/Game/SaveData/SG_PlayerProfile.SG_PlayerProfile_C|SetPlayerProfile (Variables|Default|GetSG_PlayerProfile) (Variables|Default|GetPlayerProfileInfo))
  (SaveGame|SaveGametoSlot (Variables|Default|GetSG_PlayerProfile) "PlayerProfileSlot")
  (bind _asbp_game_instance (Utilities|Casting|CastToBP_GameInstance (Game|GetGameInstance)))
  (if (Variables|/Game/Framework/BP_GameInstance.BP_GameInstance_C|GetIsSoloGame _asbp_game_instance)
    _
    (else
      (CallFunction|SvrUpdateSelectedChar (Variables|Default|GetPlayerProfileInfo))))
  (return))

(fn UIShowNewLobby
  (Utilities|IsValid (Variables|Default|GetWBP_NewLobby)
    (:Is%20Valid
      _)
    (:Is%20Not%20Valid
      (bind _returnvalue (UserInterface|CreateWidget "/Game/Widgets/WBP_MainMenu.WBP_MainMenu_C" self))
      (Variables|Default|SetWBP_NewLobby _returnvalue)))
  (UserInterface|Viewport|AddtoViewport (Variables|Default|GetWBP_NewLobby) 0)
  (Networking|SwitchHasAuthority
    (:Authority
      (Game|Player|SetViewTargetwithBlend (Pawn|GetControlledPawn) 0.5 "VTBlend_Linear" 0.0 false))
    (:Remote
      (CallFunction|SvrSetViewTargetNormal)))
  (return))