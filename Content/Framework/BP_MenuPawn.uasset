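; BP_MenuPawn is a menu pawn that sets up the player's Enhanced Input.
; On BeginPlay it caches the BP_Menu_Controller and adds IMC_Player to that controller's Enhanced Input local player subsystem.
; A separate LoadKeybings function gets user input settings from the controller and registers IMC_Player if it is not already registered.
; Nothing in this file calls that function, and its MapPlayerKey call is disconnected.
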(event EventBeginPlay
  (bind _asbp_menu_controller (Utilities|Casting|CastToBP_Menu_Controller (Game|GetPlayerController 0)))
  (Utilities|IsValid _asbp_menu_controller
    (:Is%20Valid
      (Variables|Default|SetAs%20BP%20Menu%20Controller _asbp_menu_controller)
      (Utilities|IsValid (PlayerController|LocalPlayerSubsystems|GetEnhancedInputLocalPlayerSubsystem _asbp_menu_controller)
        (:Is%20Valid
          (Input|AddMappingContext (PlayerController|LocalPlayerSubsystems|GetEnhancedInputLocalPlayerSubsystem _asbp_menu_controller) "/Game/Player/Input/IMC_Player.IMC_Player" 0 "(bIgnoreAllPressedKeysUntilRelease=True,bForceImmediately=False,bNotifyUserSettings=False)"))))))

(fn ConstructionScript)

(fn LoadKeybings
  (bind _returnvalue (Class|EnhancedInputSubsystemInterface|GetUserSettings(Message) (Variables|Default|GetAs%20BP%20Menu%20Controller)))
  (bind _output_get (Variables|Default|SetUser%20Input%20Settings _returnvalue))
  (Utilities|IsValid _output_get
    (:Is%20Valid
      (if (not (Class|EnhancedInputUserSettings|IsMappingContextRegistered (Variables|Default|GetUser%20Input%20Settings) "/Game/Player/Input/IMC_Player.IMC_Player"))
        (Class|EnhancedInputUserSettings|RegisterInputMappingContext (Variables|Default|GetUser%20Input%20Settings) "/Game/Player/Input/IMC_Player.IMC_Player")))))