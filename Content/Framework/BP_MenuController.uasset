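; Player controller for the multiplayer menu and lobby, handling loading, lobby and character screens with UI-only input.
; It loads the saved player profile and sends it to BP_Menu_Gamemode through server events, which refresh lobby names, level and character selection.
; Opening the lobby or character menu blends the camera to the pawn or lobby character, with clients routing through server events.
; Character choices are saved locally and sent to the server.
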(event Custom|EndClientSession
  (|DestroySession self
    (:then
      (Game|OpenLevel(byName) "MainMenu"))))

(event Custom|CreateLoadScreen
  (CallFunction|UIShowLoadScreen))

(event Custom|CreateLobbyMenu
  (CallFunction|UIShowLobbyMenu))

(event Custom|UpdateLevelSelection
  (params (LevelRowName :type Name))
  (bind _wpb_lobbymenu (Variables|Default|GetWPB_LobbyMenu))
  (Utilities|IsValid _wpb_lobbymenu
    (:Is%20Valid
      (Default|UpdateLevelSelection _wpb_lobbymenu LevelRowName))))

(event Custom|Initial_Setup
  (CallFunction|LoadSavedProfile)
  (CallFunction|ServerUpdateLobby (Variables|Default|GetPlayerProfileInfo)))

(event Custom|UpdatePlayerNames
  (params (PlayerProfiles :type Array%20of%20S%20Player%20Profile%20Structures))
  (bind _wpb_lobbymenu (Variables|Default|GetWPB_LobbyMenu))
  (Utilities|IsValid _wpb_lobbymenu
    (:Is%20Valid
      (Default|ClearPlayerNames _wpb_lobbymenu)
      (Default|UpdatePlayerNames _wpb_lobbymenu PlayerProfiles))))

(event Custom|Server_UpdateLobby
  (params (PlayerProfile :type S%20Player%20Profile%20Structure))
  (Variables|Default|SetPlayerProfileInfo PlayerProfile)
  (bind _asbp_menu_gamemode (Utilities|Casting|CastToBP_Menu_Gamemode (Game|GetGameMode)))
  (Default|UpdateLobby _asbp_menu_gamemode true true true))

(event Custom|Svr_SetViewTarget_Normal
  (Game|Player|SetViewTargetwithBlend (Pawn|GetControlledPawn) 1.0 "VTBlend_Cubic" 1e+01 false))

(event Custom|Svr_SetViewTarget_Char
  (Game|Player|SetViewTargetwithBlend (Variables|/Script/Engine.ChildActorComponent|GetChildActor (Variables|/Game/Player/Lobby/BP_Lobby_Character.BP_Lobby_Character_C|GetViewTarget (Variables|Default|GetBP_LobbyCharacter))) 1.0 "VTBlend_Cubic" 1e+01 false))

(event Custom|Svr_UpdateSelectedChar
  (params (PlayerProfileInfo :type S%20Player%20Profile%20Structure))
  (bind _output_get (Variables|Default|SetPlayerProfileInfo PlayerProfileInfo))
  (bind _asbp_menu_gamemode (Utilities|Casting|CastToBP_Menu_Gamemode (Game|GetGameMode)))
  (Default|UpdateCharforController _asbp_menu_gamemode self _output_get))

(event EventBeginPlay
  (if (Pawn|IsLocalController)
    (Variables|Default|SetbShowMouseCursor true)
    (Input|SetInputModeUIOnly self 0 "DoNotLock" false)))

(fn ConstructionScript)

(fn UIShowLobbyMenu
  (Utilities|IsValid (Variables|Default|GetWPB_LobbyMenu)
    (:Is%20Valid
      _)
    (:Is%20Not%20Valid
      (bind _returnvalue (UserInterface|CreateWidget "/Game/Widgets/WPB_LobbyMenu.WPB_LobbyMenu_C" self))
      (Variables|Default|SetWPB_LobbyMenu _returnvalue)))
  (UserInterface|Viewport|AddtoViewport (Variables|Default|GetWPB_LobbyMenu) 0)
  (Networking|SwitchHasAuthority
    (:Authority
      (Game|Player|SetViewTargetwithBlend (Pawn|GetControlledPawn) 0.5 "VTBlend_Linear" 0.0 false))
    (:Remote
      (CallFunction|SvrSetViewTargetNormal)))
  (return))

(fn LoadSavedProfile
  (bind _returnvalue (SaveGame|DoesSaveGameExist (LocalVariables|GetLcl_SlotName)))
  (if _returnvalue
    _
    (else
      (bind _returnvalue_2 (SaveGame|CreateSaveGameObject))
      (SaveGame|SaveGametoSlot _returnvalue_2 (LocalVariables|GetLcl_SlotName))))
  (bind _returnvalue_3 (SaveGame|LoadGamefromSlot (LocalVariables|GetLcl_SlotName)))
  (bind _assg_player_profile (Utilities|Casting|CastToSG_PlayerProfile _returnvalue_3))
  (Variables|Default|SetPlayerProfileInfo (Variables|/Game/SaveData/SG_PlayerProfile.SG_PlayerProfile_C|GetPlayerProfile _assg_player_profile))
  (return))

(fn UIShowLoadScreen
  (Viewport|RemoveAllWidgets)
  (Utilities|IsValid (Variables|Default|GetWPB_LoadScreen)
    (:Is%20Valid
      _)
    (:Is%20Not%20Valid
      (bind _returnvalue (UserInterface|CreateWidget "/Game/Widgets/WPB_LoadingScreen.WPB_LoadingScreen_C" self))
      (Variables|Default|SetWPB_LoadScreen _returnvalue)))
  (UserInterface|Viewport|AddtoViewport (Variables|Default|GetWPB_LoadScreen) 0))

(fn UIShowCharacterMenu
  (Utilities|IsValid (Variables|Default|GetWPB_CharacterMenu)
    (:Is%20Valid
      _)
    (:Is%20Not%20Valid
      (bind _returnvalue (UserInterface|CreateWidget "/Game/Widgets/WPB_CharacterMenu.WPB_CharacterMenu_C" self))
      (Variables|Default|SetWPB_CharacterMenu _returnvalue)))
  (UserInterface|Viewport|AddtoViewport (Variables|Default|GetWPB_CharacterMenu) 0)
  (Networking|SwitchHasAuthority
    (:Authority
      (Game|Player|SetViewTargetwithBlend (Variables|/Script/Engine.ChildActorComponent|GetChildActor (Variables|/Game/Player/Lobby/BP_Lobby_Character.BP_Lobby_Character_C|GetViewTarget (Variables|Default|GetBP_LobbyCharacter))) 1.0 "VTBlend_Cubic" 1e+01 false))
    (:Remote
      (CallFunction|SvrSetViewTargetChar)))
  (return))

(fn SaveSelectedCharacter
  (params (CharRowName :type Name) (Player%20Profile%20Info%20Character%20Class :type Actor%20Class%20Reference))
  (Variables|Default|SetPlayerProfileInfo (Utilities|Struct|MakeS_PlayerProfile (.playername (Variables|Default|GetPlayerProfileInfo)) CharRowName Player%20Profile%20Info%20Character%20Class (.playerxp (Variables|Default|GetPlayerProfileInfo))))
  (Utilities|IsValid (Variables|Default|GetSG_PlayerProfile)
    (:Is%20Valid
      _)
    (:Is%20Not%20Valid
      (bind _returnvalue (SaveGame|CreateSaveGameObject "/Game/SaveData/SG_PlayerProfile.SG_PlayerProfile_C"))
      (Variables|Default|SetSG_PlayerProfile _returnvalue)))
  (Variables|/Game/SaveData/SG_PlayerProfile.SG_PlayerProfile_C|SetPlayerProfile (Variables|Default|GetSG_PlayerProfile) (Variables|Default|GetPlayerProfileInfo))
  (SaveGame|SaveGametoSlot 0 "PlayerProfileSlot")
  (CallFunction|SvrUpdateSelectedChar (Variables|Default|GetPlayerProfileInfo))
  (return))