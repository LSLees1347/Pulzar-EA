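; Game mode for the menu and multiplayer lobby that tracks connected controllers, their profiles and ready states.
; Players joining on the lobby map get a lobby menu, and UpdateLobby pushes names, level, characters and readiness to every controller, copying profiles into PlayerStates.
; Each player gets a lobby character at a free spot, with name and data-table flipbook set; logout removes it and frees the spot.
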(event Custom|UpdateLobby
  (params (PlayerNames :type Boolean) (LevelSelection :type Boolean) (CharacterSelection :type Boolean) (PlayersReady :type Boolean))
  (Utilities|Array|Clear (Variables|Default|GetAll_PlayerProfiles))
  (for (_array_element _array_index) (Variables|Default|GetAllConnectedPlayers)
    (Utilities|Array|SetArrayElem (Variables|Default|GetAll_PlayerProfiles) _array_index (Variables|/Game/Framework/BP_MenuController.BP_MenuController_C|GetPlayerProfileInfo _array_element) true)
    (bind _asbp_standard_playerstate (Utilities|Casting|CastToBP_Standard_Playerstate (Variables|/Script/Engine.Controller|GetPlayerState _array_element)))
    (Variables|/Game/Framework/BP_Standard_Playerstate.BP_Standard_Playerstate_C|SetS_PlayerProfile _asbp_standard_playerstate (Variables|/Game/Framework/BP_MenuController.BP_MenuController_C|GetPlayerProfileInfo _array_element)))
  (for (_array_element_2 _array_index_2) (Variables|Default|GetAllConnectedPlayers)
    (if PlayerNames
      (Default|UpdatePlayerNames _array_element_2 (Variables|Default|GetAll_PlayerProfiles)))
    (if LevelSelection
      (Default|UpdateLevelSelection _array_element_2 (Variables|Default|GetSelectedLevelName)))
    (if CharacterSelection
      (CallFunction|UpdateSelectedCharacter _array_index_2))
    (if PlayersReady
      (Default|UpdatePlayerReady _array_element_2 (Variables|Default|GetIsPlayerReady)))))

(event Custom|UpdateSelectedCharacter
  (params (PlayerIndex :type Integer))
  (bind _allconnectedplayers (Variables|Default|GetAllConnectedPlayers))
  (bind _all_playerprofiles (Variables|Default|GetAll_PlayerProfiles))
  (bind _output (Utilities|Array|Get(acopy) _allconnectedplayers PlayerIndex))
  (bind _output_2 (Utilities|Array|Get(acopy) _all_playerprofiles PlayerIndex))
  (bind (_playername _characterrowname) (Utilities|Struct|BreakS_PlayerProfile _output_2))
  (if (== (Variables|/Game/Framework/BP_MenuController.BP_MenuController_C|GetBP_LobbyCharacter (Utilities|Array|Get(acopy) (Variables|Default|GetAllConnectedPlayers) PlayerIndex)) 0)
    (bind _avaliableplayerspot (CallFunction|GetLobbyPlayerSpot))
    (Variables|/Game/Player/Lobby/BP_LobbyPlayerSpot.BP_LobbyPlayerSpot_C|SetIsSpotUsed _avaliableplayerspot true)
    (bind _returnvalue (Game|SpawnActorfromClass "/Game/Player/Lobby/BP_Lobby_Character.BP_Lobby_Character_C" (Transformation|GetActorTransform _avaliableplayerspot) "Undefined" "MultiplyWithRoot" 0 0))
    (Variables|/Game/Framework/BP_MenuController.BP_MenuController_C|SetBP_LobbyCharacter _output _returnvalue)
    (Variables|/Game/Framework/BP_MenuController.BP_MenuController_C|SetBP_LobbyPlayerSpot _output _avaliableplayerspot))
  (Default|MCSetPlayerName (Variables|/Game/Framework/BP_MenuController.BP_MenuController_C|GetBP_LobbyCharacter (Utilities|Array|Get(acopy) (Variables|Default|GetAllConnectedPlayers) PlayerIndex)) _playername)
  (bind _returnvalue_2 (Utilities|GetDataTableRow "/Game/Player/CharacterInfoTable.CharacterInfoTable" _characterrowname)
    (:then
      (Default|MCSetFlipbook (Variables|/Game/Framework/BP_MenuController.BP_MenuController_C|GetBP_LobbyCharacter (Utilities|Array|Get(acopy) (Variables|Default|GetAllConnectedPlayers) PlayerIndex)) (Utilities|Struct|BreakS_CharacterInfo _returnvalue_2)))))

(event Custom|UpdateCharForController
  (params (Controller :type BP%20Menu%20Controller%20Object%20Reference) (PlayerProfile :type S%20Player%20Profile%20Structure))
  (bind _allconnectedplayers (Variables|Default|GetAllConnectedPlayers))
  (bind _returnvalue (Utilities|Array|FindItem _allconnectedplayers Controller))
  (Utilities|Array|SetArrayElem (Variables|Default|GetAll_PlayerProfiles) _returnvalue PlayerProfile true)
  (CallFunction|UpdateSelectedCharacter _returnvalue)
  (bind _asbp_standard_playerstate (Utilities|Casting|CastToBP_Standard_Playerstate (Variables|/Script/Engine.Controller|GetPlayerState Controller)))
  (Variables|/Game/Framework/BP_Standard_Playerstate.BP_Standard_Playerstate_C|SetS_PlayerProfile _asbp_standard_playerstate PlayerProfile))

(event Custom|SetPlayerReady
  (params (PlayerController :type BP%20Menu%20Controller%20Object%20Reference) (IsReady :type Boolean))
  (Utilities|Array|SetArrayElem (Variables|Default|GetIsPlayerReady) (Utilities|Array|FindItem (Variables|Default|GetAllConnectedPlayers) PlayerController) IsReady)
  (CallFunction|UpdateLobby false false false true))

(event EventOnLogout
  (params (ExitingController :type Controller%20Object%20Reference))
  (bind _asbp_menu_controller (Utilities|Casting|CastToBP_MenuController ExitingController))
  (if (== (Variables|/Game/Framework/BP_MenuController.BP_MenuController_C|GetBP_LobbyCharacter _asbp_menu_controller) 0)
    _
    (else
      (Actor|DestroyActor (Variables|/Game/Framework/BP_MenuController.BP_MenuController_C|GetBP_LobbyCharacter _asbp_menu_controller))
      (Variables|/Game/Player/Lobby/BP_LobbyPlayerSpot.BP_LobbyPlayerSpot_C|SetIsSpotUsed (Variables|/Game/Framework/BP_MenuController.BP_MenuController_C|GetBP_LobbyPlayerSpot _asbp_menu_controller) false)))
  (Utilities|Array|RemoveIndex (Variables|Default|GetIsPlayerReady) (Utilities|Array|FindItem (Variables|Default|GetAllConnectedPlayers) _asbp_menu_controller))
  (Utilities|Array|RemoveIndex (Variables|Default|GetAllConnectedPlayers) (Utilities|Array|FindItem (Variables|Default|GetAllConnectedPlayers) _asbp_menu_controller))
  (CallFunction|UpdateLobby true false true true))

(event EventBeginPlay
  (bind _asbp_game_instance (Utilities|Casting|CastToBP_GameInstance (Game|GetGameInstance)))
  (Variables|Default|SetbUseSeamlessTravel (Variables|/Game/Framework/BP_GameInstance.BP_GameInstance_C|GetSeamlessTravelCarry _asbp_game_instance))
  (bind _returnvalue (Game|SpawnActorfromClass "/Game/Framework/BP_MenuPawn.BP_MenuPawn_C" (Math|Transform|MakeTransform "0, 0, 0" "0, 0, 0" "1.000000,1.000000,1.000000") "Undefined" "MultiplyWithRoot" 0 0))
  (Pawn|Possess (Game|GetPlayerController 0) _returnvalue))

(event EventHandleStartingNewPlayer
  (params (NewPlayer :type Player%20Controller%20Object%20Reference))
  (bind _returnvalue (Game|GetCurrentLevelName true))
  (switch string _returnvalue
    (:LobbyMenuMap
      (bind _asbp_menu_controller (Utilities|Casting|CastToBP_MenuController NewPlayer))
      (bind _returnvalue_2 (Utilities|Array|Add (Variables|Default|GetAllConnectedPlayers) _asbp_menu_controller))
      (Utilities|Array|SetArrayElem (Variables|Default|GetIsPlayerReady) _returnvalue_2 false true)
      (Default|CreateLobbyMenu _asbp_menu_controller)
      (Default|InitialSetup _asbp_menu_controller))))

(fn ConstructionScript)

(fn GetLobbyPlayerSpot
  (if (== (Utilities|Array|Length (Variables|Default|GetAll_LobbyPlayerSpots)) 0)
    (bind _outactors (Actor|GetAllActorsOfClass "/Game/Player/Lobby/BP_LobbyPlayerSpot.BP_LobbyPlayerSpot_C"))
    (Variables|Default|SetAll_LobbyPlayerSpots _outactors))
  (bind _array_element (Utilities|Array|ForEachLoopwithBreak (Variables|Default|GetAll_LobbyPlayerSpots) :!label _label)
    (:LoopBody
      (if (not (Variables|/Game/Player/Lobby/BP_LobbyPlayerSpot.BP_LobbyPlayerSpot_C|GetIsSpotUsed _array_element))
        (goto _label Break)))
    (:Completed
      (return _array_element))))