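; Multiplayer game mode that runs Free for All, Possession and Football matches for ship characters, plus solo games.
; It gathers controllers, polls each tick until all are ready, then spawns each profile's ship at an indexed start.
; Multiplayer starts spawn mode actors (orb or ball), run a countdown and start the match timer.
; Timer expiry triggers game over (XP, server travel) for Free for All and Possession, but not Football.
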(event Custom|LevelStart
  (Utilities|FlowControl|Delay 0.1)
  (for _array_element (Variables|Default|GetAll_ConnectedControllers)
    (Default|GameStartCountdown _array_element))
  (Utilities|FlowControl|Delay 3.0)
  (for _array_element_2 (Variables|Default|GetAll_ConnectedControllers)
    (Default|EnableAllInput _array_element_2)))

(event Custom|LevelStartFootball
  (bind _asbp_game_instance (Utilities|Casting|CastToBP_GameInstance (Game|GetGameInstance)))
  (bind _output_get (Variables|Default|SetMatchDuration (Variables|/Game/Framework/BP_GameInstance.BP_GameInstance_C|GetActiveDuration _asbp_game_instance)))
  (Variables|Default|SetMatchLength _output_get)
  (CallFunction|SpawnGameplayActors)
  (for _array_element (Variables|Default|GetAll_ConnectedControllers)
    (Default|GameStartCountdown _array_element)
    (if (> (Variables|Default|GetMatchDuration) 0)
      (Default|HUDSetupMatchTimer _array_element (Variables|Default|GetMatchDuration))))
  (Utilities|FlowControl|Delay 3.0)
  (for _array_element_2 (Variables|Default|GetAll_ConnectedControllers)
    (Default|EnableAllInput _array_element_2)
    (Default|HUDStartMatchFFA _array_element_2))
  (if (> (Variables|Default|GetMatchDuration) 0)
    (bind _returnvalue (Utilities|Time|SetTimerbyFunctionName 0 "MatchTimerInterval" 1.0 true))
    (Variables|Default|SetMatchTimerHandle _returnvalue)))

(event Custom|GM_FFA_GameOver
  (for _array_element (Variables|Default|GetAll_ConnectedControllers)
    (Default|ShowGameOverScreen _array_element)
    (Default|AddPlayerXP _array_element (Variables|Default|GetMatchLength)))
  (Utilities|FlowControl|Delay 8.0)
  (bind _asbp_game_instance (Utilities|Casting|CastToBP_GameInstance (Game|GetGameInstance)))
  (if (Variables|/Game/Framework/BP_GameInstance.BP_GameInstance_C|GetIsSoloGame _asbp_game_instance)
    (Development|ExecuteConsoleCommand "servertravel MainMenu" (Game|GetPlayerController 0))
    (else
      (Development|ExecuteConsoleCommand "servertravel LobbyMenuMap" (Game|GetPlayerController 0)))))

(event Custom|GM_FB_GameOver
  (bind _returnvalue (Game|GetPlayerController 0))
  (for _array_element (Variables|Default|GetAll_ConnectedControllers)
    (Default|ShowGameOverScreen _array_element)
    (Default|AddPlayerXP _array_element (Variables|Default|GetMatchLength)))
  (Utilities|FlowControl|Delay 8.0)
  (bind _asbp_game_instance (Utilities|Casting|CastToBP_GameInstance (Game|GetGameInstance)))
  (if (Variables|/Game/Framework/BP_GameInstance.BP_GameInstance_C|GetIsSoloGame _asbp_game_instance)
    (Development|ExecuteConsoleCommand "servertravel MainMenu" _returnvalue)
    (else
      (Development|ExecuteConsoleCommand "servertravel LobbyMenuMap" _returnvalue))))

(event Custom|LevelStartPossession
  (bind _asbp_game_instance (Utilities|Casting|CastToBP_GameInstance (Game|GetGameInstance)))
  (bind _output_get (Variables|Default|SetMatchDuration (Variables|/Game/Framework/BP_GameInstance.BP_GameInstance_C|GetActiveDuration _asbp_game_instance)))
  (Variables|Default|SetMatchLength _output_get)
  (CallFunction|SpawnGameplayActors)
  (for _array_element (Variables|Default|GetAll_ConnectedControllers)
    (Default|GameStartCountdown _array_element)
    (if (> (Variables|Default|GetMatchDuration) 0)
      (Default|HUDSetupMatchTimer _array_element (Variables|Default|GetMatchDuration))))
  (Utilities|FlowControl|Delay 3.0)
  (for _array_element_2 (Variables|Default|GetAll_ConnectedControllers)
    (Default|EnableAllInput _array_element_2)
    (Default|HUDStartMatchFFA _array_element_2))
  (if (> (Variables|Default|GetMatchDuration) 0)
    (bind _returnvalue (Utilities|Time|SetTimerbyFunctionName 0 "MatchTimerInterval" 1.0 true))
    (Variables|Default|SetMatchTimerHandle _returnvalue)))

(event Custom|GM_Pos_GameOver
  (for _array_element (Variables|Default|GetAll_ConnectedControllers)
    (Default|ShowGameOverScreen _array_element)
    (Default|AddPlayerXP _array_element (Variables|Default|GetMatchLength)))
  (Utilities|FlowControl|Delay 8.0)
  (bind _asbp_game_instance (Utilities|Casting|CastToBP_GameInstance (Game|GetGameInstance)))
  (if (Variables|/Game/Framework/BP_GameInstance.BP_GameInstance_C|GetIsSoloGame _asbp_game_instance)
    (Development|ExecuteConsoleCommand "servertravel MainMenu" (Game|GetPlayerController 0))
    (else
      (Development|ExecuteConsoleCommand "servertravel LobbyMenuMap" (Game|GetPlayerController 0)))))

(event Custom|ReturnTo%20Lobby
  (Development|ExecuteConsoleCommand "servertravel LobbyMenuMap" (Game|GetPlayerController 0)))

(event Custom|SpawnGameplayActors
  (switch Utilities|FlowControl|Switch|SwitchonE_Gamemodes (Variables|Default|GetGamemode)
    (:NewEnumerator3
      (Game|SpawnActorfromClass "/Game/GameplayActors/Orb/BP_Orb.BP_Orb_C" (Math|Transform|MakeTransform (Math|Vector|MakeVector 0.0 0.0 0.0) "0, 0, 0" "1.000000,1.000000,1.000000") "Undefined" "MultiplyWithRoot" 0 0))
    (:NewEnumerator2
      (Utilities|FlowControl|DoOnce false
        (:Completed
          (bind _returnvalue (Game|SpawnActorfromClass "/Game/GameplayActors/Ball/BP_Ball.BP_Ball_C" (Math|Transform|MakeTransform (Math|Vector|MakeVector 0.0 0.0 0.0) "0, 0, 0" "1.000000,1.000000,1.000000") "Undefined" "MultiplyWithRoot" 0 0))
          (Variables|Default|SetBP_Ball _returnvalue))))))

(event Custom|LevelStart_FFA
  (bind _asbp_game_instance (Utilities|Casting|CastToBP_GameInstance (Game|GetGameInstance)))
  (bind _output_get (Variables|Default|SetMatchDuration (Variables|/Game/Framework/BP_GameInstance.BP_GameInstance_C|GetActiveDuration _asbp_game_instance)))
  (Variables|Default|SetMatchLength _output_get)
  (for _array_element (Variables|Default|GetAll_ConnectedControllers)
    (Default|GameStartCountdown _array_element)
    (if (> (Variables|Default|GetMatchDuration) 0)
      (Default|HUDSetupMatchTimer _array_element (Variables|Default|GetMatchDuration))))
  (Utilities|FlowControl|Delay 3.0)
  (for _array_element_2 (Variables|Default|GetAll_ConnectedControllers)
    (Default|EnableAllInput _array_element_2)
    (Default|HUDStartMatchFFA _array_element_2))
  (if (> (Variables|Default|GetMatchDuration) 0)
    (bind _returnvalue (Utilities|Time|SetTimerbyFunctionName 0 "MatchTimerInterval" 1.0 true))
    (Variables|Default|SetMatchTimerHandle _returnvalue)))

(event Custom|MatchTimerInterval
  (bind _result (Math|Integer|DecrementInt (Variables|Default|GetMatchDuration))
    (:%20%20
      (Default|UpdateHUDMatchTimer (Variables|Default|GetAs%20BP%20Standard%20Game%20State) _result)
      (if (== (Variables|Default|GetMatchDuration) 0)
        (Utilities|Time|ClearandInvalidateTimerbyHandle (Variables|Default|GetMatchTimerHandle))
        (switch Utilities|FlowControl|Switch|SwitchonE_Gamemodes (Variables|Default|GetGamemode)
          (:NewEnumerator0
            (CallFunction|GMFFAGameOver))
          (:NewEnumerator3
            (CallFunction|GMPosGameOver)))))))

(event EventHandleStartingNewPlayer
  (params (NewPlayer :type Player%20Controller%20Object%20Reference))
  (bind _all_connectedcontrollers (Variables|Default|GetAll_ConnectedControllers))
  (bind _output (Utilities|Array|Get(acopy) _all_connectedcontrollers))
  (bind _asbp_standard_player_controller (Utilities|Casting|CastToBP_Standard_PlayerController NewPlayer))
  (Default|LoadProfile _asbp_standard_player_controller)
  (Default|OnControllerSpawned _asbp_standard_player_controller)
  (Utilities|Array|Add (Variables|Default|GetAll_ConnectedControllers) _asbp_standard_player_controller)
  (bind _asbp_game_instance (Utilities|Casting|CastToBP_GameInstance (Game|GetGameInstance)))
  (Variables|Default|SetGamemode (Variables|/Game/Framework/BP_GameInstance.BP_GameInstance_C|GetActiveGamemode _asbp_game_instance))
  (Variables|Default|SetNum_ExpectedPlayers (Variables|/Game/Framework/BP_GameInstance.BP_GameInstance_C|GetNumConnectedPlayers _asbp_game_instance))
  (CallFunction|UpdateGamestateInfo)
  (if (Variables|/Game/Framework/BP_GameInstance.BP_GameInstance_C|GetIsSoloGame _asbp_game_instance)
    (bind _allplayersready (CallFunction|CountPlayersSpawned :!label _label))
    (if _allplayersready
      (Variables|Default|SetNum_ExpectedPlayers 1)
      (Class|GameModeBase|RestartPlayeratPlayerStart _output (Class|GameModeBase|FindPlayerStart _output "0"))
      (Default|EnableAllInput (Variables|Default|GetAll_ConnectedControllers))
      (else
        (Utilities|FlowControl|DelayUntilNextTick)
        (goto _label)))
    (elif (== (Variables|Default|GetNum_ExpectedPlayers) (Utilities|Array|Length (Variables|Default|GetAll_ConnectedControllers)))
      (bind _allplayersready_2 (CallFunction|CountPlayersSpawned :!label _label_2))
      (if _allplayersready_2
        (for (_array_element _array_index) (Variables|Default|GetAll_ConnectedControllers)
          (Class|GameModeBase|RestartPlayeratPlayerStart _array_element (Class|GameModeBase|FindPlayerStart _array_element (Utilities|String|ToString(Integer) _array_index))))
        (switch Utilities|FlowControl|Switch|SwitchonE_Gamemodes (Variables|Default|GetGamemode)
          (:NewEnumerator0
            (CallFunction|LevelStartFFA))
          (:NewEnumerator3
            (CallFunction|LevelStartPossession))
          (:NewEnumerator2
            (CallFunction|LevelStartFootball)))
        (else
          (Utilities|FlowControl|DelayUntilNextTick)
          (goto _label_2))))))

(event EventBeginPlay
  (bind _asbp_standard_game_state (Utilities|Casting|CastToBP_Standard_GameState (Game|GetGameState)))
  (Variables|Default|SetAs%20BP%20Standard%20Game%20State _asbp_standard_game_state)
  (bind _asbp_game_instance (Utilities|Casting|CastToBP_GameInstance (Game|GetGameInstance)))
  (Variables|Default|SetbUseSeamlessTravel (Variables|/Game/Framework/BP_GameInstance.BP_GameInstance_C|GetSeamlessTravelCarry _asbp_game_instance)))

(event EventOnLogout
  (params (ExitingController :type Controller%20Object%20Reference))
  (bind _asbp_standard_player_controller (Utilities|Casting|CastToBP_Standard_PlayerController ExitingController))
  (Utilities|Array|RemoveItem (Variables|Default|GetAll_ConnectedControllers) _asbp_standard_player_controller)
  (Math|Integer|DecrementInt (Variables|Default|GetNum_ExpectedPlayers)))

(fn ConstructionScript)

(fn SpawnDefaultPawnfor
  (params (NewPlayer :type Controller%20Object%20Reference) (StartSpot :type Actor%20Object%20Reference))
  (if (Variables|Default|GetbUseSeamlessTravel)
    (bind _asbp_standard_playerstate (Utilities|Casting|CastToBP_Standard_Playerstate (Variables|/Script/Engine.Controller|GetPlayerState NewPlayer)))
    (LocalVariables|SetLclCharacterClass (.CharacterClass (Utilities|Struct|BreakS_PlayerProfile (Variables|/Game/Framework/BP_Standard_Playerstate.BP_Standard_Playerstate_C|GetS_PlayerProfile _asbp_standard_playerstate))))
    (else
      (bind _asbp_standard_player_controller (Utilities|Casting|CastToBP_Standard_PlayerController NewPlayer))
      (LocalVariables|SetLclCharacterClass (Utilities|Struct|BreakS_PlayerProfile (Variables|/Game/Framework/BP_Standard_PlayerController.BP_Standard_PlayerController_C|GetPlayerProfile _asbp_standard_player_controller)))))
  (bind _returnvalue (Game|SpawnActorfromClass (LocalVariables|GetLclCharacterClass) (Transformation|GetActorTransform StartSpot) "Undefined" "MultiplyWithRoot" 0 0))
  (bind _asbp_ship_base (Utilities|Casting|CastToBP_ShipBase _returnvalue))
  (return _asbp_ship_base))

(fn GMFFAKilledPlayer
  (params (Killer :type BP%20Standard%20Player%20Controller%20Object%20Reference) (Victim :type BP%20Standard%20Player%20Controller%20Object%20Reference))
  (bind _result (Math|Integer|IncrementInt (Variables|/Game/Framework/BP_Standard_PlayerController.BP_Standard_PlayerController_C|GetDeaths Victim))
    (:%20%20
      (Variables|/Game/Framework/BP_Standard_Playerstate.BP_Standard_Playerstate_C|SetDeaths (Variables|/Game/Framework/BP_Standard_PlayerController.BP_Standard_PlayerController_C|GetBP_StandardPlayerState Victim) _result)
      (bind _result_2 (Math|Integer|IncrementInt (Variables|/Game/Framework/BP_Standard_PlayerController.BP_Standard_PlayerController_C|GetKills Killer))
        (:%20%20
          (Variables|/Game/Framework/BP_Standard_Playerstate.BP_Standard_Playerstate_C|SetKills (Variables|/Game/Framework/BP_Standard_PlayerController.BP_Standard_PlayerController_C|GetBP_StandardPlayerState Killer) _result_2))))))

(fn UpdateGamestateInfo
  (bind _as_bp_standard_game_state (Variables|Default|GetAs%20BP%20Standard%20Game%20State))
  (Variables|/Game/Framework/BP_Standard_GameState.BP_Standard_GameState_C|SetCurrentGameMode _as_bp_standard_game_state (Variables|Default|GetGamemode))
  (Variables|/Game/Framework/BP_Standard_GameState.BP_Standard_GameState_C|SetMatchDuration _as_bp_standard_game_state (Variables|Default|GetMatchLength)))

(fn CountPlayersSpawned
  (for _array_element (Variables|Default|GetAll_ConnectedControllers)
    (if (Variables|/Game/Framework/BP_Standard_PlayerController.BP_Standard_PlayerController_C|GetIsPlayerReady _array_element)
      (Math|Integer|IncrementInt (LocalVariables|GetLcl_PlayersReady))))
  (return (== (Utilities|Array|Length (Variables|Default|GetAll_ConnectedControllers)) (LocalVariables|GetLcl_PlayersReady))))