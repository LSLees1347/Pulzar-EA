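; Player controller for multiplayer ship matches, owning the local UI (HUD, cursor, scoreboard, death and game-over screens) and the death-to-respawn cycle.
; It sends the saved profile to the server and polls until profile, GameState and PlayerState are ready.
; On death it possesses a spectator, views the killer, then respawns the profile's ship class at a random position after a delay.
; HUD-dependent calls retry each tick until the widget exists.
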(event Custom|EnableAllInput
  (Input|EnableInput (Pawn|GetControlledPawn) self))

(event Custom|GameStartCountdown
  (bind _wbp_hud (Variables|Default|GetWBP_HUD))
  (Utilities|IsValid _wbp_hud :!label _label
    (:Is%20Valid
      (Default|GameStartCountdown _wbp_hud))
    (:Is%20Not%20Valid
      (Utilities|FlowControl|DelayUntilNextTick)
      (goto _label))))

(event Custom|ExitSpectating
  (Networking|SwitchHasAuthority
    (:Authority
      (CallFunction|ReSpawnPlayer)
      (CallFunction|ClientRespawnHUD))
    (:Remote
      (CallFunction|SvrExitSpectator))))

(event Custom|Svr_ExitSpectator
  (CallFunction|ReSpawnPlayer)
  (Widget|SetVisibility (Variables|Default|GetWBP_HUD) "Hidden")
  (CallFunction|ClientRespawnHUD))

(event Custom|AddPlayerXP
  (params (MatchDuration :type Integer))
  (bind _asbp_game_instance (Utilities|Casting|CastToBP_GameInstance (Game|GetGameInstance)))
  (Default|AddPlayerXP _asbp_game_instance (+ MatchDuration (* (Variables|Default|GetKills) 10))))

(event Custom|ShowGameOverScreen
  (Viewport|RemoveAllWidgets)
  (bind _returnvalue (UserInterface|CreateWidget "/Game/Widgets/GameOver/WBP_GameOver.WBP_GameOver_C" self))
  (UserInterface|Viewport|AddtoViewport _returnvalue 0)
  (Input|SetInputModeUIOnly self _returnvalue "DoNotLock" true))

(event Custom|Client_DeathScreen
  (Viewport|RemoveAllWidgets)
  (bind _returnvalue (UserInterface|CreateWidget "/Game/Widgets/Player/WBP_DeathScreen.WBP_DeathScreen_C" self))
  (UserInterface|Viewport|AddtoViewport _returnvalue 0))

(event Custom|LoadProfile
  (bind _asbp_game_instance (Utilities|Casting|CastToBP_GameInstance (Game|GetGameInstance)))
  (bind _output_get (Variables|Default|SetPlayer%20Profile%20Slot (Variables|/Game/Framework/BP_GameInstance.BP_GameInstance_C|GetPlayerProfileSlot _asbp_game_instance)))
  (bind _returnvalue (SaveGame|LoadGamefromSlot _output_get))
  (bind _assg_player_profile (Utilities|Casting|CastToSG_PlayerProfile _returnvalue))
  (Variables|Default|SetAs%20SG%20Player%20Profile _assg_player_profile)
  (Networking|SwitchHasAuthority
    (:Authority
      (Variables|Default|SetPlayerProfile (Variables|/Game/SaveData/SG_PlayerProfile.SG_PlayerProfile_C|GetPlayerProfile _assg_player_profile))
      (Variables|Default|SetIsProfileLoaded true))
    (:Remote
      (CallFunction|SvrSetPlayerProfile (Variables|/Game/SaveData/SG_PlayerProfile.SG_PlayerProfile_C|GetPlayerProfile _assg_player_profile)))))

(event Custom|Client_RespawnHUD
  (Viewport|RemoveAllWidgets)
  (CallFunction|UIShowHUD))

(event Custom|UnHide_HUD
  (Widget|SetVisibility (Variables|Default|GetWBP_HUD) "Visible"))

(event Custom|EndClientSession
  (bind _asbp_game_instance (Utilities|Casting|CastToBP_GameInstance (Game|GetGameInstance)))
  (Variables|/Game/Framework/BP_GameInstance.BP_GameInstance_C|SetMP_IsPauseMenuVisible _asbp_game_instance false)
  (|DestroySession self
    (:then
      (Game|OpenLevel(byName) "MainMenu"))))

(event Custom|Svr_SetPlayerProfile
  (params (S_PlayerProfile :type S%20Player%20Profile%20Structure))
  (Variables|Default|SetPlayerProfile S_PlayerProfile)
  (Variables|Default|SetIsProfileLoaded true))

(event Custom|OnControllerSpawned
  (if (Variables|Default|GetIsGameStateReady) :!label _label
    _
    (else
      (bind _asbp_standard_game_state (Utilities|Casting|CastToBP_Standard_GameState (Game|GetGameState))
        (:then
          (Variables|Default|SetBP_StandardGameState _asbp_standard_game_state)
          (Variables|Default|SetIsGameStateReady true))
        (:CastFailed
          _))))
  (if (Variables|Default|GetIsPlayerStateReady)
    _
    (else
      (bind _asbp_standard_playerstate (Utilities|Casting|CastToBP_Standard_Playerstate (Variables|GetPlayerState))
        (:then
          (Variables|Default|SetBP_StandardPlayerState _asbp_standard_playerstate)
          (Variables|Default|SetIsPlayerStateReady true))
        (:CastFailed
          _))))
  (if (Math|Boolean|ANDBoolean (Variables|Default|GetIsProfileLoaded) (Variables|Default|GetIsGameStateReady) (Variables|Default|GetIsPlayerStateReady))
    (Variables|Default|SetIsPlayerReady true)
    (else
      (Utilities|FlowControl|Delay 0.1)
      (goto _label))))

(event Custom|HUD_StartMatch_FFA
  (Default|GMFFAStartMatch (Variables|Default|GetWBP_HUD)))

(event Custom|HUD_SetupMatchTimer
  (params (TimeLeftSec :type Integer))
  (bind _wbp_hud (Variables|Default|GetWBP_HUD))
  (Utilities|IsValid _wbp_hud :!label _label
    (:Is%20Valid
      (Widget|SetVisibility (Variables|/Game/Widgets/Player/WBP_HUD.WBP_HUD_C|GetText_MatchDuration _wbp_hud) "Visible")
      (Default|UpdateMatchTimer (Variables|Default|GetWBP_HUD) TimeLeftSec))
    (:Is%20Not%20Valid
      (Utilities|FlowControl|DelayUntilNextTick)
      (goto _label))))

(event Custom|PlayerDeath
  (params (Player :type Actor%20Object%20Reference) (Killer :type Actor%20Object%20Reference))
  (Input|DisableInput self)
  (bind _returnvalue (Game|SpawnActorfromClass "/Game/Player/BP_Spectator.BP_Spectator_C" (Math|Transform|MakeTransform "0, 0, 0" "0, 0, 0" "1.000000,1.000000,1.000000") "Undefined" "MultiplyWithRoot" 0 0))
  (Pawn|Possess self _returnvalue)
  (Actor|DestroyActor Player)
  (Game|Player|SetViewTargetwithBlend self Killer 0.0 "VTBlend_Cubic" 0.0 false)
  (CallFunction|ClientDeathScreen)
  (Utilities|FlowControl|Delay 5.0)
  (CallFunction|ExitSpectating))

(event Custom|Local%20Set%20HUDVar
  (bind _wbp_hud (Variables|Default|GetWBP_HUD))
  (Utilities|IsValid (Variables|Default|GetWBP_HUD) :!label _label
    (:Is%20Valid
      (bind _asbp_ship_base (Utilities|Casting|CastToBP_ShipBase (Pawn|GetControlledPawn)))
      (Variables|/Game/Player/BP_ShipBase.BP_ShipBase_C|SetWPB%20HUD _asbp_ship_base _wbp_hud)
      (Default|UpdateHealth _wbp_hud (Math|Conversions|ToFloat(Integer) (Variables|/Game/Player/BP_ShipBase.BP_ShipBase_C|GetHealth _asbp_ship_base)) false))
    (:Is%20Not%20Valid
      (Utilities|FlowControl|DelayUntilNextTick)
      (goto _label))))

(event EventBeginPlay
  (if (Pawn|IsLocalPlayerController)
    (Input|SetInputModeGameandUI self 0 "LockOnCapture" false false)
    (Variables|Default|SetbShowMouseCursor true)
    (CallFunction|UIShowHUD)
    (bind _returnvalue (UserInterface|CreateWidget "/Game/Widgets/WBP_Cursor.WBP_Cursor_C"))
    (Class|PlayerController|SetMouseCursorWidget "Default" _returnvalue)))

(event EventPossess
  (params (PossessedPawn :type Pawn%20Object%20Reference))
  (CallFunction|LocalSetHUDVar)
  (bind _asbp_ship_base (Utilities|Casting|CastToBP_ShipBase PossessedPawn))
  (bind _asbp_game_instance (Utilities|Casting|CastToBP_GameInstance (Game|GetGameInstance)))
  (switch Utilities|FlowControl|Switch|SwitchonE_PlayerColours (Variables|/Game/Framework/BP_GameInstance.BP_GameInstance_C|GetPlayerColour _asbp_game_instance)
    (:NewEnumerator0
      (Rendering|Material|SetMaterial (Variables|/Game/Player/BP_ShipBase.BP_ShipBase_C|GetPlayer_Icon _asbp_ship_base) 0 "/Game/Player/M_Colours/M_Red.M_Red"))
    (:NewEnumerator1
      (Rendering|Material|SetMaterial (Variables|/Game/Player/BP_ShipBase.BP_ShipBase_C|GetPlayer_Icon _asbp_ship_base) 0 "/Game/Player/M_Colours/M_Green.M_Green"))
    (:NewEnumerator2
      (Rendering|Material|SetMaterial (Variables|/Game/Player/BP_ShipBase.BP_ShipBase_C|GetPlayer_Icon _asbp_ship_base) 0 "/Game/Player/M_Colours/M_Blue.M_Blue"))
    (:NewEnumerator3
      (Rendering|Material|SetMaterial (Variables|/Game/Player/BP_ShipBase.BP_ShipBase_C|GetPlayer_Icon _asbp_ship_base) 0 "/Game/Player/M_Colours/M_Yellow.M_Yellow"))
    (:NewEnumerator4
      (Rendering|Material|SetMaterial (Variables|/Game/Player/BP_ShipBase.BP_ShipBase_C|GetPlayer_Icon _asbp_ship_base) 0 "/Game/Player/M_Colours/M_Purple.M_Purple"))))

(fn ConstructionScript)

(fn UIShowHUD
  (Utilities|IsValid (Variables|Default|GetWBP_HUD)
    (:Is%20Valid
      _)
    (:Is%20Not%20Valid
      (bind _returnvalue (UserInterface|CreateWidget "/Game/Widgets/Player/WBP_HUD.WBP_HUD_C" self))
      (Variables|Default|SetWBP_HUD _returnvalue)))
  (UserInterface|Viewport|AddtoViewport (Variables|Default|GetWBP_HUD) 0))

(fn SpawnSpectator
  (params (Player :type Actor%20Object%20Reference))
  (bind _returnvalue (Transformation|GetActorLocation Player))
  (bind _returnvalue_2 (Game|SpawnActorfromClass "/Game/Player/BP_Spectator.BP_Spectator_C" (Math|Transform|MakeTransform (Math|Vector|MakeVector (.x _returnvalue) (.y _returnvalue) 0.0) "0, 0, 0" "1.000000,1.000000,1.000000") "Undefined" "MultiplyWithRoot" 0 0))
  (Pawn|Possess _returnvalue_2)
  (Actor|DestroyActor Player)
  (CallFunction|EnableAllInput)
  (return))

(fn ReSpawnPlayer
  (bind _returnvalue (Game|SpawnActorfromClass (Utilities|Struct|BreakS_PlayerProfile (Variables|Default|GetPlayerProfile)) (Math|Transform|MakeTransform (Math|Vector|MakeVector (Math|Random|RandomFloatinRange -5e+02 5e+02) (Math|Random|RandomFloatinRange -5e+02 5e+02) 0.0) "0, 0, 0" "1.000000,1.000000,1.000000") "Undefined" "MultiplyWithRoot" 0 0))
  (bind _asbp_ship_base (Utilities|Casting|CastToBP_ShipBase _returnvalue))
  (Pawn|Possess _asbp_ship_base)
  (CallFunction|EnableAllInput)
  (return))

(fn UIToggleScoreboard
  (params (NewVisibility :type Boolean))
  (if NewVisibility
    (Utilities|IsValid (Variables|Default|GetWBP_Scoreboard)
      (:Is%20Valid
        _)
      (:Is%20Not%20Valid
        (bind _returnvalue (UserInterface|CreateWidget "/Game/Widgets/Scoreboard/WBP_Scoreboard.WBP_Scoreboard_C" self))
        (Variables|Default|SetWBP_Scoreboard _returnvalue)))
    (UserInterface|Viewport|AddtoViewport (Variables|Default|GetWBP_Scoreboard) 0)
    (else
      (Utilities|IsValid (Variables|Default|GetWBP_Scoreboard)
        (:Is%20Valid
          (Widget|RemovefromParent (Variables|Default|GetWBP_Scoreboard)))
        (:Is%20Not%20Valid
          _))))
  (return))