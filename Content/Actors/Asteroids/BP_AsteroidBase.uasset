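; Base asteroid actor that drifts and spins in a random horizontal direction until it is destroyed by hits.
; BeginPlay rolls a random planar direction and yaw speed, which Tick applies as per-frame world offset and relative rotation, without delta-time scaling.
; Each Hit event increments a counter; on reaching HitPoints it asks GM_Player to spawn another asteroid, then disables tick and destroys itself.
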(event Custom|Hit
  (Variables|Default|SetHitCounter (+ (Variables|Default|GetHitCounter) 1))
  (if (>= (Variables|Default|GetHitCounter) (Variables|Default|GetHitPoints))
    (bind _asgm_player (Utilities|Casting|CastToGM_Player (Game|GetGameMode)))
    (Default|SpawnAsteroid _asgm_player)
    (Actor|Tick|SetActorTickEnabled false)
    (Actor|DestroyActor)))

(event EventTick
  (params (DeltaSeconds :type Float%20%28single-precision%29))
  (bind _randomdirection (Variables|Default|GetRandomDirection))
  (Transformation|AddWorldOffset (Variables|Default|GetScene) (Math|Vector|MakeVector (.x _randomdirection) (.y _randomdirection) 0.0) false false)
  (Transformation|AddRelativeRotation (Variables|Default|GetScene) (Math|Rotator|MakeRotator 0.0 0.0 (Variables|Default|GetRandomRotation)) false false))

(event EventBeginPlay
  (Variables|Default|SetRandomDirection (Math|Vector|MakeVector (Math|Random|RandomFloatinRange -4.0 4.0) (Math|Random|RandomFloatinRange -4.0 4.0) 0.0))
  (Variables|Default|SetRandomRotation (Math|Random|RandomFloatinRange -0.7 0.7)))

(fn ConstructionScript)