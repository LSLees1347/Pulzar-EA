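; BP_Orb is a capturable orb that a ship takes possession of by touching it.
; On overlap with a BP_ShipBase, it homes its ProjectileMovement on the ship's Sprite, calls the ship's GainPossession and blocks further capture.
; ReleaseOrb clears the homing target and re-enables capture after a short delay.
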(event Custom|ReleaseOrb
  (Variables|/Script/Engine.ProjectileMovementComponent|SetHomingTargetComponent (Variables|Default|GetProjectileMovement) 0)
  (Utilities|FlowControl|Delay 1.0)
  (Variables|Default|SetCanBeCaptured true))

(event Collision|EventActorBeginOverlap
  (params (OtherActor :type Actor%20Object%20Reference))
  (if (Variables|Default|GetCanBeCaptured)
    (bind _asbp_ship_base (Utilities|Casting|CastToBP_ShipBase OtherActor))
    (Variables|/Script/Engine.ProjectileMovementComponent|SetHomingTargetComponent (Variables|Default|GetProjectileMovement) (Variables|/Script/Paper2D.PaperCharacter|GetSprite _asbp_ship_base))
    (Default|GainPossession _asbp_ship_base self)
    (Variables|Default|SetCanBeCaptured false)))

(fn ConstructionScript)