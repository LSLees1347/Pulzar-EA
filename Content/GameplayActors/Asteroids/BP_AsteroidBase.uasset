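; BP_AsteroidBase is a base actor for destructible asteroids with a Paper2D flipbook visual.
; Shortly after BeginPlay it resets its location, keeping only X and Y.
; Incoming damage lowers clamped health, triggering MC-prefixed events that spawn an impact effect at the flipbook's location, or a death effect before the actor is destroyed at zero health.
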(event Custom|MC_Impact
  (params (Location :type Vector))
  (Niagara|SpawnSystematLocation (Variables|Default|GetImpactEffect) Location "0, 0, 0" "0.150000,0.150000,0.150000"))

(event Custom|MC_Death
  (params (Location :type Vector))
  (Niagara|SpawnSystematLocation (Variables|Default|GetDeathEffect) Location))

(event EventBeginPlay
  (bind _returnvalue (Transformation|GetActorLocation))
  (Utilities|FlowControl|Delay 0.1)
  (Transformation|SetActorLocation (Math|Vector|MakeVector (.x _returnvalue) (.y _returnvalue) 0.0) false false))

(event Game|Damage|EventAnyDamage
  (params (Damage :type Float%20%28single-precision%29) (DamageType :type Damage%20Type%20Object%20Reference) (InstigatedBy :type Controller%20Object%20Reference) (DamageCauser :type Actor%20Object%20Reference))
  (bind _paperflipbook (Variables|Default|GetPaperFlipbook))
  (bind _returnvalue (Transformation|GetWorldLocation _paperflipbook))
  (Variables|Default|SetHealth (Math|Float|Clamp(Float) (- (Variables|Default|GetHealth) Damage) 0.0 (Variables|Default|GetMaxHealth)))
  (if (<= (Variables|Default|GetHealth) 0.0)
    (CallFunction|MCDeath _returnvalue)
    (Actor|DestroyActor)
    (else
      (CallFunction|MCImpact _returnvalue))))

(fn ConstructionScript)