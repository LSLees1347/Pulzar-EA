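; BP_oobTrigger is an out-of-bounds volume that recycles asteroids leaving the play area.
; When a BP_AsteroidBase ends overlap with the Destroy component, it resets that asteroid's Scene component relative transform rather than destroying it.
; Two disconnected experiments remain: destroy and respawn at a random position, and respawn via GM_Gameplay, noted as adding two asteroids instead of one.
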(event OnComponentEndOverlap(Destroy)
  (params (OverlappedComponent :type Primitive%20Component%20Object%20Reference) (OtherActor :type Actor%20Object%20Reference) (OtherComp :type Primitive%20Component%20Object%20Reference) (OtherBodyIndex :type Integer))
  (bind _asbp_asteroid_base (Utilities|Casting|CastToBP_AsteroidBase OtherActor))
  (Transformation|ResetRelativeTransform (Variables|/Game/LevelObjects/BP_AsteroidBase.BP_AsteroidBase_C|GetScene _asbp_asteroid_base)))

(fn ConstructionScript)