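; BP_GameplayBoundaries is a play-area boundary actor that bounces the player's BP_StarterShip off walls.
; Overlapping a wall flips the ship's X or Y momentum and scales it.
; Outer walls use WallBouncynessMultiplier, or double the momentum when it is low on both axes, while inner walls always double it.
; Leaving FarBounds triggers a fail-safe that zeroes momentum and resets the ship's location, with debug prints throughout.
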(event OnComponentEndOverlap(FarBounds)
  (params (OverlappedComponent :type Primitive%20Component%20Object%20Reference) (OtherActor :type Actor%20Object%20Reference) (OtherComp :type Primitive%20Component%20Object%20Reference) (OtherBodyIndex :type Integer))
  (bind _as_bp_starter_ship (Variables|Default|GetAs%20BP%20Starter%20Ship))
  (Variables|/Game/Player/BP_PlayerShipBase.BP_PlayerShipBase_C|SetCurrentMomentum _as_bp_starter_ship "0, 0, 0")
  (Transformation|SetWorldLocation (Variables|/Game/Player/BP_PlayerShipBase.BP_PlayerShipBase_C|GetPhysicsRoot _as_bp_starter_ship) (Math|Vector|MakeVector 0.0 0.0 0.0) false false)
  (Development|PrintString "fail safe"))

(event OnComponentBeginOverlap(InnerBoundsL1)
  (params (OverlappedComponent :type Primitive%20Component%20Object%20Reference) (OtherActor :type Actor%20Object%20Reference) (OtherComp :type Primitive%20Component%20Object%20Reference) (OtherBodyIndex :type Integer) (bFromSweep :type Boolean) (SweepResult :type Hit%20Result%20Structure%20%28by%20ref%29))
  (bind _as_bp_starter_ship (Variables|Default|GetAs%20BP%20Starter%20Ship))
  (Variables|/Game/Player/BP_PlayerShipBase.BP_PlayerShipBase_C|SetCurrentMomentum _as_bp_starter_ship (Math|Vector|MakeVector (* (* (.x (Variables|/Game/Player/BP_PlayerShipBase.BP_PlayerShipBase_C|GetCurrentMomentum _as_bp_starter_ship)) 1.0) 2.0) (* (* (.y (Variables|/Game/Player/BP_PlayerShipBase.BP_PlayerShipBase_C|GetCurrentMomentum _as_bp_starter_ship)) -1.0) 2.0) 0.0))
  (Development|PrintString "inner wall hit"))

(event OnComponentBeginOverlap(InnerBoundsR)
  (params (OverlappedComponent :type Primitive%20Component%20Object%20Reference) (OtherActor :type Actor%20Object%20Reference) (OtherComp :type Primitive%20Component%20Object%20Reference) (OtherBodyIndex :type Integer) (bFromSweep :type Boolean) (SweepResult :type Hit%20Result%20Structure%20%28by%20ref%29))
  (bind _as_bp_starter_ship (Variables|Default|GetAs%20BP%20Starter%20Ship))
  (Variables|/Game/Player/BP_PlayerShipBase.BP_PlayerShipBase_C|SetCurrentMomentum _as_bp_starter_ship (Math|Vector|MakeVector (* (* (.x (Variables|/Game/Player/BP_PlayerShipBase.BP_PlayerShipBase_C|GetCurrentMomentum _as_bp_starter_ship)) 1.0) (Math|Float|SelectFloat 2.0 (Variables|Default|GetWallBouncynessMultiplier) (Math|Boolean|ANDBoolean (< (.x (Variables|/Game/Player/BP_PlayerShipBase.BP_PlayerShipBase_C|GetCurrentMomentum _as_bp_starter_ship)) 2e+01) (> (.x (Variables|/Game/Player/BP_PlayerShipBase.BP_PlayerShipBase_C|GetCurrentMomentum _as_bp_starter_ship)) -2e+01) (< (.y (Variables|/Game/Player/BP_PlayerShipBase.BP_PlayerShipBase_C|GetCurrentMomentum _as_bp_starter_ship)) 2e+01) (> (.y (Variables|/Game/Player/BP_PlayerShipBase.BP_PlayerShipBase_C|GetCurrentMomentum _as_bp_starter_ship)) -2e+01)))) (* (* (.y (Variables|/Game/Player/BP_PlayerShipBase.BP_PlayerShipBase_C|GetCurrentMomentum _as_bp_starter_ship)) -1.0) (Math|Float|SelectFloat 2.0 (Variables|Default|GetWallBouncynessMultiplier) (Math|Boolean|ANDBoolean (< (.x (Variables|/Game/Player/BP_PlayerShipBase.BP_PlayerShipBase_C|GetCurrentMomentum _as_bp_starter_ship)) 2e+01) (> (.x (Variables|/Game/Player/BP_PlayerShipBase.BP_PlayerShipBase_C|GetCurrentMomentum _as_bp_starter_ship)) -2e+01) (< (.y (Variables|/Game/Player/BP_PlayerShipBase.BP_PlayerShipBase_C|GetCurrentMomentum _as_bp_starter_ship)) 2e+01) (> (.y (Variables|/Game/Player/BP_PlayerShipBase.BP_PlayerShipBase_C|GetCurrentMomentum _as_bp_starter_ship)) -2e+01)))) 0.0))
  (Development|PrintString "outer wall hit"))

(event OnComponentBeginOverlap(InnerBoundsL)
  (params (OverlappedComponent :type Primitive%20Component%20Object%20Reference) (OtherActor :type Actor%20Object%20Reference) (OtherComp :type Primitive%20Component%20Object%20Reference) (OtherBodyIndex :type Integer) (bFromSweep :type Boolean) (SweepResult :type Hit%20Result%20Structure%20%28by%20ref%29))
  (bind _as_bp_starter_ship (Variables|Default|GetAs%20BP%20Starter%20Ship))
  (Variables|/Game/Player/BP_PlayerShipBase.BP_PlayerShipBase_C|SetCurrentMomentum _as_bp_starter_ship (Math|Vector|MakeVector (* (* (.x (Variables|/Game/Player/BP_PlayerShipBase.BP_PlayerShipBase_C|GetCurrentMomentum _as_bp_starter_ship)) 1.0) (Math|Float|SelectFloat 2.0 (Variables|Default|GetWallBouncynessMultiplier) (Math|Boolean|ANDBoolean (< (.x (Variables|/Game/Player/BP_PlayerShipBase.BP_PlayerShipBase_C|GetCurrentMomentum _as_bp_starter_ship)) 2e+01) (> (.x (Variables|/Game/Player/BP_PlayerShipBase.BP_PlayerShipBase_C|GetCurrentMomentum _as_bp_starter_ship)) -2e+01) (< (.y (Variables|/Game/Player/BP_PlayerShipBase.BP_PlayerShipBase_C|GetCurrentMomentum _as_bp_starter_ship)) 2e+01) (> (.y (Variables|/Game/Player/BP_PlayerShipBase.BP_PlayerShipBase_C|GetCurrentMomentum _as_bp_starter_ship)) -2e+01)))) (* (* (.y (Variables|/Game/Player/BP_PlayerShipBase.BP_PlayerShipBase_C|GetCurrentMomentum _as_bp_starter_ship)) -1.0) (Math|Float|SelectFloat 2.0 (Variables|Default|GetWallBouncynessMultiplier) (Math|Boolean|ANDBoolean (< (.x (Variables|/Game/Player/BP_PlayerShipBase.BP_PlayerShipBase_C|GetCurrentMomentum _as_bp_starter_ship)) 2e+01) (> (.x (Variables|/Game/Player/BP_PlayerShipBase.BP_PlayerShipBase_C|GetCurrentMomentum _as_bp_starter_ship)) -2e+01) (< (.y (Variables|/Game/Player/BP_PlayerShipBase.BP_PlayerShipBase_C|GetCurrentMomentum _as_bp_starter_ship)) 2e+01) (> (.y (Variables|/Game/Player/BP_PlayerShipBase.BP_PlayerShipBase_C|GetCurrentMomentum _as_bp_starter_ship)) -2e+01)))) 0.0))
  (Development|PrintString "outer wall hit"))

(event OnComponentBeginOverlap(InnerBoundsT)
  (params (OverlappedComponent :type Primitive%20Component%20Object%20Reference) (OtherActor :type Actor%20Object%20Reference) (OtherComp :type Primitive%20Component%20Object%20Reference) (OtherBodyIndex :type Integer) (bFromSweep :type Boolean) (SweepResult :type Hit%20Result%20Structure%20%28by%20ref%29))
  (bind _as_bp_starter_ship (Variables|Default|GetAs%20BP%20Starter%20Ship))
  (Variables|/Game/Player/BP_PlayerShipBase.BP_PlayerShipBase_C|SetCurrentMomentum _as_bp_starter_ship (Math|Vector|MakeVector (* (* (.x (Variables|/Game/Player/BP_PlayerShipBase.BP_PlayerShipBase_C|GetCurrentMomentum _as_bp_starter_ship)) -1.0) (Math|Float|SelectFloat 2.0 (Variables|Default|GetWallBouncynessMultiplier) (Math|Boolean|ANDBoolean (< (.x (Variables|/Game/Player/BP_PlayerShipBase.BP_PlayerShipBase_C|GetCurrentMomentum _as_bp_starter_ship)) 2e+01) (> (.x (Variables|/Game/Player/BP_PlayerShipBase.BP_PlayerShipBase_C|GetCurrentMomentum _as_bp_starter_ship)) -2e+01) (< (.y (Variables|/Game/Player/BP_PlayerShipBase.BP_PlayerShipBase_C|GetCurrentMomentum _as_bp_starter_ship)) 2e+01) (> (.y (Variables|/Game/Player/BP_PlayerShipBase.BP_PlayerShipBase_C|GetCurrentMomentum _as_bp_starter_ship)) -2e+01)))) (* (* (.y (Variables|/Game/Player/BP_PlayerShipBase.BP_PlayerShipBase_C|GetCurrentMomentum _as_bp_starter_ship)) 1.0) (Math|Float|SelectFloat 2.0 (Variables|Default|GetWallBouncynessMultiplier) (Math|Boolean|ANDBoolean (< (.x (Variables|/Game/Player/BP_PlayerShipBase.BP_PlayerShipBase_C|GetCurrentMomentum _as_bp_starter_ship)) 2e+01) (> (.x (Variables|/Game/Player/BP_PlayerShipBase.BP_PlayerShipBase_C|GetCurrentMomentum _as_bp_starter_ship)) -2e+01) (< (.y (Variables|/Game/Player/BP_PlayerShipBase.BP_PlayerShipBase_C|GetCurrentMomentum _as_bp_starter_ship)) 2e+01) (> (.y (Variables|/Game/Player/BP_PlayerShipBase.BP_PlayerShipBase_C|GetCurrentMomentum _as_bp_starter_ship)) -2e+01)))) 0.0))
  (Development|PrintString "outer wall hit"))

(event OnComponentBeginOverlap(InnerBoundsB)
  (params (OverlappedComponent :type Primitive%20Component%20Object%20Reference) (OtherActor :type Actor%20Object%20Reference) (OtherComp :type Primitive%20Component%20Object%20Reference) (OtherBodyIndex :type Integer) (bFromSweep :type Boolean) (SweepResult :type Hit%20Result%20Structure%20%28by%20ref%29))
  (bind _as_bp_starter_ship (Variables|Default|GetAs%20BP%20Starter%20Ship))
  (Variables|/Game/Player/BP_PlayerShipBase.BP_PlayerShipBase_C|SetCurrentMomentum _as_bp_starter_ship (Math|Vector|MakeVector (* (* (.x (Variables|/Game/Player/BP_PlayerShipBase.BP_PlayerShipBase_C|GetCurrentMomentum _as_bp_starter_ship)) -1.0) (Math|Float|SelectFloat 2.0 (Variables|Default|GetWallBouncynessMultiplier) (Math|Boolean|ANDBoolean (< (.x (Variables|/Game/Player/BP_PlayerShipBase.BP_PlayerShipBase_C|GetCurrentMomentum _as_bp_starter_ship)) 2e+01) (> (.x (Variables|/Game/Player/BP_PlayerShipBase.BP_PlayerShipBase_C|GetCurrentMomentum _as_bp_starter_ship)) -2e+01) (< (.y (Variables|/Game/Player/BP_PlayerShipBase.BP_PlayerShipBase_C|GetCurrentMomentum _as_bp_starter_ship)) 2e+01) (> (.y (Variables|/Game/Player/BP_PlayerShipBase.BP_PlayerShipBase_C|GetCurrentMomentum _as_bp_starter_ship)) -2e+01)))) (* (* (.y (Variables|/Game/Player/BP_PlayerShipBase.BP_PlayerShipBase_C|GetCurrentMomentum _as_bp_starter_ship)) 1.0) (Math|Float|SelectFloat 2.0 (Variables|Default|GetWallBouncynessMultiplier) (Math|Boolean|ANDBoolean (< (.x (Variables|/Game/Player/BP_PlayerShipBase.BP_PlayerShipBase_C|GetCurrentMomentum _as_bp_starter_ship)) 2e+01) (> (.x (Variables|/Game/Player/BP_PlayerShipBase.BP_PlayerShipBase_C|GetCurrentMomentum _as_bp_starter_ship)) -2e+01) (< (.y (Variables|/Game/Player/BP_PlayerShipBase.BP_PlayerShipBase_C|GetCurrentMomentum _as_bp_starter_ship)) 2e+01) (> (.y (Variables|/Game/Player/BP_PlayerShipBase.BP_PlayerShipBase_C|GetCurrentMomentum _as_bp_starter_ship)) -2e+01)))) 0.0))
  (Development|PrintString "outer wall hit"))

(event OnComponentBeginOverlap(InnerBoundsR1)
  (params (OverlappedComponent :type Primitive%20Component%20Object%20Reference) (OtherActor :type Actor%20Object%20Reference) (OtherComp :type Primitive%20Component%20Object%20Reference) (OtherBodyIndex :type Integer) (bFromSweep :type Boolean) (SweepResult :type Hit%20Result%20Structure%20%28by%20ref%29))
  (bind _as_bp_starter_ship (Variables|Default|GetAs%20BP%20Starter%20Ship))
  (Variables|/Game/Player/BP_PlayerShipBase.BP_PlayerShipBase_C|SetCurrentMomentum _as_bp_starter_ship (Math|Vector|MakeVector (* (* (.x (Variables|/Game/Player/BP_PlayerShipBase.BP_PlayerShipBase_C|GetCurrentMomentum _as_bp_starter_ship)) 1.0) 2.0) (* (* (.y (Variables|/Game/Player/BP_PlayerShipBase.BP_PlayerShipBase_C|GetCurrentMomentum _as_bp_starter_ship)) -1.0) 2.0) 0.0))
  (Development|PrintString "inner wall hit"))

(event OnComponentBeginOverlap(InnerBoundsT1)
  (params (OverlappedComponent :type Primitive%20Component%20Object%20Reference) (OtherActor :type Actor%20Object%20Reference) (OtherComp :type Primitive%20Component%20Object%20Reference) (OtherBodyIndex :type Integer) (bFromSweep :type Boolean) (SweepResult :type Hit%20Result%20Structure%20%28by%20ref%29))
  (bind _as_bp_starter_ship (Variables|Default|GetAs%20BP%20Starter%20Ship))
  (Variables|/Game/Player/BP_PlayerShipBase.BP_PlayerShipBase_C|SetCurrentMomentum _as_bp_starter_ship (Math|Vector|MakeVector (* (* (.x (Variables|/Game/Player/BP_PlayerShipBase.BP_PlayerShipBase_C|GetCurrentMomentum _as_bp_starter_ship)) -1.0) 2.0) (* (* (.y (Variables|/Game/Player/BP_PlayerShipBase.BP_PlayerShipBase_C|GetCurrentMomentum _as_bp_starter_ship)) 1.0) 2.0) 0.0))
  (Development|PrintString "inner wall hit"))

(event OnComponentBeginOverlap(InnerBoundsB1)
  (params (OverlappedComponent :type Primitive%20Component%20Object%20Reference) (OtherActor :type Actor%20Object%20Reference) (OtherComp :type Primitive%20Component%20Object%20Reference) (OtherBodyIndex :type Integer) (bFromSweep :type Boolean) (SweepResult :type Hit%20Result%20Structure%20%28by%20ref%29))
  (bind _as_bp_starter_ship (Variables|Default|GetAs%20BP%20Starter%20Ship))
  (Variables|/Game/Player/BP_PlayerShipBase.BP_PlayerShipBase_C|SetCurrentMomentum _as_bp_starter_ship (Math|Vector|MakeVector (* (* (.x (Variables|/Game/Player/BP_PlayerShipBase.BP_PlayerShipBase_C|GetCurrentMomentum _as_bp_starter_ship)) -1.0) 2.0) (* (* (.y (Variables|/Game/Player/BP_PlayerShipBase.BP_PlayerShipBase_C|GetCurrentMomentum _as_bp_starter_ship)) 1.0) 2.0) 0.0))
  (Development|PrintString "inner wall hit"))

(event EventBeginPlay
  (bind _asbp_starter_ship (Utilities|Casting|CastToBP_StarterShip (Game|Player|GetPlayerPawn 0)))
  (Variables|Default|SetAs%20BP%20Starter%20Ship _asbp_starter_ship))

(fn ConstructionScript)