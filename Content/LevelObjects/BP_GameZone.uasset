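; BP_GameZone is a level object that defines the playable bounds through overlap events on its Destroy component.
; A player ship entering the zone is told it is in bounds, and its exit is reported through a DoOnce that re-entry resets.
; Asteroids that leave the zone are destroyed.
; Unconnected leftover nodes hold abandoned attempts at respawning asteroids, and the HitCollision function is empty.
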(event OnComponentBeginOverlap(Destroy)
  (params (OverlappedComponent :type Primitive%20Component%20Object%20Reference) (OtherActor :type Actor%20Object%20Reference) (OtherComp :type Primitive%20Component%20Object%20Reference) (OtherBodyIndex :type Integer) (bFromSweep :type Boolean) (SweepResult :type Hit%20Result%20Structure%20%28by%20ref%29))
  (bind _asbp_player_ship (Utilities|Casting|CastToBP_PlayerShip OtherActor))
  (Default|EnterGameBounds _asbp_player_ship)
  (Utilities|FlowControl|DoOnce false) ; enters at Reset
)

(event OnComponentEndOverlap(Destroy)
  (params (OverlappedComponent :type Primitive%20Component%20Object%20Reference) (OtherActor :type Actor%20Object%20Reference) (OtherComp :type Primitive%20Component%20Object%20Reference) (OtherBodyIndex :type Integer))
  (bind _asbp_player_ship (Utilities|Casting|CastToBP_PlayerShip OtherActor)
    (:then
      (Utilities|FlowControl|DoOnce false
        (:Completed
          (Default|ExitGameBounds _asbp_player_ship))))
    (:CastFailed
      (bind _asbp_asteroid_base (Utilities|Casting|CastToBP_AsteroidBase OtherActor))
      (Actor|DestroyActor _asbp_asteroid_base))))

(fn ConstructionScript)

(fn HitCollision
  (params (CollisionHit :type BP%20DEPRECITED%20Object%20Reference))
  (return 0))