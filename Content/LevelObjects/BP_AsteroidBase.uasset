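; Base asteroid actor that drifts through the level and rewards the player with coins when destroyed.
; On BeginPlay it picks a random XY offset, then applies it to its Scene component every Tick with sweep, unscaled by delta time.
; Each Hit event, whatever the source, increments a counter; at HitPoints it adds CoinReward to the BP_PlayerShipBase player pawn's Coins and destroys itself.
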(event Custom|Hit
  (Variables|Default|SetHitCounter (+ (Variables|Default|GetHitCounter) 1))
  (if (>= (Variables|Default|GetHitCounter) (Variables|Default|GetHitPoints))
    (bind _asbp_player_ship_base (Utilities|Casting|CastToBP_PlayerShipBase (Game|Player|GetPlayerPawn 0)))
    (Variables|/Game/Player/BP_PlayerShipBase.BP_PlayerShipBase_C|SetCoins _asbp_player_ship_base (+ (Variables|/Game/Player/BP_PlayerShipBase.BP_PlayerShipBase_C|GetCoins _asbp_player_ship_base) (Variables|Default|GetCoinReward)))
    (Actor|DestroyActor)))

(event EventTick
  (params (DeltaSeconds :type Float%20%28single-precision%29))
  (bind _randomdirection (Variables|Default|GetRandomDirection))
  (Transformation|AddWorldOffset (Variables|Default|GetScene) (Math|Vector|MakeVector (.x _randomdirection) (.y _randomdirection) 0.0) true false))

(event EventBeginPlay
  (Variables|Default|SetRandomDirection (Math|Vector|MakeVector (Math|Random|RandomFloatinRange -4.0 4.0) (Math|Random|RandomFloatinRange -4.0 4.0) 0.0)))

(fn ConstructionScript)