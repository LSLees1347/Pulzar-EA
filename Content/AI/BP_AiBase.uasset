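; BP_AiBase is a base AI with random movement, pawn sensing and attack logic, apparently unfinished.
; BeginPlay rolls random BP_AiBase instances for a self-check and an AIMoveTo target.
; Seeing a pawn clears IsSeeEnemy before FollowPlayer tests it, so that path skips the chase.
; The chase would call the empty SvrPrimaryFire on arrival, with a Timeline looping into an unreset DoOnce.
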(event OnSeePawn(PawnSensing)
  (params (Pawn :type Pawn%20Object%20Reference))
  (Variables|Default|SetisSeeEnemy false)
  (CallFunction|FollowPlayer))

(event Custom|Follow%20Player
  (if (Variables|Default|GetisSeeEnemy)
    (AI|AIMoveTo self "0, 0, 0" (stale OnSeePawn(PawnSensing) Pawn) 15.0 false
      (:OnSuccess
        (if (Variables|Default|GetcanAttack)
          (Variables|Default|SetcanAttack false)
          (Utilities|FlowControl|DoOnce false :!label _label
            (:Completed
              (CallFunction|SvrPrimaryFire)
              (Timeline|Timeline_0 PlayFromStart
                (:Finished
                  (goto _label))))))))))

(event EventBeginPlay
  (bind _outactors (Actor|GetAllActorsOfClass "BP_AiBase_C"))
  (if (not (== self (Utilities|Array|Get(acopy) _outactors (Math|Random|RandomInteger (Utilities|Array|Length _outactors)))))
    (AI|AIMoveTo 0 "0, 0, 0" (Utilities|Array|Get(acopy) _outactors (Math|Random|RandomInteger (Utilities|Array|Length _outactors))) 0.0 false)))

(event Collision|EventActorBeginOverlap
  (params (OtherActor :type Actor%20Object%20Reference)))

(event EventTick
  (params (DeltaSeconds :type Float%20%28single-precision%29)))

(fn ConstructionScript)

(fn FollowPlayer)

(fn SvrPrimaryFire)