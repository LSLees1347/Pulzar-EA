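; BP_BGAI is an enemy AI pawn meant to chase and fire on pawns it sees.
; PawnSensing calls FollowPlayer, whose AIMoveTo branch requires IsSeenEnemy, but the sighting event sets that flag false first.
; A successful move consumes CanAttack, then fires through a DoOnce and Timeline that loops back without a visible reset.
; SvrPrimaryFire is an empty stub.
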(event OnSeePawn(PawnSensing)
  (params (Pawn :type Pawn%20Object%20Reference))
  (Variables|Default|SetIsSeenEnemy false)
  (CallFunction|FollowPlayer))

(event Custom|FollowPlayer
  (if (Variables|Default|GetIsSeenEnemy)
    (AI|AIMoveTo self "0, 0, 0" (stale OnSeePawn(PawnSensing) Pawn) 15.0 false
      (:OnSuccess
        (if (Variables|Default|GetCanAttack)
          (Variables|Default|SetCanAttack false)
          (Utilities|FlowControl|DoOnce false :!label _label
            (:Completed
              (CallFunction|SvrPrimaryFire)
              (Timeline|Timeline PlayFromStart
                (:Finished
                  (goto _label))))))))))

(event EventBeginPlay
  (|CallParentFunction) ; This node is disabled and will not be called.\nDrag off pins to build functionality.
)

(event Collision|EventActorBeginOverlap
  (params (OtherActor :type Actor%20Object%20Reference)))

(event EventTick
  (params (DeltaSeconds :type Float%20%28single-precision%29)))

(fn ConstructionScript
  (|CallParentFunction))

(fn SvrPrimaryFire)