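; Base AI pawn that picks a player ship (BP_ShipBase) and chases it while alive.
; Possession by BP_AI_Controller_Base starts a FindEnemy retry loop, then MoveToPlayer re-issues AIMoveTo two seconds after each success or failure.
; FindEnemy takes a lone ship directly.
; With several, it looks up the lowest NumAiAttackers, but its inverted -1 index check rejects every valid result, so no target is assigned.
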(event Custom|OnAiSpawned
  (bind (_isvalidplayerfound _newenemy) (CallFunction|FindEnemy :!label _label))
  (if _isvalidplayerfound
    (Variables|Default|SetTargetPlayer _newenemy)
    (CallFunction|MovetoPlayer)
    (else
      (Utilities|FlowControl|Delay 0.5)
      (goto _label))))

(event Custom|MoveToPlayer
  (bind _targetplayer (Variables|Default|GetTargetPlayer))
  (if (Variables|Default|GetIsAlive)
    (AI|AIMoveTo self "0, 0, 0" _targetplayer 0.0 false
      (:OnSuccess
        _)
      (:OnFail
        _))
    (Utilities|FlowControl|Delay 2.0)
    (CallFunction|MovetoPlayer)
    (Development|PrintString (Utilities|GetDisplayName _targetplayer))))

(event EventPossessed
  (params (NewController :type Controller%20Object%20Reference))
  (bind _asbp_ai_controller_base (Utilities|Casting|CastToBP_AI_Controller_Base NewController))
  (Variables|Default|SetAs%20BP%20AI%20Controller%20Base _asbp_ai_controller_base)
  (CallFunction|OnAiSpawned))

(fn ConstructionScript)

(fn FindEnemy
  (bind _outactors (Actor|GetAllActorsOfClass "/Game/Player/BP_ShipBase.BP_ShipBase_C"))
  (bind _output_get (LocalVariables|SetLcl_All_Players _outactors))
  (if (Utilities|Array|IsNotEmpty _output_get)
    (if (== (Utilities|Array|Length (LocalVariables|GetLcl_All_Players)) 1)
      (LocalVariables|SetLcl_IsValidPlayerFound true)
      (LocalVariables|SetLcl_NewEnemy (Utilities|Array|Get(acopy) (LocalVariables|GetLcl_All_Players)))
      (else
        (for _array_element (LocalVariables|GetLcl_All_Players)
          (Utilities|Array|Add (LocalVariables|GetLcl_AllAttackerNums) (Variables|/Game/Player/BP_ShipBase.BP_ShipBase_C|GetNum_AiAttackers _array_element)))
        (LocalVariables|SetLcl_LowestIndex (.IndexOfMinValue (Math|Integer|MinOfIntArray (LocalVariables|GetLcl_AllAttackerNums))))
        (if (== (LocalVariables|GetLcl_LowestIndex) -1)
          (Math|Integer|IncrementInt (Variables|/Game/Player/BP_ShipBase.BP_ShipBase_C|GetNum_AiAttackers (Utilities|Array|Get(acopy) (LocalVariables|GetLcl_All_Players) (LocalVariables|GetLcl_LowestIndex)))
            (:%20%20
              (LocalVariables|SetLcl_NewEnemy (Utilities|Array|Get(acopy) (LocalVariables|GetLcl_All_Players) (LocalVariables|GetLcl_LowestIndex)))
              (LocalVariables|SetLcl_IsValidPlayerFound true)))
          (else
            (LocalVariables|SetLcl_IsValidPlayerFound false)))))
    (else
      (LocalVariables|SetLcl_IsValidPlayerFound false)))
  (return (LocalVariables|GetLcl_IsValidPlayerFound) (LocalVariables|GetLcl_NewEnemy)))